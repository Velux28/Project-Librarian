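; Throwable can item that makes noise on impact and reacts to landing in a trash bin bottom.
; Its first hit on anything but the player plays a sound and reports a noise event, with the player as instigator.
; Hitting BP_fondocestino calls that actor's SitEvent and destroys the can.
; LookAt returns formatted name and description text from the data table row set in its item data component.
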(event `self.ReceiveHit`
  (params (MyComp :type "PrimitiveComponent Object Reference") (Other :type "Actor Object Reference") (OtherComp :type "PrimitiveComponent Object Reference") (bSelfMoved :type Boolean) (HitLocation :type "Vector Structure") (HitNormal :type "Vector Structure") (NormalImpulse :type "Vector Structure") (Hit :type "HitResult Structure (by ref)"))
  (bind _returnvalue (`GameplayStatics.GetPlayerCharacter` 0))
  (bind _returnvalue_2 (`self.K2_GetActorLocation`))
  (`|ExecutionSequence`
    (:`then_0`
      (`self.FondoCestino` Other))
    (:`then_1`
      (if (!= Other _returnvalue)
        (`/Engine/EditorBlueprintResources/StandardMacros.DoOnce` false
          (:`Completed`
            (`GameplayStatics.PlaySoundAtLocation` "/Game/SOUNDS/GENERIC/SC_Can.SC_Can" _returnvalue_2 (struct) 1.0 1.0 0.0 null null null null)
            (`AISense_Hearing.ReportNoiseEvent` _returnvalue_2 3.0 _returnvalue)))))))

(fn `FondoCestino`
  (params (Object :type "Object Object Reference"))
  (`/Engine/EditorBlueprintResources/StandardMacros.DoOnce` false
    (:`Completed`
      (bind _asfondocestino (cast `/Game/BP_BO/Environment/BP_fondocestino` Object))
      (`/Game/BP_BO/Environment/BP_fondocestino.SitEvent` _asfondocestino)
      (`self.K2_DestroyActor` self))))

(fn `LookAt`
  (returns (Message :type Text))
  (bind (_itemid_datatable _itemid_rowname) (break `DataTableRowHandle` (`/Game/BP_BO/Inventory/BP_AC_ItemData.ItemID` (`self.BP_AC_ItemData`))))
  (bind _returnvalue (`|GetDataTableRow` _itemid_datatable _itemid_rowname) ; Prendo in considerazione la Row dell'Item_DataTable\nassociata a questo oggetto tramite la variabile ItemID \npropria del BP_AC_ItemData.
    (:`then`
      (bind (_name _description) (break `/Game/BP_BO/Inventory/FItemStruct` _returnvalue))
      (return (`|FormatText` "{item}: {descriprion}" _name _description)) ; Printo il nome e la descrizione scritti nella Row presa in considerazione.
    )))

(fn `UserConstructionScript`)