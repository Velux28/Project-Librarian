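; BP_Respawn is a checkpoint actor that records a respawn point when BP_TPCharacter enters its trigger.
; On overlap it stores the character's current transform, rather than its own, as SpawnTransform on BP_TPGamemode and sets SpawnIsSet.
; It then plays a checkpoint sound and shows the laser and text components for two seconds.
; BeginPlay reuses the hide chain so these visuals start hidden.
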(event `self.CheckpointTrigger.OnComponentBeginOverlap`
  (params (OverlappedComponent :type "PrimitiveComponent Object Reference") (OtherActor :type "Actor Object Reference") (OtherComp :type "PrimitiveComponent Object Reference") (OtherBodyIndex :type Integer) (bFromSweep :type Boolean) (SweepResult :type "HitResult Structure (by ref)"))
  (bind _asbp_tpcharacter (cast `/Game/BP_BO/PlayerCharacter/BP_TPCharacter` OtherActor))
  (bind _asbp_tpgamemode (cast `/Game/BP_BO/PlayerCharacter/BP_TPGamemode` (`GameplayStatics.GetGameMode`)))
  (set `/Game/BP_BO/PlayerCharacter/BP_TPGamemode.SpawnTransform` (`self.GetTransform` _asbp_tpcharacter) _asbp_tpgamemode)
  (set `/Game/BP_BO/PlayerCharacter/BP_TPGamemode.SpawnIsSet` true _asbp_tpgamemode)
  (`GameplayStatics.PlaySound2D` "/Game/BP_BO/PlayerCharacter/SC_Checkpoint.SC_Checkpoint" 1.0 1.0 0.0 null null)
  (`SceneComponent.SetVisibility` (`self.LaserSquareBase`) true false)
  (`SceneComponent.SetVisibility` (`self.CHECKPOINT TXT`) true false)
  (`SceneComponent.SetVisibility` (`self.LaserBeam`) true false)
  (`KismetSystemLibrary.Delay` 2.0)
  (`SceneComponent.SetVisibility` (`self.LaserSquareBase`) false false :!label _label)
  (`SceneComponent.SetVisibility` (`self.CHECKPOINT TXT`) false false)
  (`SceneComponent.SetVisibility` (`self.LaserBeam`) false false))

(event `self.ReceiveBeginPlay`
  (goto _label))

(fn `UserConstructionScript`)