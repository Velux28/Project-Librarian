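; BP_ButtonD2 is an interactable button, labelled "Button" on look-at, that opens the BP_SlidingDoor2 whose GateValue matches its ButtonValue.
; Interaction passes a DoOnce, plays sounds at hardcoded locations, searches all doors, then calls OpenGate after delayed jingle and verification cues.
; The DoOnce resets only after a match opens.
; An older BP_Gate branch with AI noise reporting and a camera switch is left unconnected.
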(event `CustomEvent`
  (params (PlayerCharacter :type "/Game/BP_BO/PlayerCharacter/BP_TPCharacter Object Reference")))

(event `/Game/BP_BO/Inventory/BPI_InteractInterface.InteractWith`
  (params (PlayerCharacter :type "/Game/BP_BO/PlayerCharacter/BP_TPCharacter Object Reference"))
  (`/Engine/EditorBlueprintResources/StandardMacros.DoOnce` false :!label _label
    (:`Completed`
      (`GameplayStatics.PlaySoundAtLocation` "/Game/SOUNDS/TUT_LEV/Cues/SC_Button.SC_Button" (-90.0 669.0 1.0) (struct) 1.0 1.0 0.0 null null null null)
      (bind _outactors (`GameplayStatics.GetAllActorsOfClass` "/Game/BP_BO/Environment/SlidingDoors/BP_SlidingDoor2.BP_SlidingDoor2_C"))
      (for _array_element _outactors
        (if (== (`/Game/BP_BO/Environment/SlidingDoors/BP_SlidingDoor2.Gate Value` _array_element) (`self.ButtonValue`))
          (`GameplayStatics.PlaySoundAtLocation` "/Game/SOUNDS/TUT_LEV/Cues/SC_Jingle.SC_Jingle" (-24.029825 445.914062 -29.0) (struct) 1.0 1.0 0.0 null null null null)
          (`KismetSystemLibrary.Delay` 1.0)
          (`GameplayStatics.PlaySoundAtLocation` "/Game/SOUNDS/TUT_LEV/Cues/SC_Verified.SC_Verified" (-24.029825 445.914062 -29.0) (struct) 1.0 1.0 0.0 null null null null)
          (`KismetSystemLibrary.Delay` 2.0)
          (`/Game/BP_BO/Environment/SlidingDoors/BP_SlidingDoor2.Open Gate` _array_element PlayerCharacter)
          (goto _label :!via `Reset`))))))

(fn `LookAt`
  (returns (Message :type Text))
  (return "Button"))

(fn `UserConstructionScript`)