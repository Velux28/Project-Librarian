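; Two-panel sliding door that opens on an OpenGate event and closes itself after a delay.
; Opening and closing timelines lerp each panel's relative location toward its offset vector, each playing a sliding sound at a hardcoded world position.
; The DoOnce guard resets in the same sequence without waiting for the delay, so repeated calls can restart the opening.
; A BP_CardGate lookup is present but never runs.
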(event `Open Gate`
  (params (PlayerCharacter :type "Actor Object Reference"))
  (`/Engine/EditorBlueprintResources/StandardMacros.DoOnce` false :!label _label
    (:`Completed`
      (`|ExecutionSequence`
        (:`then_0`
          (`GameplayStatics.PlaySoundAtLocation` "/Game/SOUNDS/TUT_LEV/Cues/SC_SlidingDoor.SC_SlidingDoor" (-24.0 445.0 -29.0) (struct) 1.0 1.0 0.0 null "/Game/SOUNDS/TUT_LEV/Cues/CONC_Environment.CONC_Environment" null null)
          (bind (_direction _newtrack_0) (`Timeline|OPENING TIMELINE` :!via `PlayFromStart`)
            (:`Update`
              (`SceneComponent.K2_SetRelativeLocation` (`self.RightPanel`) (`KismetMathLibrary.VLerp` (0.0 0.0 0.0) (`self.RightPanelV`) _newtrack_0) false false)
              (`SceneComponent.K2_SetRelativeLocation` (`self.LeftPanel`) (`KismetMathLibrary.VLerp` (0.0 0.0 0.0) (`self.LeftPanelV`) _newtrack_0) false false))))
        (:`then_1`
          (`KismetSystemLibrary.Delay` 10.0)
          (`GameplayStatics.PlaySoundAtLocation` "/Game/SOUNDS/TUT_LEV/Cues/SC_SlidingDoor.SC_SlidingDoor" (-24.0 445.0 -29.0) (struct) 1.0 1.0 0.0 null "/Game/SOUNDS/TUT_LEV/Cues/CONC_Environment.CONC_Environment" null null)
          (bind (_direction_2 _newtrack_0_2) (`Timeline|CLOSING TIMELINE` :!via `PlayFromStart`)
            (:`Update`
              (`SceneComponent.K2_SetRelativeLocation` (`self.RightPanel`) (`KismetMathLibrary.VLerp` (0.0 0.0 0.0) (`self.RightPanelV`) _newtrack_0_2) false false)
              (`SceneComponent.K2_SetRelativeLocation` (`self.LeftPanel`) (`KismetMathLibrary.VLerp` (0.0 0.0 0.0) (`self.LeftPanelV`) _newtrack_0_2) false false))))
        (:`then_2`
          (goto _label :!via `Reset`))))))

(fn `UserConstructionScript`)