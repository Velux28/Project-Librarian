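; BP_Dozer is an actor that fakes AI movement by riding a spline path through the level.
; On BeginPlay it finds the SPL_TestRoom actor and starts a timeline whose play rate is the inverse of TimeToCompleteSec.
; Each update maps the timeline alpha to a distance along the FakeAIPath spline and sets the actor's world location and rotation from that point.
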(event `self.ReceiveBeginPlay`
  (bind _returnvalue (`GameplayStatics.GetActorOfClass` "/Game/BP_BO/ArtificialIntelligence/Dozer/SPL_TestRoom.SPL_TestRoom_C"))
  (set `self.SplineRef` _returnvalue)
  (`self.MovingObject`))

(event `MovingObject`
  (`TimelineComponent.SetPlayRate` (`self.Timeline_0`) (/ 1.0 (`self.TimeToComplete (sec)`)))
  (bind (_direction _newtrack_0) (`Timeline|Timeline_0`)
    (:`Update`
      (bind _returnvalue (`KismetMathLibrary.Lerp` 0.0 (`SplineComponent.GetSplineLength` (`/Game/BP_BO/ArtificialIntelligence/Dozer/SPL_TestRoom.FakeAI_Path` (`self.SplineRef`))) _newtrack_0))
      (`self.K2_SetActorTransform` (`KismetMathLibrary.MakeTransform` (`SplineComponent.GetLocationAtDistanceAlongSpline` (`/Game/BP_BO/ArtificialIntelligence/Dozer/SPL_TestRoom.FakeAI_Path` (`self.SplineRef`)) _returnvalue "World") (`SplineComponent.GetRotationAtDistanceAlongSpline` (`/Game/BP_BO/ArtificialIntelligence/Dozer/SPL_TestRoom.FakeAI_Path` (`self.SplineRef`)) _returnvalue "World"))))))

(fn `UserConstructionScript`)