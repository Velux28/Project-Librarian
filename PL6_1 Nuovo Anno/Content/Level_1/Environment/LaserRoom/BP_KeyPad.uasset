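; BP_KeyPad is a keypad actor in the Level 1 laser room.
; When BP_TPCharacter leaves its Box, it removes all widgets.
; Logic to show the W_Keypad widget with mouse cursor and Game and UI input while IsCorrect is false is present but unconnected, so it never runs.
; Its LookAt function returns an empty string.
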(event `self.Box.OnComponentEndOverlap`
  (params (OverlappedComponent :type "PrimitiveComponent Object Reference") (OtherActor :type "Actor Object Reference") (OtherComp :type "PrimitiveComponent Object Reference") (OtherBodyIndex :type Integer))
  (cast `/Game/BP_BO/PlayerCharacter/BP_TPCharacter` OtherActor)
  (`WidgetLayoutLibrary.RemoveAllWidgets`))

(fn `LookAt`
  (returns (Message :type Text))
  (return ""))

(fn `UserConstructionScript`)