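; Card reader that opens sliding gates when the player interacts while holding at least one key, and otherwise plays access-denied sounds.
; On success it flashes a spotlight, plays verification audio and slides a runtime-spawned data chip mesh along a timeline.
; It then calls OpenGate on every BP_SlidingDoor2 whose GateValue matches its ButtonValue.
; A DoOnce blocks repeat use until denial finishes or 15 seconds after opening.
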(event `self.ReceiveBeginPlay`
  (`ActorComponent.Deactivate` (`self.SpotLight`)))

(event `/Game/BP_BO/Inventory/BPI_InteractInterface.InteractWith`
  (params (PlayerCharacter :type "/Game/BP_BO/PlayerCharacter/BP_TPCharacter Object Reference"))
  (`/Engine/EditorBlueprintResources/StandardMacros.DoOnce` false :!label _label
    (:`Completed`
      (if (> (`/Game/BP_BO/PlayerCharacter/BP_TPCharacter.NumberOfKeys` PlayerCharacter) 0)
        (`ActorComponent.Activate` (`self.SpotLight`) false)
        (`GameplayStatics.PlaySoundAtLocation` "/Game/SOUNDS/TUT_LEV/Cues/SC_Jingle.SC_Jingle" (-1441.0 7080.0 103.0) (struct) 1.0 1.0 0.0 null null null null)
        (`KismetSystemLibrary.Delay` 1.0)
        (`GameplayStatics.PlaySoundAtLocation` "/Game/SOUNDS/TUT_LEV/Cues/SC_Verified.SC_Verified" (-1441.0 7080.0 103.0) (struct) 1.0 1.0 0.0 null null null null)
        (bind _returnvalue (`AddComponent|NODE_AddStaticMeshComponent-9`))
        (bind _output_get (set `self.data chip` _returnvalue))
        (`SceneComponent.K2_AttachToComponent` _output_get null "None" "KeepRelative" "KeepRelative" "SnapToTarget" true)
        (bind (_direction _keyposition) (`Timeline|Timeline_0` :!via `PlayFromStart`)
          (:`Update`
            (`SceneComponent.K2_SetRelativeLocationAndRotation` (`self.data chip`) (`KismetMathLibrary.MakeVector` 25.75 _keyposition) (struct :`Pitch` 90.0) false false)
            (`ActorComponent.Deactivate` (`self.SpotLight`)))
          (:`Finished`
            (bind _outactors (`GameplayStatics.GetAllActorsOfClass` "/Game/BP_BO/Environment/SlidingDoors/BP_SlidingDoor2.BP_SlidingDoor2_C"))
            (for _array_element _outactors
              (if (== (`/Game/BP_BO/Environment/SlidingDoors/BP_SlidingDoor2.Gate Value` _array_element) (`self.ButtonValue`))
                (`GameplayStatics.PlaySoundAtLocation` "/Game/SOUNDS/TUT_LEV/Cues/SC_SlidingDoor.SC_SlidingDoor" (-1440.0 6857.0 -0.0) (struct) 1.0 1.0 0.0 null "/Game/SOUNDS/TUT_LEV/Cues/CONC_Environment.CONC_Environment" null null)
                (`/Game/BP_BO/Environment/SlidingDoors/BP_SlidingDoor2.Open Gate` _array_element PlayerCharacter)
                (`ActorComponent.K2_DestroyComponent` (`self.data chip`))
                (`KismetSystemLibrary.Delay` 15.0)
                (goto _label :!via `Reset`)))))
        (else
          (`GameplayStatics.PlaySoundAtLocation` "/Game/SOUNDS/TUT_LEV/Cues/SC_InteractionDenied.SC_InteractionDenied" (-1441.0 7080.0 103.0) (struct) 1.0 1.0 0.0 null null null null)
          (`KismetSystemLibrary.Delay` 1.0)
          (`GameplayStatics.PlaySoundAtLocation` "/Game/SOUNDS/TUT_LEV/Cues/SC_AccesDenied__VOICE.SC_AccesDenied__VOICE" (-1441.0 7080.0 103.0) (struct) 1.0 1.0 0.0 null null null null)
          (goto _label :!via `Reset`))))))

(fn `LookAt`
  (returns (Message :type Text))
  (return "Button"))

(fn `UserConstructionScript`)