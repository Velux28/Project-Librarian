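; Interactable button that opens the level's laser gate when the player has at least one key.
; On interaction it flashes a spotlight, plays verification sounds and animates a spawned data chip along a timeline, then destroys the LASER_GATE_BP actor found by class.
; Without a key it plays denial sounds and resets its DoOnce for another try; key count is left unchanged.
; Sounds play at hardcoded world locations, and LookAt returns "Button".
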(event `self.ReceiveBeginPlay`
  (`ActorComponent.Deactivate` (`self.SpotLight`)))

(event `/Game/BP_BO/Inventory/BPI_InteractInterface.InteractWith`
  (params (PlayerCharacter :type "/Game/BP_BO/PlayerCharacter/BP_TPCharacter Object Reference"))
  (bind _datachip (`self.DataChip`))
  (`/Engine/EditorBlueprintResources/StandardMacros.DoOnce` false :!label _label
    (:`Completed`
      (if (> (`/Game/BP_BO/PlayerCharacter/BP_TPCharacter.NumberOfKeys` PlayerCharacter) 0)
        (`ActorComponent.Activate` (`self.SpotLight`) false)
        (`GameplayStatics.PlaySoundAtLocation` "/Game/SOUNDS/TUT_LEV/Cues/SC_Jingle.SC_Jingle" (1830.0 4677.0 118.0) (struct) 1.0 1.0 0.0 null null null null)
        (`KismetSystemLibrary.Delay` 1.0)
        (`GameplayStatics.PlaySoundAtLocation` "/Game/SOUNDS/TUT_LEV/Cues/SC_Verified.SC_Verified" (1830.0 4677.0 118.0) (struct) 1.0 1.0 0.0 null null null null)
        (bind _returnvalue (`AddComponent|NODE_AddStaticMeshComponent-7`))
        (bind _output_get (set `self.DataChip` _returnvalue))
        (`SceneComponent.K2_AttachToComponent` _output_get null "None" "KeepRelative" "KeepRelative" "SnapToTarget" true)
        (bind (_direction _keyposition) (`Timeline|Timeline_0` :!via `PlayFromStart`)
          (:`Update`
            (`SceneComponent.K2_SetRelativeRotation` _datachip (struct :`Pitch` 180.0 :`Roll` 90.0) false false)
            (`SceneComponent.K2_SetRelativeLocation` _datachip (`KismetMathLibrary.MakeVector` _keyposition 25.75) false false)
            (`ActorComponent.Deactivate` (`self.SpotLight`)))
          (:`Finished`
            (`GameplayStatics.PlaySound2D` "/Game/Level_1/Environment/Sounds/SC_PowerDown.SC_PowerDown" 1.0 1.0 0.0 null null)
            (bind _returnvalue_2 (`GameplayStatics.GetActorOfClass` "/Game/Level_1/Environment/LaserGate/LASER_GATE_BP.LASER_GATE_BP_C"))
            (bind _output_get_2 (set `self.LaserGate` _returnvalue_2))
            (`self.K2_DestroyActor` _output_get_2)))
        (else
          (`GameplayStatics.PlaySoundAtLocation` "/Game/SOUNDS/TUT_LEV/Cues/SC_InteractionDenied.SC_InteractionDenied" (1833.0 4741.0 113.0) (struct) 1.0 1.0 0.0 null null null null)
          (`KismetSystemLibrary.Delay` 1.0)
          (`GameplayStatics.PlaySoundAtLocation` "/Game/SOUNDS/TUT_LEV/Cues/SC_AccesDenied__VOICE.SC_AccesDenied__VOICE" (1833.0 4741.0 113.0) (struct) 1.0 1.0 0.0 null null null null)
          (goto _label :!via `Reset`))))))

(fn `LookAt`
  (returns (Message :type Text))
  (return "Button"))

(fn `UserConstructionScript`)