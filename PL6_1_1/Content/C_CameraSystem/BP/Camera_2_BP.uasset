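; Placeable surveillance camera Blueprint that feeds its scene capture into one of four render targets on a CameraSystem actor.
; The construction script applies the FOV to the camera and capture components, sets per-frame capture, and creates a dynamic lens material with configurable colors and brightness.
; On BeginPlay, after a short delay, it matches CameraSystem ScreenID to Monitor, selects the target by Position, then destroys the Camera component.
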(event `self.ReceiveTick`
  (params (DeltaSeconds :type "Float (single-precision)")))

(event `self.ReceiveBeginPlay`
  (bind _scenecapture (`self.SceneCapture`))
  (bind _outactors (`GameplayStatics.GetAllActorsOfClass` "/Game/C_CameraSystem/BP/CameraSystem.CameraSystem_C"))
  (`KismetSystemLibrary.Delay` 2.0)
  (for _array_element _outactors
    (if (== (`/Game/C_CameraSystem/BP/CameraSystem.ScreenID` _array_element) (`self.Monitor?`))
      (switch `int` (`self.Position`)
        (:`0`
          (set `SceneCaptureComponent2D.TextureTarget` (`/Game/C_CameraSystem/BP/CameraSystem.Render1` _array_element) _scenecapture))
        (:`1`
          (set `SceneCaptureComponent2D.TextureTarget` (`/Game/C_CameraSystem/BP/CameraSystem.Render2` _array_element) _scenecapture))
        (:`2`
          (set `SceneCaptureComponent2D.TextureTarget` (`/Game/C_CameraSystem/BP/CameraSystem.Render3` _array_element) _scenecapture))
        (:`3`
          (set `SceneCaptureComponent2D.TextureTarget` (`/Game/C_CameraSystem/BP/CameraSystem.Render4` _array_element) _scenecapture)))))
  (`ActorComponent.K2_DestroyComponent` (`self.Camera`)))

(fn `UserConstructionScript`
  (bind _fov (`self.FOV`))
  (bind _scenecapture (`self.SceneCapture`))
  (`CameraComponent.SetFieldOfView` (`self.Camera`) _fov)
  (set `SceneCaptureComponent2D.FOVAngle` _fov _scenecapture)
  (set `SceneCaptureComponent.bCaptureEveryFrame` (`self.CaptureEveryFrame?`) _scenecapture)
  (bind _returnvalue (`PrimitiveComponent.CreateDynamicMaterialInstance` (`self.Camera2_Static_Camera_1_2`) 0 "/Game/C_CameraSystem/Material/Cam2_Lense_Inst.Cam2_Lense_Inst" "None"))
  (`MaterialInstanceDynamic.SetVectorParameterValue` _returnvalue "LenseColor" (`self.LenseColor`))
  (`MaterialInstanceDynamic.SetVectorParameterValue` _returnvalue "LightColor" (`self.LightColor`))
  (`MaterialInstanceDynamic.SetScalarParameterValue` _returnvalue "LenseBrightness" (`self.LenseBrightness`))
  (`MaterialInstanceDynamic.SetScalarParameterValue` _returnvalue "LightBrightness" (`self.LightBrightness`)))