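; BP_RestroomLights_JS is a one-shot trigger event, named for restroom lights, that flashes a skeletal mesh into view along with four rect lights.
; Lights and mesh start hidden on BeginPlay.
; The first overlap of any actor destroys the trigger, shows everything briefly, then cuts to dark.
; After a longer delay, only the lights return, leaving the mesh hidden.
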(event `self.ReceiveBeginPlay`
  (`SceneComponent.SetVisibility` (`self.RectLight3`) false false)
  (`SceneComponent.SetVisibility` (`self.RectLight`) false false)
  (`SceneComponent.SetVisibility` (`self.RectLight2`) false false)
  (`SceneComponent.SetVisibility` (`self.RectLight1`) false false)
  (`SceneComponent.SetVisibility` (`self.SkeletalMesh`) false false))

(event `self.Trigger.OnComponentBeginOverlap`
  (params (OverlappedComponent :type "PrimitiveComponent Object Reference") (OtherActor :type "Actor Object Reference") (OtherComp :type "PrimitiveComponent Object Reference") (OtherBodyIndex :type Integer) (bFromSweep :type Boolean) (SweepResult :type "HitResult Structure (by ref)"))
  (`ActorComponent.K2_DestroyComponent` (`self.Trigger`))
  (`SceneComponent.SetVisibility` (`self.RectLight3`) true false)
  (`SceneComponent.SetVisibility` (`self.RectLight`) true false)
  (`SceneComponent.SetVisibility` (`self.RectLight2`) true false)
  (`SceneComponent.SetVisibility` (`self.RectLight1`) true false)
  (`SceneComponent.SetVisibility` (`self.SkeletalMesh`) true false)
  (`KismetSystemLibrary.Delay` 0.5)
  (`SceneComponent.SetVisibility` (`self.RectLight3`) false false)
  (`SceneComponent.SetVisibility` (`self.RectLight`) false false)
  (`SceneComponent.SetVisibility` (`self.RectLight2`) false false)
  (`SceneComponent.SetVisibility` (`self.RectLight1`) false false)
  (`SceneComponent.SetVisibility` (`self.SkeletalMesh`) false false)
  (`KismetSystemLibrary.Delay` 2.0)
  (`SceneComponent.SetVisibility` (`self.RectLight3`) true false)
  (`SceneComponent.SetVisibility` (`self.RectLight`) true false)
  (`SceneComponent.SetVisibility` (`self.RectLight2`) true false)
  (`SceneComponent.SetVisibility` (`self.RectLight1`) true false))

(fn `UserConstructionScript`)