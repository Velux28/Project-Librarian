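; Flickering lamp Blueprint that switches a static mesh and rect light on and off in an irregular, endless loop.
; BeginPlay starts a chain of randomized delays alternating TurnOn and TurnOff, which ends by calling Flicker again to repeat.
; Each state swaps the mesh between lit and unlit oval-light materials and sets the RectLight's visibility to match.
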(event `Flicker`
  (`KismetSystemLibrary.Delay` (`KismetMathLibrary.RandomFloatInRange` 1.0 1.5) :!label _label)
  (`self.Turn On`)
  (`KismetSystemLibrary.Delay` (`KismetMathLibrary.RandomFloatInRange` 0.8 1.3))
  (`self.Turn Off`)
  (`KismetSystemLibrary.Delay` (`KismetMathLibrary.RandomFloatInRange` 0.1 0.3))
  (`self.Turn On`)
  (`KismetSystemLibrary.Delay` (`KismetMathLibrary.RandomFloatInRange` 0.5 0.7))
  (`self.Turn Off`)
  (`KismetSystemLibrary.Delay` (`KismetMathLibrary.RandomFloatInRange` 0.2 0.4))
  (`self.Turn On`)
  (`KismetSystemLibrary.Delay` (`KismetMathLibrary.RandomFloatInRange` 0.9 1.4))
  (`self.Turn Off`)
  (`KismetSystemLibrary.Delay` (`KismetMathLibrary.RandomFloatInRange` 0.1 0.4))
  (`self.Turn On`)
  (`KismetSystemLibrary.Delay` (`KismetMathLibrary.RandomFloatInRange` 1.0 1.0))
  (`self.Turn Off`)
  (`KismetSystemLibrary.Delay` (`KismetMathLibrary.RandomFloatInRange` 0.1 0.3))
  (`self.Turn On`)
  (`KismetSystemLibrary.Delay` (`KismetMathLibrary.RandomFloatInRange` 0.2 0.5))
  (`self.Turn Off`)
  (`KismetSystemLibrary.Delay` (`KismetMathLibrary.RandomFloatInRange` 0.3 0.7))
  (`self.Turn On`)
  (`KismetSystemLibrary.Delay` (`KismetMathLibrary.RandomFloatInRange` 0.2 0.2))
  (`self.Turn Off`)
  (`self.Flicker`))

(event `self.ReceiveBeginPlay`
  (goto _label))

(event `Turn Off`
  (`self.Off functionality`))

(event `Turn On`
  (`self.On functionality`))

(fn `Off functionality`
  (`PrimitiveComponent.SetMaterial` (`self.StaticMesh`) 0 "/Game/3DAssetLevel/3DArt/Materials/MaterialInstances/Roof_OvalLamp/MI_LuceOvale_spenta.MI_LuceOvale_spenta")
  (`SceneComponent.SetVisibility` (`self.RectLight`) false false))

(fn `On functionality`
  (`PrimitiveComponent.SetMaterial` (`self.StaticMesh`) 0 "/Game/3DAssetLevel/3DArt/Materials/MaterialInstances/Roof_OvalLamp/MI_LuceOvale.MI_LuceOvale")
  (`SceneComponent.SetVisibility` (`self.RectLight`) true false))

(fn `UserConstructionScript`)