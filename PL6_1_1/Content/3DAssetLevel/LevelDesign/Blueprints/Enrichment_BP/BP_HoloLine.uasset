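; BP_HoloLine is a level-dressing holographic line mesh with a selectable line variant, emissive color and optional glitchy look.
; Both the Construction Script and BeginPlay swap in the glitch security-lines material when flagged, then call ChangeLineColor.
; That function creates a dynamic material instance and, if the key exists in LinesKeys, uses its index as the vertical UV offset and applies the color.
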(event `self.ReceiveBeginPlay`
  (if (`self.B_IsGlitchy`)
    (`PrimitiveComponent.SetMaterial` (`self.HoloMesh`) 0 "/Game/3DAssetLevel/LevelDesign/Materials/BP_Mats/Instances/MI_Holo_SecurityLines_Glitch.MI_Holo_SecurityLines_Glitch"))
  (`self.Change Line & Color` (`self.Curr key`) (`self.Emissive Color`)))

(fn `Change Line & Color`
  (params (`New key` :type "/Game/BP_BO/Enum/E_HoloLines Enum" :default "NewEnumerator0") (`Emissive Color` :type "LinearColor Structure"))
  (bind _holomesh (`self.HoloMesh`))
  (bind _output_get (set `self.Curr key` `New key`))
  (bind _output_get_2 (set `self.Emissive Color` `Emissive Color`))
  (bind _returnvalue (`PrimitiveComponent.CreateDynamicMaterialInstance` _holomesh 0 (`PrimitiveComponent.GetMaterial` _holomesh 0) "None"))
  (bind _returnvalue_2 (`KismetArrayLibrary.Array_Find` (`self.Lines keys`) _output_get))
  (if (> _returnvalue_2 -1)
    (`MaterialInstanceDynamic.SetScalarParameterValue` _returnvalue "UVOffset_Y" (`KismetMathLibrary.Conv_IntToDouble` _returnvalue_2))
    (`MaterialInstanceDynamic.SetVectorParameterValue` _returnvalue "EmissiveColor" _output_get_2)))

(fn `UserConstructionScript`
  (if (`self.B_IsGlitchy`)
    (`PrimitiveComponent.SetMaterial` (`self.HoloMesh`) 0 "/Game/3DAssetLevel/LevelDesign/Materials/BP_Mats/Instances/MI_Holo_SecurityLines_Glitch.MI_Holo_SecurityLines_Glitch"))
  (`self.Change Line & Color` (`self.Curr key`) (`self.Emissive Color`)))