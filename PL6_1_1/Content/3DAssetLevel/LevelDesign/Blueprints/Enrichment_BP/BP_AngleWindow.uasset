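; Angled window prop whose glass can be broken once through the BreakGlass event.
; BreakGlass passes a DoOnce, destroys the intact Glass1 component and reveals the BrokenGlass piece components, swapping components rather than simulating fracture.
; The crash sound is only a debug PrintString, and the construction script is empty.
; Nothing in this Blueprint calls BreakGlass itself.
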(event `BreakGlass`
  (`/Engine/EditorBlueprintResources/StandardMacros.DoOnce` false
    (:`Completed`
      (`ActorComponent.K2_DestroyComponent` (`self.Glass1`))
      (`SceneComponent.SetVisibility` (`self.BrokenGlass_2`) true false)
      (`SceneComponent.SetVisibility` (`self.BrokenGlass_3`) true false)
      (`SceneComponent.SetVisibility` (`self.BrokenGlass_4`) true false)
      (`SceneComponent.SetVisibility` (`self.BrokenGlass_5`) true false)
      (`SceneComponent.SetVisibility` (`self.BrokenGlass_0`) true false)
      (`SceneComponent.SetVisibility` (`self.BrokenGlass_6`) true false)
      (`SceneComponent.SetVisibility` (`self.BrokenGlass_7`) true false)
      (`SceneComponent.SetVisibility` (`self.BrokenGlass_8`) true false)
      (`SceneComponent.SetVisibility` (`self.BrokenGlass_1`) true false)
      (`KismetSystemLibrary.PrintString` "Loud crash sounds"))))

(fn `UserConstructionScript`)