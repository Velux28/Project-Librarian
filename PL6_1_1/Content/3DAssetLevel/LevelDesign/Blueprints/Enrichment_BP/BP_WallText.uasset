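; Wall text decoration actor for level design that displays configurable emissive text through a text render component.
; The construction script maps a font enum to one of five font and emissive material pairs, then sets the text, size and alignment.
; It also creates a dynamic material instance from TextMaterialInstance to apply text color and emissive intensity.
; The event graph has no logic, so all setup happens at construction.
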(fn `UserConstructionScript`
  (bind _walltext (`self.WallText`))
  (bind _walltext_2 (`self.WallText`))
  (bind _walltext_3 (`self.WallText`))
  (bind _walltext_4 (`self.WallText`))
  (bind _walltext_5 (`self.WallText`))
  (bind _walltext_6 (`self.WallText`))
  (`|ExecutionSequence`
    (:`then_0`
      (if (`|EnumEquality` (`self.ENUM_Font`) "NewEnumerator0")
        (`TextRenderComponent.SetTextMaterial` _walltext_6 "/Game/3DAssetLevel/LevelDesign/Materials/Fonts/Orbitron/MI_Orbitron_Emissive.MI_Orbitron_Emissive")
        (`TextRenderComponent.SetFont` _walltext_6 "/Game/3DAssetLevel/LevelDesign/Materials/Fonts/Orbitron/FONT_Orbitron.FONT_Orbitron")
        (elif (`|EnumEquality` (`self.ENUM_Font`) "NewEnumerator1")
          (`TextRenderComponent.SetTextMaterial` _walltext_2 "/Game/3DAssetLevel/LevelDesign/Materials/Fonts/Derelict/Derelict_Regular/MI_DerelictRegular_Emissive.MI_DerelictRegular_Emissive")
          (`TextRenderComponent.SetFont` _walltext_2 "/Game/3DAssetLevel/LevelDesign/Materials/Fonts/Derelict/Derelict_Regular/F_Derelict_Regular_Font.F_Derelict_Regular_Font")
          (elif (`|EnumEquality` (`self.ENUM_Font`) "NewEnumerator2")
            (`TextRenderComponent.SetTextMaterial` _walltext_3 "/Game/3DAssetLevel/LevelDesign/Materials/Fonts/Derelict/Derelict_Rough/MI_DerelictRough_Emissive.MI_DerelictRough_Emissive")
            (`TextRenderComponent.SetFont` _walltext_3 "/Game/3DAssetLevel/LevelDesign/Materials/Fonts/Derelict/Derelict_Rough/F_Derelict_Rough_Font.F_Derelict_Rough_Font")
            (elif (`|EnumEquality` (`self.ENUM_Font`) "NewEnumerator3")
              (`TextRenderComponent.SetTextMaterial` _walltext_4 "/Game/3DAssetLevel/LevelDesign/Materials/Fonts/Neuropol/M_Neuropol_Emissive.M_Neuropol_Emissive")
              (`TextRenderComponent.SetFont` _walltext_4 "/Game/3DAssetLevel/LevelDesign/Materials/Fonts/Neuropol/F_Neuropol_Font.F_Neuropol_Font")
              (elif (`|EnumEquality` (`self.ENUM_Font`) "NewEnumerator4")
                (`TextRenderComponent.SetTextMaterial` _walltext "/Game/3DAssetLevel/LevelDesign/Materials/Fonts/Inter/MI_Inter_Emissive.MI_Inter_Emissive")
                (`TextRenderComponent.SetFont` _walltext "/Game/3DAssetLevel/LevelDesign/Materials/Fonts/Inter/FONT_Inter.FONT_Inter")))))))
    (:`then_1`
      (`TextRenderComponent.K2_SetText` _walltext_5 (`self.ShownText`))
      (bind _returnvalue (`PrimitiveComponent.CreateDynamicMaterialInstance` _walltext_5 0 (`self.TextMaterialInstance`) "None"))
      (`MaterialInstanceDynamic.SetScalarParameterValue` _returnvalue "Emissive" (`self.EmissiveIntensity`))
      (`MaterialInstanceDynamic.SetVectorParameterValue` _returnvalue "TextColor" (`self.TextColor`))
      (`TextRenderComponent.SetWorldSize` _walltext_5 (`self.Text WorldSize`))
      (`TextRenderComponent.SetHorizontalAlignment` _walltext_5 (`self.HorizontalAlignment`))
      (`TextRenderComponent.SetVerticalAlignment` _walltext_5 (`self.VerticalAlignment`)))))