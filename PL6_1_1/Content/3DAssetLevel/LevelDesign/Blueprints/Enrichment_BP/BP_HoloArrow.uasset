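; BP_HoloArrow is a placeable level-design arrow actor that shows a holographic direction marker.
; The construction script configures the HoloArrow mesh from the ArrowDirection enum: straight mesh, 180-degree rotation, or scaled curved mesh.
; The two curved variants share one mesh, mirrored through negative Y scale.
; Rotation and scale are set in world space, and the event graph holds no active logic.
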(fn `UserConstructionScript`
  (bind _holoarrow (`self.HoloArrow`))
  (bind _holoarrow_2 (`self.HoloArrow`))
  (if (`|EnumEquality` (`self.ArrowDirection`) "NewEnumerator0")
    (`StaticMeshComponent.SetStaticMesh` (`self.HoloArrow`) "/Game/3DAssetLevel/3DArt/StaticMeshes/Guidance/SM_HoloArrow_Straight.SM_HoloArrow_Straight")
    (elif (`|EnumEquality` (`self.ArrowDirection`) "NewEnumerator1")
      (`SceneComponent.K2_SetWorldRotation` (`self.HoloArrow`) (struct :`Yaw` 180.0) false false)
      (elif (`|EnumEquality` (`self.ArrowDirection`) "NewEnumerator3")
        (`StaticMeshComponent.SetStaticMesh` _holoarrow_2 "/Game/3DAssetLevel/3DArt/StaticMeshes/Guidance/SM_HoloArrow_Curved.SM_HoloArrow_Curved")
        (`SceneComponent.SetWorldScale3D` _holoarrow_2 (1.5 1.0 1.5))
        (elif (`|EnumEquality` (`self.ArrowDirection`) "NewEnumerator2")
          (`StaticMeshComponent.SetStaticMesh` _holoarrow "/Game/3DAssetLevel/3DArt/StaticMeshes/Guidance/SM_HoloArrow_Curved.SM_HoloArrow_Curved")
          (`SceneComponent.SetWorldScale3D` _holoarrow (1.5 -1.0 1.5)))))))