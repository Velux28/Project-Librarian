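; BP_LaserLocks_B is a room lock that seals the player in with two laser barriers when they enter a trigger.
; BeginPlay hides both lasers and a text render and disables laser collision.
; The one-shot trigger destroys itself on overlap, shows the lasers and text with blocking collision, then a temporary five-second delay releases them.
; An empty QuizComplete event exists, but its call is never executed.
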(event `self.ReceiveBeginPlay`
  ;[1 1 1] RoomSetup
  (`SceneComponent.SetVisibility` (`self.LaserLock_1`) false false)
  (`SceneComponent.SetVisibility` (`self.LaserLock_2`) false false)
  (`SceneComponent.SetVisibility` (`self.TextRender`) false false)
  (`PrimitiveComponent.SetCollisionEnabled` (`self.LaserLock_1`) "NoCollision")
  (`PrimitiveComponent.SetCollisionEnabled` (`self.LaserLock_2`) "NoCollision"))

(event `self.LockTrigger.OnComponentBeginOverlap`
  (params (OverlappedComponent :type "PrimitiveComponent Object Reference") (OtherActor :type "Actor Object Reference") (OtherComp :type "PrimitiveComponent Object Reference") (OtherBodyIndex :type Integer) (bFromSweep :type Boolean) (SweepResult :type "HitResult Structure (by ref)"))
  ;[1 1 1] LaserLocks Activation
  (`ActorComponent.K2_DestroyComponent` (`self.LockTrigger`))
  (`SceneComponent.SetVisibility` (`self.LaserLock_1`) true false)
  (`SceneComponent.SetVisibility` (`self.LaserLock_2`) true false)
  (`SceneComponent.SetVisibility` (`self.TextRender`) true false)
  (`PrimitiveComponent.SetCollisionEnabled` (`self.LaserLock_1`) "QueryAndPhysics")
  (`PrimitiveComponent.SetCollisionEnabled` (`self.LaserLock_2`) "QueryAndPhysics")
  ;[1 0.02754 0] TEMPORARY SOLUTION
  (`KismetSystemLibrary.Delay` 5.0)
  ;[1 1 1] LaserLocks Deactivation
  (`SceneComponent.SetVisibility` (`self.LaserLock_1`) false false)
  (`SceneComponent.SetVisibility` (`self.LaserLock_2`) false false)
  (`SceneComponent.SetVisibility` (`self.TextRender`) false false)
  (`PrimitiveComponent.SetCollisionEnabled` (`self.LaserLock_1`) "NoCollision")
  (`PrimitiveComponent.SetCollisionEnabled` (`self.LaserLock_2`) "NoCollision"))

(event `QuizComplete`
  ;[1 1 1] LaserLocks Deactivation
)

(fn `UserConstructionScript`)