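; BP_OfficeDoor_JS is an office door that swings open once when something enters its trigger box.
; BeginPlay sets fixed closed and open rotations about the yaw axis.
; The first overlap destroys the trigger, so it cannot fire again, then plays a timeline that lerps ContDoor's relative rotation from closed to open.
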(event `self.ReceiveBeginPlay`
  (set `self.RotationStart` (struct))
  (set `self.RotationEnd` (struct :`Yaw` -50.0)))

(event `self.TriggerBox.OnComponentBeginOverlap`
  (params (OverlappedComponent :type "PrimitiveComponent Object Reference") (OtherActor :type "Actor Object Reference") (OtherComp :type "PrimitiveComponent Object Reference") (OtherBodyIndex :type Integer) (bFromSweep :type Boolean) (SweepResult :type "HitResult Structure (by ref)"))
  (`ActorComponent.K2_DestroyComponent` (`self.TriggerBox`))
  (bind (_direction _rotatortrack) (`Timeline|T_DoorRotation`)
    (:`Update`
      (`SceneComponent.K2_SetRelativeRotation` (`self.ContDoor`) (`KismetMathLibrary.RLerp` (`self.RotationStart`) (`self.RotationEnd`) _rotatortrack) false false))))

(fn `UserConstructionScript`)