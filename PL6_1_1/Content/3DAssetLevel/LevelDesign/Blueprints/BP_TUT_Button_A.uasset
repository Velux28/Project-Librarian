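; BP_TUT_Button_A is a tutorial button the player interacts with to trigger level events.
; On its first interaction only, guarded by a DoOnce, it plays a click sound.
; It then activates the BP_TUT_DynamicGlass transparency and, after a short delay, starts the BP_TUT_CanDispenser, finding both by class lookup.
; LookAt returns the "Button" label for the interaction system.
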(event `/Game/BP_BO/Inventory/BPI_InteractInterface.InteractWith`
  (params (PlayerCharacter :type "/Game/BP_BO/PlayerCharacter/BP_TPCharacter Object Reference"))
  (`/Engine/EditorBlueprintResources/StandardMacros.DoOnce` false
    (:`Completed`
      ;[1 0 0] SUONO DA CAMBIARE
      (`GameplayStatics.PlaySoundAtLocation` "/Game/BO_Custom/SOUNDS/TUT_LEV/SE_ButtonClick.SE_ButtonClick" (`SceneComponent.RelativeLocation` (`self.Button`)) (struct) 1.0 1.0 0.0 null null null null)
      (`|ExecutionSequence`
        (:`then_0`
          ;[1 1 1] Attivazione trasparenza vetro
          (bind _returnvalue (`GameplayStatics.GetActorOfClass` "/Game/3DAssetLevel/LevelDesign/Blueprints/BP_TUT_DynamicGlass.BP_TUT_DynamicGlass_C"))
          (`/Game/3DAssetLevel/LevelDesign/Blueprints/BP_TUT_DynamicGlass.GlassActivation` _returnvalue))
        (:`then_1`
          (`KismetSystemLibrary.Delay` 2.0)
          (bind _returnvalue_2 (`GameplayStatics.GetActorOfClass` "/Game/3DAssetLevel/LevelDesign/Blueprints/BP_TUT_CanDispenser.BP_TUT_CanDispenser_C"))
          (`/Game/3DAssetLevel/LevelDesign/Blueprints/BP_TUT_CanDispenser.Dispenser Activated` _returnvalue_2))))))

(fn `LookAt`
  (returns (Message :type Text))
  (return "Button"))

(fn `UserConstructionScript`)