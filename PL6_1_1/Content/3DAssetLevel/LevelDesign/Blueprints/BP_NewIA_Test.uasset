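; BP_NewIA_Test is a test actor that moves a NewRobot component along a spline path.
; Each Tick advances the distance by SplineSpeed scaled by delta time and applies the spline's local location and rotation to the robot, keeping its scale.
; A Box overlap destroys the trigger and sets CanMove, but the branch reading that flag is disconnected, so movement does not wait for the trigger.
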(event `self.Box.OnComponentBeginOverlap`
  (params (OverlappedComponent :type "PrimitiveComponent Object Reference") (OtherActor :type "Actor Object Reference") (OtherComp :type "PrimitiveComponent Object Reference") (OtherBodyIndex :type Integer) (bFromSweep :type Boolean) (SweepResult :type "HitResult Structure (by ref)"))
  (`ActorComponent.K2_DestroyComponent` (`self.Box`))
  (set `self.CanMove` true))

(event `self.ReceiveTick`
  (params (DeltaSeconds :type "Float (single-precision)"))
  (bind (_returnvalue_location _returnvalue_rotation) (`KismetMathLibrary.BreakTransform` (`SplineComponent.GetTransformAtDistanceAlongSpline` (`self.Spline`) (`self.Distance Along Spline`) "Local" false)))
  (set `self.Distance Along Spline` (+ (* DeltaSeconds (`self.Spline Speed`)) (`self.Distance Along Spline`)))
  (`SceneComponent.K2_SetRelativeTransform` (`self.NewRobot`) (`KismetMathLibrary.MakeTransform` _returnvalue_location _returnvalue_rotation (`SceneComponent.RelativeScale3D` (`self.NewRobot`))) false false))

(fn `UserConstructionScript`)