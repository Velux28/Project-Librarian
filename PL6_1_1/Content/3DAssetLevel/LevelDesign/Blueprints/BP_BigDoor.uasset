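; BP_BigDoor is a two-panel sliding door that opens when something overlaps its Box trigger and closes when the overlap ends.
; Two timelines drive the relative locations of DoorMesh1 and DoorMesh2, playing to open and reversing to close.
; IsSFXPlayable limits the opening sound at DoorFrame until a timeline finishes.
; The closing sound node is disconnected, so closing is silent.
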(event `self.Box.OnComponentBeginOverlap`
  (params (OverlappedComponent :type "PrimitiveComponent Object Reference") (OtherActor :type "Actor Object Reference") (OtherComp :type "PrimitiveComponent Object Reference") (OtherBodyIndex :type Integer) (bFromSweep :type Boolean) (SweepResult :type "HitResult Structure (by ref)"))
  (if (`self.IsSFXPlayable`)
    (`GameplayStatics.PlaySoundAtLocation` "/Game/SoundDesign/Environment_SFX/SoundCues/SC_SlidingDoor_A.SC_SlidingDoor_A" (`SceneComponent.K2_GetComponentLocation` (`self.DoorFrame`)) (struct) 1.0 1.0 0.0 null null null null))
  (`|ExecutionSequence`
    (:`then_0`
      (set `self.IsSFXPlayable` false)
      (bind (_direction _door1track) (`Timeline|T_Door1` :!label _label)
        (:`Update`
          (`SceneComponent.K2_SetRelativeLocation` (`self.DoorMesh_1`) _door1track false false))
        (:`Finished`
          (set `self.IsSFXPlayable` true :!label _label_2))))
    (:`then_1`
      (bind (_direction_2 _door2track) (`Timeline|T_Door2` :!label _label_3)
        (:`Update`
          (`SceneComponent.K2_SetRelativeLocation` (`self.DoorMesh_2`) _door2track false false))
        (:`Finished`
          (goto _label_2))))))

(event `self.Box.OnComponentEndOverlap`
  (params (OverlappedComponent :type "PrimitiveComponent Object Reference") (OtherActor :type "Actor Object Reference") (OtherComp :type "PrimitiveComponent Object Reference") (OtherBodyIndex :type Integer))
  (if (`self.IsSFXPlayable`)
    _
    (else
      _))
  (`|ExecutionSequence`
    (:`then_0`
      (set `self.IsSFXPlayable` false)
      (goto _label :!via `Reverse`))
    (:`then_1`
      (goto _label_3 :!via `Reverse`))))

(fn `UserConstructionScript`)