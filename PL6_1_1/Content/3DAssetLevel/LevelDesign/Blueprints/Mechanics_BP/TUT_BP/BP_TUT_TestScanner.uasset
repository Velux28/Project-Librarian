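; Tutorial scanner prop that plays a timed arm-and-scan sequence, with placeholder crouch and hold-breath scans.
; TutorialStart moves Arm1 along a timeline while parallel delayed branches briefly show each scan mesh and swap its optic material from glass to laser.
; After the second scan it finds the BP_TUT_LaserLocks_A actor and calls QuizComplete on it.
; The sequence runs purely on delays, with no player detection.
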(event `self.ReceiveBeginPlay`
  (`SceneComponent.SetVisibility` (`self.Scan1`) false false)
  (`SceneComponent.SetVisibility` (`self.Scan2`) false false))

(event `TutorialStart`
  ;[1 1 1] ARM SETUM MOVEMENT
  (`KismetSystemLibrary.Delay` 1.0)
  (`|ExecutionSequence`
    (:`then_0`
      (bind (_direction _arm1track) (`Timeline|T_Arm1`)
        (:`Update`
          (`SceneComponent.K2_SetRelativeLocation` (`self.Arm1`) _arm1track false false))))
    (:`then_1`
      (`KismetSystemLibrary.Delay` 4.5)
      ;[1 1 1] SCAN CROUCH [PLACEHOLDER]
      (`PrimitiveComponent.SetMaterial` (`self.Optical1`) 0 "/Engine/VREditor/LaserPointer/LaserPointerMaterial.LaserPointerMaterial")
      (`SceneComponent.SetVisibility` (`self.Scan1`) true false)
      (`KismetSystemLibrary.Delay` 3.0)
      (`SceneComponent.SetVisibility` (`self.Scan1`) false false)
      (`PrimitiveComponent.SetMaterial` (`self.Optical1`) 0 "/Game/3DAssetLevel/LevelDesign/Materials/GridMats/MI_Grid_Glass.MI_Grid_Glass"))
    (:`then_2`
      (`KismetSystemLibrary.Delay` 9.0)
      ;[1 1 1] SCAN HOLDBREATH [PLACEHOLDER]
      (`PrimitiveComponent.SetMaterial` (`self.Optical2`) 0 "/Engine/VREditor/LaserPointer/TranslucentLaserPointerMaterialInst_BLUE.TranslucentLaserPointerMaterialInst_BLUE")
      (`SceneComponent.SetVisibility` (`self.Scan2`) true false)
      (`KismetSystemLibrary.Delay` 3.0)
      (`SceneComponent.SetVisibility` (`self.Scan2`) false false)
      (`PrimitiveComponent.SetMaterial` (`self.Optical2`) 0 "/Game/3DAssetLevel/LevelDesign/Materials/GridMats/MI_Grid_Glass.MI_Grid_Glass")
      (`KismetSystemLibrary.Delay` 1.5)
      (bind _returnvalue (`GameplayStatics.GetActorOfClass` "/Game/3DAssetLevel/LevelDesign/Blueprints/Mechanics_BP/TUT_BP/BP_TUT_LaserLocks_A.BP_TUT_LaserLocks_A_C"))
      (`/Game/3DAssetLevel/LevelDesign/Blueprints/Mechanics_BP/TUT_BP/BP_TUT_LaserLocks_A.QuizComplete` _returnvalue))))

(fn `UserConstructionScript`)