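; Restroom lamp Blueprint that plays a scripted flicker-and-blackout when EV_BathTrigger is called.
; The event plays a flicker sound and briefly lights six rect lights, cuts them, then restores them after a pause, swapping the roof lamp's material to match and ending on a low-light look.
; A parallel delayed Sequence branch finds BP_Restroom_JS by class and calls its despawn event just after the lights go dark.
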(event `EV_BathTrigger`
  (`|ExecutionSequence`
    (:`then_0`
      (`GameplayStatics.PlaySoundAtLocation` "/Game/3DAssetLevel/NewRoom/Sound/165239-SFX-Flash-Flicker_Spin_1.165239-SFX-Flash-Flicker_Spin_1" (`SceneComponent.K2_GetComponentLocation` (`self.RoofLamp`)) (struct) 1.0 1.0 0.0 null null null null)
      (`SceneComponent.SetVisibility` (`self.RectLight`) true false)
      (`SceneComponent.SetVisibility` (`self.RectLight1`) true false)
      (`SceneComponent.SetVisibility` (`self.RectLight5`) true false)
      (`SceneComponent.SetVisibility` (`self.RectLight4`) true false)
      (`SceneComponent.SetVisibility` (`self.RectLight3`) true false)
      (`SceneComponent.SetVisibility` (`self.RectLight2`) true false)
      (`PrimitiveComponent.SetMaterial` (`self.RoofLamp`) 1 "/Game/C_MSF_Office/Materials/Trim/M_Trim_01_Plastic_White.M_Trim_01_Plastic_White")
      (`KismetSystemLibrary.Delay` 0.3)
      (`SceneComponent.SetVisibility` (`self.RectLight`) false false)
      (`SceneComponent.SetVisibility` (`self.RectLight1`) false false)
      (`SceneComponent.SetVisibility` (`self.RectLight5`) false false)
      (`SceneComponent.SetVisibility` (`self.RectLight4`) false false)
      (`SceneComponent.SetVisibility` (`self.RectLight3`) false false)
      (`SceneComponent.SetVisibility` (`self.RectLight2`) false false)
      (`PrimitiveComponent.SetMaterial` (`self.RoofLamp`) 1 "/Game/StarterContent/Materials/M_BLACK.M_BLACK")
      (`KismetSystemLibrary.Delay` 2.0)
      (`SceneComponent.SetVisibility` (`self.RectLight`) true false)
      (`SceneComponent.SetVisibility` (`self.RectLight1`) true false)
      (`SceneComponent.SetVisibility` (`self.RectLight5`) true false)
      (`SceneComponent.SetVisibility` (`self.RectLight4`) true false)
      (`SceneComponent.SetVisibility` (`self.RectLight3`) true false)
      (`SceneComponent.SetVisibility` (`self.RectLight2`) true false)
      (`PrimitiveComponent.SetMaterial` (`self.RoofLamp`) 1 "/Game/StarterContent/Materials/MI_LowLight.MI_LowLight"))
    (:`then_1`
      (`KismetSystemLibrary.Delay` 0.4)
      (bind _returnvalue (`GameplayStatics.GetActorOfClass` "/Game/3DAssetLevel/LevelDesign/Blueprints/Mechanics_BP/BP_RESTROOM/BP_Restroom_JS.BP_Restroom_JS_C"))
      (`/Game/3DAssetLevel/LevelDesign/Blueprints/Mechanics_BP/BP_RESTROOM/BP_Restroom_JS.EV_Despawn` _returnvalue))))

(fn `UserConstructionScript`)