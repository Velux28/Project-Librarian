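; BP_EmergencySwitch is an interactable switch that opens exit and container doors and wakes up an AI character.
; On Interactwith it calls OpenExit on its referenced door and OpenContainer on the BP_ContainerDoors actor found by class lookup.
; After a short delay it activates the referenced AI through ACAIActivator with the fixed-patrol behavior tree, noted as enabling AI hearing.
; Its LookAt function returns an empty string.
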(event `/Game/BP_BO/Inventory/BPI_InteractInterface.InteractWith`
  (params (PlayerCharacter :type "/Game/BP_BO/PlayerCharacter/BP_TPCharacter Object Reference"))
  (bind _doorref (`self.DoorRef`))
  (`|ExecutionSequence`
    (:`then_0`
      (`/Engine/EditorBlueprintResources/StandardMacros.IsValid` _doorref
        (:`Is Valid`
          (`/Game/3DAssetLevel/LevelDesign/Blueprints/Mechanics_BP/BP_VertDoor_EXIT.Open Exit` _doorref))))
    (:`then_1`
      (bind _returnvalue (`GameplayStatics.GetActorOfClass` "/Game/3DAssetLevel/LevelDesign/Blueprints/Mechanics_BP/BP_ContainerDoors.BP_ContainerDoors_C"))
      (`/Game/3DAssetLevel/LevelDesign/Blueprints/Mechanics_BP/BP_ContainerDoors.Open Container` _returnvalue))
    (:`then_2`
      (`KismetSystemLibrary.Delay` 3.0)
      ;[1 1 1] Attivazione Udito I.A.
      (`/Game/3DAssetLevel/LevelDesign/Blueprints/Mechanics_BP/AC_AIActivator.Activate AI` (`self.AC_AIActivator`) (`self.AI_Reference`) "/Game/BP_BO/ArtificialIntelligence/BT_NPC_FixedPatrol.BT_NPC_FixedPatrol"))))

(fn `LookAt`
  (returns (Message :type Text))
  (return ""))

(fn `UserConstructionScript`)