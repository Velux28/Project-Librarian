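; BP_NPC_Guard_B is a tutorial guard NPC that shows a dialogue line when the player character enters its trigger box.
; Overlap makes the NPCDialogue widget visible with Dialogue line "L01_SH_02" and the actor's object name as speaker, and leaving hides it.
; The nodes that fill the dialogue map and create the widget are unconnected, so this graph never initializes NPCDialogue itself.
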(event `self.ReceiveBeginPlay`)

(event `self.TriggerBox.OnComponentBeginOverlap`
  (params (OverlappedComponent :type "PrimitiveComponent Object Reference") (OtherActor :type "Actor Object Reference") (OtherComp :type "PrimitiveComponent Object Reference") (OtherBodyIndex :type Integer) (bFromSweep :type Boolean) (SweepResult :type "HitResult Structure (by ref)"))
  (bind _npcdialogue (`self.NPCDialogue`))
  (cast `/Game/BP_BO/PlayerCharacter/BP_TPCharacter` OtherActor)
  ;[1 1 1] Widget ClosedWay
  (`Widget.SetVisibility` (`self.NPCDialogue`) "Visible")
  (bind _returnvalue (`DialogueComponent.ShowDialogue` (`self.Dialogue`) "L01_SH_02"))
  (`/Game/UI/PlayerUI/Environment_UI/NPCs/W_HUD_NPCDialogue.Set Dialogue` _npcdialogue (`KismetTextLibrary.Conv_StringToText` _returnvalue))
  (`/Game/UI/PlayerUI/Environment_UI/NPCs/W_HUD_NPCDialogue.Set Speaker Name` _npcdialogue (`KismetTextLibrary.Conv_StringToText` (`KismetSystemLibrary.GetObjectName` self))))

(event `self.TriggerBox.OnComponentEndOverlap`
  (params (OverlappedComponent :type "PrimitiveComponent Object Reference") (OtherActor :type "Actor Object Reference") (OtherComp :type "PrimitiveComponent Object Reference") (OtherBodyIndex :type Integer))
  (cast `/Game/BP_BO/PlayerCharacter/BP_TPCharacter` OtherActor)
  ;[1 1 1] Widget ClosedWay
  (`Widget.SetVisibility` (`self.NPCDialogue`) "Hidden"))

(fn `UserConstructionScript`)