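; Tutorial guard NPC that starts a dialogue when the player character enters its trigger box and hides it on exit.
; SetDialogue extends the parent's version to show each line on the player controller's HUD.
; A timer on HandleDialogue advances lines by their duration, handing turns to the player character's own dialogue handler when flagged.
; SkipDialogue advances early while the guard speaks; the last key closes the widget.
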(event `self.ReceiveBeginPlay`)

(event `self.TriggerBox.OnComponentBeginOverlap`
  (params (OverlappedComponent :type "PrimitiveComponent Object Reference") (OtherActor :type "Actor Object Reference") (OtherComp :type "PrimitiveComponent Object Reference") (OtherBodyIndex :type Integer) (bFromSweep :type Boolean) (SweepResult :type "HitResult Structure (by ref)"))
  ;[1 1 1] Widget ClosedWay
  (bind _asbp_tpcharacter (cast `/Game/BP_BO/PlayerCharacter/BP_TPCharacter` OtherActor))
  (`self.HUD`
    (:`then`
      _)
    (:`else`
      (bind _asmy_player_controller (cast `/Game/BP_BO/PlayerCharacter/MyPlayerController` (`GameplayStatics.GetPlayerController` 0)))
      (set `self.HUD` (`/Game/BP_BO/PlayerCharacter/MyPlayerController.HUD` _asmy_player_controller))))
  (set `/Game/BP_BO/PlayerCharacter/BP_TPCharacter.As Base NPC` null _asbp_tpcharacter)
  (bind _returnvalue (`self.SetDialogue` (`self.DialogueKey`)))
  (`KismetSystemLibrary.K2_SetTimer` null "HandleDialogue" (`.DialogueDuration` (break `Dialogue` _returnvalue))))

(event `self.TriggerBox.OnComponentEndOverlap`
  (params (OverlappedComponent :type "PrimitiveComponent Object Reference") (OtherActor :type "Actor Object Reference") (OtherComp :type "PrimitiveComponent Object Reference") (OtherBodyIndex :type Integer))
  ;[1 1 1] Widget ClosedWay
  (cast `/Game/BP_BO/PlayerCharacter/BP_TPCharacter` OtherActor)
  (`/Game/UI/PlayerUI/Basic_UI/W_PlayerHUD.Deactivate Dialogue` (`self.HUD`)))

(event `self.SkipDialogue`
  (if (`self.IsGuardSpeaking`)
    (`self.HandleDialogue`)))

(fn `Deactivate Dialogue Widget`
  (`/Game/UI/PlayerUI/Basic_UI/W_PlayerHUD.Deactivate Dialogue` (`self.HUD`))
  (set `self.IsGuardSpeaking` false))

(fn `HandleDialogue`
  (bind _returnvalue (`GameplayStatics.GetPlayerCharacter` 0))
  (bind (_dialoguekey _nextdialoguekey _dialoguetext _bnextdialogueisplayer) (break `Dialogue` (`self.CurrNPCDialogue`)))
  (if (`self.IsGuardSpeaking`)
    (if (!= (`DialogueComponent.GetLastDialogueKey` (`self.NPCDialogues`)) (`.NextDialogueKey` (break `Dialogue` (`self.CurrNPCDialogue`))))
      (if _bnextdialogueisplayer
        (bind _asbp_tpcharacter (cast `/Game/BP_BO/PlayerCharacter/BP_TPCharacter` _returnvalue))
        (bind _dialogue (`/Game/BP_BO/PlayerCharacter/BP_TPCharacter.Set Dialogue` _asbp_tpcharacter _nextdialoguekey self))
        (`KismetSystemLibrary.K2_ClearTimer` null "HandleDialogue")
        (`KismetSystemLibrary.K2_SetTimer` _returnvalue "HandleDialogue" (`.DialogueDuration` (break `Dialogue` _dialogue)))
        (set `self.IsGuardSpeaking` false)
        (else
          (bind _returnvalue_2 (`self.SetDialogue` _nextdialoguekey))
          (`KismetSystemLibrary.K2_ClearTimer` null "HandleDialogue")
          (`KismetSystemLibrary.K2_SetTimer` null "HandleDialogue" (`.DialogueDuration` (break `Dialogue` _returnvalue_2)))))
      (else
        (`self.SetNextInteractionDialogueKey` "")
        (`self.Deactivate Dialogue Widget`)))))

(fn `SetDialogue`
  (params (_DialogueKey :type String))
  (returns (ReturnValue :type "Dialogue Structure"))
  (bind _returnvalue (`parent.SetDialogue` _DialogueKey))
  (`/Game/UI/PlayerUI/Basic_UI/W_PlayerHUD.Set Dialogue` :`self` (`self.HUD`) :`Speaker Name` (`KismetTextLibrary.Conv_StringToText` (`self.ActorName`)) :`Dialogue Text` (`KismetTextLibrary.Conv_StringToText` (`.DialogueText` (break `Dialogue` _returnvalue))))
  (set `self.IsGuardSpeaking` true)
  (return _returnvalue))

(fn `UserConstructionScript`)