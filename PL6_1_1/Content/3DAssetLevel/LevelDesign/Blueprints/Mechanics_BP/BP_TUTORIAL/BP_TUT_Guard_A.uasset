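; Tutorial guard NPC that holds a timed, skippable dialogue chain with the player, shown on the HUD.
; Its trigger box enables interaction; interacting starts the chain or skips to the next line, and leaving hides the dialogue.
; Function-name timers on guard or BP_TPCharacter advance lines, handing turns between speakers, while reaching the important line switches the next interaction's dialogue.
; Author comments flag that timer clearing on exit fails, letting the widget reopen.
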(event `self.ReceiveBeginPlay`
  ;[1 1 1] Setup delle variabili necessarie per il funzionamento
  (`KismetSystemLibrary.Delay` 0.2) ; Necessary to give enough time to TPCharacter to set up HUD,\notherwise it returns invalid later
  (bind _asbp_tpcharacter (cast `/Game/BP_BO/PlayerCharacter/BP_TPCharacter` (`GameplayStatics.GetPlayerCharacter` 0)))
  (set `self.HUD` (`/Game/BP_BO/PlayerCharacter/BP_TPCharacter.HUD` _asbp_tpcharacter))
  (bind _output_get (set `self.As BP TPCharacter` _asbp_tpcharacter))
  (set `/Game/BP_BO/PlayerCharacter/BP_TPCharacter.As Base NPC` self _output_get))

(event `self.TriggerBox.OnComponentBeginOverlap`
  (params (OverlappedComponent :type "PrimitiveComponent Object Reference") (OtherActor :type "Actor Object Reference") (OtherComp :type "PrimitiveComponent Object Reference") (OtherBodyIndex :type Integer) (bFromSweep :type Boolean) (SweepResult :type "HitResult Structure (by ref)"))
  ;[1 1 1] On Begin Overlap - Si può parlare con la Guardia = Risponde all'interazione
  (if (== OtherActor (`self.As BP TPCharacter`))
    (set `self.CanSpeak` true)))

(event `self.TriggerBox.OnComponentEndOverlap`
  (params (OverlappedComponent :type "PrimitiveComponent Object Reference") (OtherActor :type "Actor Object Reference") (OtherComp :type "PrimitiveComponent Object Reference") (OtherBodyIndex :type Integer))
  ;[1 1 1] On End Overlap -  Non si può più parlare con la guardia = Non risponde all'interazione
  (if (== OtherActor (`self.As BP TPCharacter`))
    (set `self.CanSpeak` false)
    ;[1 0.5 0] Questo funziona
    (`/Game/UI/PlayerUI/Basic_UI/W_PlayerHUD.Deactivate Dialogue` (`self.HUD`))
    ;[1 0 0] Questo non sembra funzionare.
    ; Quando esco dalla triggerbox il widget scompare, ma passato il tempo poi si riapre. Suppongo che il Clear Timer non stia operando come deve
    (set `self.CurrNPCDialogue` (struct))
    (if (`self.IsGuardSpeaking`)
      (`KismetSystemLibrary.K2_ClearTimer` null "HandleDialogue")
      (else
        (`KismetSystemLibrary.K2_ClearTimer` (`self.As BP TPCharacter`) "HandleDialogue")))))

(event `self.SkipDialogue`
  ;[1 1 1] Passo alla prossima linea di dialogo
  (if (`self.IsGuardSpeaking`)
    (`self.HandleDialogue`)
    (else
      (`/Game/BP_BO/PlayerCharacter/BP_TPCharacter.HandleDialogue` (`self.As BP TPCharacter`)))))

(event `/Game/BP_BO/Inventory/BPI_InteractInterface.InteractWith`
  (params (PlayerCharacter :type "/Game/BP_BO/PlayerCharacter/BP_TPCharacter Object Reference"))
  (bind _currnpcdialogue_dialoguekey (break `Dialogue` (`self.CurrNPCDialogue`)))
  ;[1 1 1] Interazione - a condizione che possa parlare (attivato/disattivato dalle Triggerbox) - controlla la dialogue key:
  ; - se vuota inizia il dialogo
  ; - se non vuota > [Event Skip Dialogue]
  (if (`self.CanSpeak`)
    (if (`KismetStringLibrary.IsEmpty` _currnpcdialogue_dialoguekey)
      ;[1 1 1] If is the first Interaction or the dialogue chain is over, setup first dialogue of the chain
      (bind _returnvalue (`self.SetDialogue` (`self.DialogueKey`)))
      (`KismetSystemLibrary.K2_SetTimer` null "HandleDialogue" (`.DialogueDuration` (break `Dialogue` _returnvalue)))
      (else
        ;[1 1 1] If the chain isnt over pass to the next dialogue
        (`self.SkipDialogue`)))))

(fn `Check IF Interactable`
  (returns (`Is NOT Interactable` :type Boolean))
  (return false))

(fn `Deactivate Dialogue Widget`
  (`/Game/UI/PlayerUI/Basic_UI/W_PlayerHUD.Deactivate Dialogue` (`self.HUD`))
  (set `self.IsGuardSpeaking` false))

(fn `HandleDialogue`
  (bind (_dialoguekey _nextdialoguekey) (break `Dialogue` (`self.CurrNPCDialogue`)))
  (bind (_dialoguekey_2 _nextdialoguekey_2 _dialoguetext _bnextdialogueisplayer) (break `Dialogue` (`self.CurrNPCDialogue`)))
  (if (`self.IsGuardSpeaking`)
    (if (!= (`DialogueComponent.GetLastDialogueKey` (`self.NPCDialogues`)) _nextdialoguekey)
      (if (not (!= _nextdialoguekey (`self.ImportantDialogueKey`)))
        ;[1 1 1 1 13] If the important dialogue is displayed, change next dialogue to the recap dialogue
        (`self.SetNextInteractionDialogueKey` "") ; "DialogueKey" of the function, must be set only \nif we want a different Dialogue on the third interaction. \nThis function does "DialogueKey" (of the blueprint) ="NextInteractionDialogueKey"\n and does "NextInteractionDialogueKey"="DialogueKey" (of the function), \nif "DialogueKey" (of the function) is empty the second assign is skipped
      )
      (if _bnextdialogueisplayer
        ;[1 1 1] Setup next player dialogue
        (bind _dialogue (`/Game/BP_BO/PlayerCharacter/BP_TPCharacter.Set Dialogue` (`self.As BP TPCharacter`) _nextdialoguekey_2 self))
        (`KismetSystemLibrary.K2_ClearTimer` null "HandleDialogue")
        (`KismetSystemLibrary.K2_SetTimer` (`self.As BP TPCharacter`) "HandleDialogue" (`.DialogueDuration` (break `Dialogue` _dialogue)))
        (set `self.IsGuardSpeaking` false)
        (else
          ;[1 1 1] Setup next guard dialogue
          (bind _returnvalue (`self.SetDialogue` _nextdialoguekey_2))
          (`KismetSystemLibrary.K2_ClearTimer` null "HandleDialogue")
          (`KismetSystemLibrary.K2_SetTimer` null "HandleDialogue" (`.DialogueDuration` (break `Dialogue` _returnvalue)))))
      (else
        ;[1 1 1] If this was the last dialogue of the chain  deactivate widget
        (`self.Deactivate Dialogue Widget`)
        (set `self.CurrNPCDialogue` (struct))))))

(fn `SetDialogue`
  (params (_DialogueKey :type String))
  (returns (ReturnValue :type "Dialogue Structure"))
  (bind _returnvalue (`parent.SetDialogue` _DialogueKey))
  (`/Game/UI/PlayerUI/Basic_UI/W_PlayerHUD.Set Dialogue` (`self.HUD`) (`KismetTextLibrary.Conv_StringToText` (`self.ActorName`)) (`KismetTextLibrary.Conv_StringToText` (`.DialogueText` (break `Dialogue` _returnvalue))) (`self.SpeakerNameColor`))
  (set `self.IsGuardSpeaking` true)
  (return _returnvalue))

(fn `UserConstructionScript`)