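; BP_TUT_LaserLocks_B is a tutorial level mechanic that switches a pair of laser lock barriers on and off.
; Both locks start hidden without collision, then become visible and solid when something overlaps the trigger, which destroys itself to fire once.
; A QuizComplete event hides them and disables their collision again.
; The test scanner lookup after activation feeds nothing, and the TutorialStart call is disconnected.
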(event `self.ReceiveBeginPlay`
  ;[1 1 1] RoomSetup
  (`SceneComponent.SetVisibility` (`self.LaserLock_3`) false false)
  (`SceneComponent.SetVisibility` (`self.LaserLock_2`) false false)
  (`PrimitiveComponent.SetCollisionEnabled` (`self.LaserLock_3`) "NoCollision")
  (`PrimitiveComponent.SetCollisionEnabled` (`self.LaserLock_2`) "NoCollision"))

(event `self.LockTrigger.OnComponentBeginOverlap`
  (params (OverlappedComponent :type "PrimitiveComponent Object Reference") (OtherActor :type "Actor Object Reference") (OtherComp :type "PrimitiveComponent Object Reference") (OtherBodyIndex :type Integer) (bFromSweep :type Boolean) (SweepResult :type "HitResult Structure (by ref)"))
  ;[1 1 1] LaserLocks Activation
  (`ActorComponent.K2_DestroyComponent` (`self.LockTrigger`))
  (`SceneComponent.SetVisibility` (`self.LaserLock_3`) true false)
  (`SceneComponent.SetVisibility` (`self.LaserLock_2`) true false)
  (`PrimitiveComponent.SetCollisionEnabled` (`self.LaserLock_3`) "QueryAndPhysics")
  (`PrimitiveComponent.SetCollisionEnabled` (`self.LaserLock_2`) "QueryAndPhysics")
  (`GameplayStatics.GetActorOfClass` "/Game/3DAssetLevel/LevelDesign/Blueprints/Mechanics_BP/BP_TUTORIAL/BP_TUT_TestScanner.BP_TUT_TestScanner_C"))

(event `QuizComplete`
  ;[1 1 1] LaserLocks Deactivation
  (`SceneComponent.SetVisibility` (`self.LaserLock_3`) false false)
  (`SceneComponent.SetVisibility` (`self.LaserLock_2`) false false)
  (`PrimitiveComponent.SetCollisionEnabled` (`self.LaserLock_3`) "NoCollision")
  (`PrimitiveComponent.SetCollisionEnabled` (`self.LaserLock_2`) "NoCollision"))

(fn `UserConstructionScript`)