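; Tutorial test-window actor that stages a lesson when the player enters a one-shot LockTrigger.
; The trigger activates an AI and laser barriers with sound, then timelines dim lamp emissives and lights, fade the glass panel without collision, and show a HUD widget.
; TUT_Complete, called by BP_TUT_CanTarget, reverses this, with a TutorialIsOver flag keeping glass collision on, and deactivates the AI after a delay.
; GlassActivation is an empty leftover from the former button trigger.
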(event `self.ReceiveBeginPlay`
  (bind _returnvalue (`|CreateWidget` "/Game/UI/PlayerUI/Tutorial_UI/MnK_TUT/W_HUD_TUT_Test_Mnk.W_HUD_TUT_Test_Mnk_C"))
  (bind _output_get (set `self.Widget` _returnvalue))
  (`UserWidget.AddToViewport` _output_get 0)
  (`Widget.SetVisibility` _output_get "Hidden"))

(event `self.LockTrigger.OnComponentBeginOverlap`
  (params (OverlappedComponent :type "PrimitiveComponent Object Reference") (OtherActor :type "Actor Object Reference") (OtherComp :type "PrimitiveComponent Object Reference") (OtherBodyIndex :type Integer) (bFromSweep :type Boolean) (SweepResult :type "HitResult Structure (by ref)"))
  (bind _glasspanel (`self.GlassPanel`))
  ;[1 1 1] Attivazione dei Blocchi Laser
  (if (== OtherActor (`GameplayStatics.GetPlayerCharacter` 0))
    (`/Game/BP_BO/ArtificialIntelligence/AC_AIActivator.Activate AI` (`self.AC_AIActivator`) (`self.AI to Activate`) "/Game/BP_BO/ArtificialIntelligence/BT_NPC.BT_NPC")
    (`ActorComponent.K2_DestroyComponent` (`self.LockTrigger`))
    (`|ExecutionSequence`
      (:`then_0`
        (`SceneComponent.SetVisibility` (`self.PanelDX`) true false)
        (`SceneComponent.SetVisibility` (`self.LsrDXUp`) true false)
        (`SceneComponent.SetVisibility` (`self.LsrDXDown`) true false)
        (`SceneComponent.SetVisibility` (`self.PanelSX`) true false)
        (`SceneComponent.SetVisibility` (`self.LsrSXUp`) true false)
        (`SceneComponent.SetVisibility` (`self.LsrSXDwon`) true false)
        (`PrimitiveComponent.SetCollisionEnabled` (`self.PanelDX`) "QueryAndPhysics")
        (`PrimitiveComponent.SetCollisionEnabled` (`self.PanelSX`) "QueryAndPhysics")
        ;[1 1 1] Dimming dell'emissive dei materiali
        (`|ExecutionSequence`
          (:`then_0`
            (bind _returnvalue (`PrimitiveComponent.CreateDynamicMaterialInstance` (`self.StaticMesh`) 0 "/Game/3DAssetLevel/3DArt/Materials/MaterialInstances/Roof_OvalLamp/MI_LuceOvale.MI_LuceOvale" "None"))
            (bind (_direction _newtrack_0) (`Timeline|Timeline_0` :!label _label) ; Scala l'emissive delle lampade tra 100 e 5 in 1.25 secondi
              (:`Update`
                (`|ExecutionSequence`
                  (:`then_0`
                    (`MaterialInstanceDynamic.SetScalarParameterValue` _returnvalue "Emissive" _newtrack_0))
                  (:`then_1`
                    (`MaterialInstanceDynamic.SetScalarParameterValue` (stale _returnvalue_2) "Emissive" _newtrack_0))
                  (:`then_2`
                    (`MaterialInstanceDynamic.SetScalarParameterValue` (stale _returnvalue_3) "Emissive" _newtrack_0)
                    ;[1 1 1] Dimming delle Luci
                    (bind (_direction_2 _newtrack_0_2) (`Timeline|Light Dim On`) ; Scala la Intensity delle luci tra 75 e 20 lumens in 1.25 secondi
                      (:`Update`
                        (`LightComponent.SetIntensity` (`self.RectLight`) _newtrack_0_2)
                        (`LightComponent.SetIntensity` (`self.RectLight1`) _newtrack_0_2)
                        (`LightComponent.SetIntensity` (`self.RectLight2`) _newtrack_0_2)
                        (`/Engine/EditorBlueprintResources/StandardMacros.DoOnce` false
                          (:`Completed`
                            ;[1 1 1] Slider opacità e disattivazione collisioni nel vetro; comparsa Widget Tutorial
                            (`|ExecutionSequence`
                              (:`then_0`
                                (bind (_direction_3 _opacityfade) (`Timeline|T_OpacityFade` :!label _label_2)
                                  (:`Update`
                                    (`MeshComponent.SetScalarParameterValueOnMaterials` _glasspanel "Opacity" _opacityfade)
                                    (if (not (`self.Tutorial is over`))
                                      (`PrimitiveComponent.SetCollisionEnabled` _glasspanel "NoCollision")))))
                              (:`then_1`
                                (`Widget.SetVisibility` (`self.Widget`) "Visible"))))))))))))
          (:`then_1`
            (bind _returnvalue_2 (`PrimitiveComponent.CreateDynamicMaterialInstance` (`self.StaticMesh1`) 0 "/Game/3DAssetLevel/3DArt/Materials/MaterialInstances/Roof_OvalLamp/MI_LuceOvale.MI_LuceOvale" "None"))
            (goto _label))
          (:`then_2`
            (bind _returnvalue_3 (`PrimitiveComponent.CreateDynamicMaterialInstance` (`self.StaticMesh2`) 0 "/Game/3DAssetLevel/3DArt/Materials/MaterialInstances/Roof_OvalLamp/MI_LuceOvale.MI_LuceOvale" "None"))
            (goto _label))))
      (:`then_1`
        ;[0.6519 0 1] LASER SFX
        (`KismetSystemLibrary.Delay` 0.2)
        (`GameplayStatics.PlaySound2D` null 0.1 1.0 0.0 "/Game/BO_Custom/SOUNDS/TUT_LEV/Cues/CONC_Environment.CONC_Environment" null false)
        (`ActorComponent.Activate` (`self.LaserBarrierSFX`) false)
        (`ActorComponent.Activate` (`self.LaserBarrierSFX2_0`) false)))))

(event `GlassActivation`
  ;[1 1 1] Il richiamo del bottone è stato dichiarato controintuitivo. Parte tutto con la TriggerBox ora
)

(event `TUT_Complete`
  ;[1 1 1] revert del dimming dell'emissive dei materiali
  (`|ExecutionSequence`
    (:`then_0`
      (bind _returnvalue (`PrimitiveComponent.CreateDynamicMaterialInstance` (`self.StaticMesh`) 0 "/Game/3DAssetLevel/3DArt/Materials/MaterialInstances/Roof_OvalLamp/MI_LuceOvale.MI_LuceOvale" "None"))
      (bind (_direction _newtrack_0) (`Timeline|Timeline_1` :!label _label_3) ; Scala l'emissive delle lampade tra 5 e 100 in 1.25 secondi
        (:`Update`
          (`|ExecutionSequence`
            (:`then_0`
              (`MaterialInstanceDynamic.SetScalarParameterValue` _returnvalue "Emissive" _newtrack_0))
            (:`then_1`
              (`MaterialInstanceDynamic.SetScalarParameterValue` (stale _returnvalue_2) "Emissive" _newtrack_0))
            (:`then_2`
              (`MaterialInstanceDynamic.SetScalarParameterValue` (stale _returnvalue_3) "Emissive" _newtrack_0)
              ;[1 1 1] Fine del Tutorial e Fine del Dimming delle Luci
              (bind (_direction_2 _newtrack_0_2) (`Timeline|Light Dim Off`) ; Scala la Intensity delle luci tra 20 e 75 lumens in 1.25 secondi
                (:`Update`
                  (`LightComponent.SetIntensity` (`self.RectLight`) _newtrack_0_2)
                  (`LightComponent.SetIntensity` (`self.RectLight1`) _newtrack_0_2)
                  (`LightComponent.SetIntensity` (`self.RectLight2`) _newtrack_0_2)
                  (`|ExecutionSequence`
                    (:`then_0`
                      ;[1 1 1] A tutorial finito, disattiva visibilità e riattiva collisioni nel vetro
                      (set `self.Tutorial is over` true) ; Impedisco di spegnere nuovamente le collisioni del vetro
                      (`PrimitiveComponent.SetCollisionEnabled` (`self.GlassPanel`) "QueryAndPhysics")
                      (`ActorComponent.Deactivate` (`self.LaserBarrierSFX`))
                      (`ActorComponent.Deactivate` (`self.LaserBarrierSFX2_0`))
                      (goto _label_2 :!via `Reverse`))
                    (:`then_1`
                      ;[1 1 1] Spegnimento dei Blocchi Laser e scomparsa Widget Tutorial
                      (`SceneComponent.SetVisibility` (`self.PanelDX`) false false)
                      (`SceneComponent.SetVisibility` (`self.LsrDXUp`) false false)
                      (`SceneComponent.SetVisibility` (`self.LsrDXDown`) false false)
                      (`SceneComponent.SetVisibility` (`self.PanelSX`) false false)
                      (`SceneComponent.SetVisibility` (`self.LsrSXUp`) false false)
                      (`SceneComponent.SetVisibility` (`self.LsrSXDwon`) false false)
                      (`PrimitiveComponent.SetCollisionEnabled` (`self.PanelDX`) "NoCollision")
                      (`PrimitiveComponent.SetCollisionEnabled` (`self.PanelSX`) "NoCollision")
                      ;[1 1 1] Slider opacità e disattivazione collisioni nel vetro; comparsa Widget Tutorial
                      (`Widget.SetVisibility` (`self.Widget`) "Hidden")
                      ;;[1 0.84 0] If deactivate too early the scan laser never disaperars, an option is to never deactivate the tutorialAI
                      (`KismetSystemLibrary.Delay` 10.0)
                      (`/Game/BP_BO/ArtificialIntelligence/AC_AIActivator.De-activate AI` (`self.AC_AIActivator`) (`self.AI to Activate`)))))))))))
    (:`then_1`
      (bind _returnvalue_2 (`PrimitiveComponent.CreateDynamicMaterialInstance` (`self.StaticMesh1`) 0 "/Game/3DAssetLevel/3DArt/Materials/MaterialInstances/Roof_OvalLamp/MI_LuceOvale.MI_LuceOvale" "None"))
      (goto _label_3))
    (:`then_2`
      (bind _returnvalue_3 (`PrimitiveComponent.CreateDynamicMaterialInstance` (`self.StaticMesh2`) 0 "/Game/3DAssetLevel/3DArt/Materials/MaterialInstances/Roof_OvalLamp/MI_LuceOvale.MI_LuceOvale" "None"))
      (goto _label_3))))

(fn `Emissive Dimmer`
  (returns (ReturnValue :type "MaterialInstanceDynamic Object Reference") (ReturnValue2 :type "MaterialInstanceDynamic Object Reference") (ReturnValue3 :type "MaterialInstanceDynamic Object Reference"))
  (`|ExecutionSequence`
    (:`then_0`
      (bind _returnvalue (`PrimitiveComponent.CreateDynamicMaterialInstance` (`self.StaticMesh`) 0 "/Game/3DAssetLevel/3DArt/Materials/MaterialInstances/Roof_OvalLamp/MI_LuceOvale.MI_LuceOvale" "None")))
    (:`then_1`
      (bind _returnvalue_2 (`PrimitiveComponent.CreateDynamicMaterialInstance` (`self.StaticMesh1`) 0 "/Game/3DAssetLevel/3DArt/Materials/MaterialInstances/Roof_OvalLamp/MI_LuceOvale.MI_LuceOvale" "None")))
    (:`then_2`
      (bind _returnvalue_3 (`PrimitiveComponent.CreateDynamicMaterialInstance` (`self.StaticMesh2`) 0 "/Game/3DAssetLevel/3DArt/Materials/MaterialInstances/Roof_OvalLamp/MI_LuceOvale.MI_LuceOvale" "None"))))
  (return _returnvalue _returnvalue_2 _returnvalue_3))

(fn `NewFunction_0`
  (returns (ReturnValue :type "MaterialInstanceDynamic Object Reference") (ReturnValue2 :type "MaterialInstanceDynamic Object Reference") (ReturnValue3 :type "MaterialInstanceDynamic Object Reference"))
  (`|ExecutionSequence`
    (:`then_0`
      (bind _returnvalue (`PrimitiveComponent.CreateDynamicMaterialInstance` (`self.StaticMesh`) 0 "/Game/3DAssetLevel/3DArt/Materials/MaterialInstances/Roof_OvalLamp/MI_LuceOvale.MI_LuceOvale" "None")))
    (:`then_1`
      (bind _returnvalue_2 (`PrimitiveComponent.CreateDynamicMaterialInstance` (`self.StaticMesh1`) 0 "/Game/3DAssetLevel/3DArt/Materials/MaterialInstances/Roof_OvalLamp/MI_LuceOvale.MI_LuceOvale" "None"))
      (return _returnvalue_2 _returnvalue (stale _returnvalue_3)))
    (:`then_2`
      (bind _returnvalue_3 (`PrimitiveComponent.CreateDynamicMaterialInstance` (`self.StaticMesh2`) 0 "/Game/3DAssetLevel/3DArt/Materials/MaterialInstances/Roof_OvalLamp/MI_LuceOvale.MI_LuceOvale" "None")))))

(fn `NewFunction_1`
  (params (self2 :type "MaterialInstanceDynamic Object Reference") (self3 :type "MaterialInstanceDynamic Object Reference") (self4 :type "MaterialInstanceDynamic Object Reference"))
  (`|ExecutionSequence`
    (:`then_0`
      (`MaterialInstanceDynamic.SetScalarParameterValue` self2 "Emissive" 20.0))
    (:`then_1`
      (`MaterialInstanceDynamic.SetScalarParameterValue` self3 "Emissive" 20.0))
    (:`then_2`
      (`MaterialInstanceDynamic.SetScalarParameterValue` self4 "Emissive" 20.0))))

(fn `UserConstructionScript`)