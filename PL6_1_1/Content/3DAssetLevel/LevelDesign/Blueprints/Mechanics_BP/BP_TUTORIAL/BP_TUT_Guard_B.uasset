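; Tutorial guard Blueprint that shows guard dialogue about a hallway closed for maintenance, with scaffolding to pass under.
; BeginPlay fills its Dialogue member with two keyed lines and adds a W_GuardDialogue_B widget to the viewport.
; When BP_TPCharacter enters TriggerBox, it adds another such widget and prints the second line via ShowDialogue.
; Leaving the box hides that overlap widget without removing it.
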(event `self.ReceiveBeginPlay`
  (`DialogueComponent.FillDialogue` (`self.Dialogue`) (`|MakeMap` "L01_SH_01" "Sorry Sir, this hallway is currently under maintenance. Please wait until the repair operations have ended, or pass under the scaffolding. The Corporation rejects any responsibilities if you choose to do so" "L01_SH_02" "“Even though I am not a robot I am able to pass under a scaffolding”"))
  (bind _returnvalue (`|CreateWidget` "/Game/UI/PlayerUI/Environment_UI/NPCs/W_GuardDialogue_B.W_GuardDialogue_B_C"))
  (`UserWidget.AddToViewport` _returnvalue 0))

(event `self.TriggerBox.OnComponentBeginOverlap`
  (params (OverlappedComponent :type "PrimitiveComponent Object Reference") (OtherActor :type "Actor Object Reference") (OtherComp :type "PrimitiveComponent Object Reference") (OtherBodyIndex :type Integer) (bFromSweep :type Boolean) (SweepResult :type "HitResult Structure (by ref)"))
  (cast `/Game/BP_BO/PlayerCharacter/BP_TPCharacter` OtherActor)
  ;[1 1 1] Widget ClosedWay
  (bind _returnvalue (`|CreateWidget` "/Game/UI/PlayerUI/Environment_UI/NPCs/W_GuardDialogue_B.W_GuardDialogue_B_C"))
  (`UserWidget.AddToViewport` _returnvalue 0)
  (bind _returnvalue_2 (`DialogueComponent.ShowDialogue` (`self.Dialogue`) "L01_SH_02"))
  (`KismetSystemLibrary.PrintString` _returnvalue_2))

(event `self.TriggerBox.OnComponentEndOverlap`
  (params (OverlappedComponent :type "PrimitiveComponent Object Reference") (OtherActor :type "Actor Object Reference") (OtherComp :type "PrimitiveComponent Object Reference") (OtherBodyIndex :type Integer))
  (cast `/Game/BP_BO/PlayerCharacter/BP_TPCharacter` OtherActor)
  ;[1 1 1] Widget ClosedWay
  (`Widget.SetVisibility` (stale `self.TriggerBox.OnComponentBeginOverlap` _returnvalue) "Hidden"))

(fn `UserConstructionScript`)