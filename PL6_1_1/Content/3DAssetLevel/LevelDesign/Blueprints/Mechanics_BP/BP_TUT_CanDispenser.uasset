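; Tutorial can dispenser that slides into place and drops an environmental can for the player.
; On DispenserActivated a timeline moves the base, then after a delay it spawns BP_EnvCan and animates the panel with a second timeline.
; Lattinasprecata re-runs the spawn and panel steps for a wasted can; the inventory check is only noted in a comment.
; TutorialAEnded reverses the base movement but is marked inactive.
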(event `Dispenser Activated`
  (`|ExecutionSequence`
    (:`then_0`
      ;[1 1 1] Animazione Dispenser
      (bind (_direction _newtrack_2) (`Timeline|T_DispenserMovement` :!label _label)
        (:`Update`
          (`SceneComponent.K2_SetRelativeLocation` (`self.DispenserBase`) _newtrack_2 false false))))
    (:`then_1`
      (`KismetSystemLibrary.Delay` 4.0)
      ;[1 0.2543 0] Spawn EnvCan [TEMPORANEO]
      (`|SpawnActorFromClass` "/Game/BP_BO/Inventory/Items/BP_EnvCan.BP_EnvCan_C" (`KismetMathLibrary.MakeTransform` (65.0 50.0 -40.0) (struct :`Yaw` 90.0 :`Roll` -180.0) (1.5 1.5 1.5)) "AlwaysSpawn" "OverrideRootScale" null null :!label _label_2)
      (`KismetSystemLibrary.Delay` 1.0)
      ;[1 1 1] Apertura/chiusura sportello
      (bind (_direction_2 _panelmovement) (`Timeline|T_PanelOpening`)
        (:`Update`
          (`SceneComponent.K2_SetRelativeLocation` (`self.DispenserPanel`) (`KismetMathLibrary.MakeVector` 110.0 0.0 _panelmovement) false false))))))

(event `Tutorial A Ended`
  ;[1 0.02604 0.02604] NON ATTIVO
  (goto _label :!via `Reverse`))

(event `Lattina sprecata`
  ;[1 0 0] Controllare che il player non abbia già una o più lattine nell'inventario, se ne ha meno di una spawnare quella nuova
  (goto _label_2))

(fn `UserConstructionScript`)