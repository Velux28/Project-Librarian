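; BP_CCTV_LevelEnd is a trigger actor that ends the CCTV section with a fainting cutscene and opens MAP_Level_1.
; Its Trigger has collision disabled at BeginPlay until the ActivateEnd event enables it.
; The first overlap, with no check on the overlapping actor, destroys the Trigger and plays the LS_CCTV_Fainting sequence.
; After short delays, the camera fades out and holds, then the level loads.
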(event `ActivateEnd`
  (`PrimitiveComponent.SetCollisionEnabled` (`self.Trigger`) "QueryAndPhysics"))

(event `self.ReceiveBeginPlay`
  (`PrimitiveComponent.SetCollisionEnabled` (`self.Trigger`) "NoCollision"))

(event `self.Trigger.OnComponentBeginOverlap`
  (params (OverlappedComponent :type "PrimitiveComponent Object Reference") (OtherActor :type "Actor Object Reference") (OtherComp :type "PrimitiveComponent Object Reference") (OtherBodyIndex :type Integer) (bFromSweep :type Boolean) (SweepResult :type "HitResult Structure (by ref)"))
  (`ActorComponent.K2_DestroyComponent` (`self.Trigger`))
  (bind _outactor (`LevelSequencePlayer.CreateLevelSequencePlayer` "/Game/3DAssetLevel/LevelDesign/Cutscenes/LS_CCTV_Fainting.LS_CCTV_Fainting"))
  (`MovieSceneSequencePlayer.Play` (`LevelSequenceActor.SequencePlayer` _outactor))
  (`KismetSystemLibrary.Delay` 1.0)
  (`PlayerCameraManager.StartCameraFade` :`self` (`GameplayStatics.GetPlayerCameraManager` 0) :`FromAlpha` 0.0 :`ToAlpha` 1.0 :`Duration` 3.0 :`bHoldWhenFinished` true)
  (`KismetSystemLibrary.Delay` 10.0)
  (`GameplayStatics.OpenLevelBySoftObjectPtr` "/Game/3DAssetLevel/LevelDesign/Maps/MAP_Level_1.MAP_Level_1"))

(fn `UserConstructionScript`)