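; Interactable button for a CCTV door that signals the door when used and plays a positive or negative click sound.
; A busy flag and DoOnce gate forward one press to the first BPCCTV_Door found by GetActorOfClass, rejecting further presses until ButtonReset re-arms it.
; LookAt returns the label "Button", and sounds play at the button component's relative location.
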(event `/Game/BP_BO/Inventory/BPI_InteractInterface.InteractWith`
  (params (PlayerCharacter :type "/Game/BP_BO/PlayerCharacter/BP_TPCharacter Object Reference"))
  (if (`self.IsBusy`)
    (`GameplayStatics.PlaySoundAtLocation` "/Game/SoundDesign/Environment_SFX/SoundCues/SC_ButtonNegative.SC_ButtonNegative" (`SceneComponent.RelativeLocation` (`self.Button`)) (struct) 1.0 1.0 0.0 null null null null)
    (else
      (`GameplayStatics.PlaySoundAtLocation` "/Game/SoundDesign/Environment_SFX/SoundCues/SC_Button_Positive.SC_Button_Positive" (`SceneComponent.RelativeLocation` (`self.Button`)) (struct) 1.0 1.0 0.0 null null null null)
      (`/Engine/EditorBlueprintResources/StandardMacros.DoOnce` false :!label _label
        (:`Completed`
          (set `self.IsBusy` true)
          (bind _returnvalue (`GameplayStatics.GetActorOfClass` "/Game/3DAssetLevel/LevelDesign/Blueprints/Mechanics_BP/BP-CCTV/BP-CCTV_Door.BP-CCTV_Door_C"))
          (`/Game/3DAssetLevel/LevelDesign/Blueprints/Mechanics_BP/BP-CCTV/BP-CCTV_Door.ButtonClicked` _returnvalue))))))

(event `ButtonReset`
  (set `self.IsBusy` false)
  (goto _label :!via `Reset`))

(fn `LookAt`
  (returns (Message :type Text))
  (return "Button"))

(fn `UserConstructionScript`)