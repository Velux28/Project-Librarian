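; BP_CCTV_Screens drives a bank of eight CCTV monitors that switch to an error screen for a cinematic.
; The CinematicStart event swaps one material slot on each monitor to the drone screen error material, with short delays between them.
; A Sequence launches the A and B rows together, with an initial delay on row B so the failure cascades through A first, then B.
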(event `CinematicStart`
  (`|ExecutionSequence`
    (:`then_0`
      (`PrimitiveComponent.SetMaterial` (`self.MonitorA_1`) 1 "/Game/C_ServiceDrone/MATERIAL/SCREEN/S-Drone_ScreenError_MAT.S-Drone_ScreenError_MAT")
      (`KismetSystemLibrary.Delay` 0.5)
      (`PrimitiveComponent.SetMaterial` (`self.MonitorA_2`) 1 "/Game/C_ServiceDrone/MATERIAL/SCREEN/S-Drone_ScreenError_MAT.S-Drone_ScreenError_MAT")
      (`KismetSystemLibrary.Delay` 0.5)
      (`PrimitiveComponent.SetMaterial` (`self.MonitorA_3`) 1 "/Game/C_ServiceDrone/MATERIAL/SCREEN/S-Drone_ScreenError_MAT.S-Drone_ScreenError_MAT")
      (`KismetSystemLibrary.Delay` 0.5)
      (`PrimitiveComponent.SetMaterial` (`self.MonitorA_4`) 1 "/Game/C_ServiceDrone/MATERIAL/SCREEN/S-Drone_ScreenError_MAT.S-Drone_ScreenError_MAT"))
    (:`then_1`
      (`KismetSystemLibrary.Delay` 2.0)
      (`PrimitiveComponent.SetMaterial` (`self.MonitorB_1`) 1 "/Game/C_ServiceDrone/MATERIAL/SCREEN/S-Drone_ScreenError_MAT.S-Drone_ScreenError_MAT")
      (`KismetSystemLibrary.Delay` 0.5)
      (`PrimitiveComponent.SetMaterial` (`self.MonitorB_2`) 1 "/Game/C_ServiceDrone/MATERIAL/SCREEN/S-Drone_ScreenError_MAT.S-Drone_ScreenError_MAT")
      (`KismetSystemLibrary.Delay` 0.5)
      (`PrimitiveComponent.SetMaterial` (`self.MonitorB_3`) 1 "/Game/C_ServiceDrone/MATERIAL/SCREEN/S-Drone_ScreenError_MAT.S-Drone_ScreenError_MAT")
      (`KismetSystemLibrary.Delay` 0.5)
      (`PrimitiveComponent.SetMaterial` (`self.MonitorB_4`) 1 "/Game/C_ServiceDrone/MATERIAL/SCREEN/S-Drone_ScreenError_MAT.S-Drone_ScreenError_MAT"))))

(fn `UserConstructionScript`)