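; BP_CCTV_Vent is a vent actor in the CCTV mechanics set that emits a gas leak effect with sound on demand.
; BeginPlay switches off the Gas effect and SFXGasLeak audio.
; The GasLeakStart event activates both, then plays a timeline that continuously adjusts the leak sound's volume.
; The file contains no stop logic, and the construction script is empty.
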(event `self.ReceiveBeginPlay`
  (`ActorComponent.SetActive` (`self.Gas`) false false)
  (`ActorComponent.SetActive` (`self.SFX_GasLeak`) false false))

(event `GasLeak Start`
  (`ActorComponent.Activate` (`self.Gas`) false)
  (`ActorComponent.Activate` (`self.SFX_GasLeak`) false)
  (bind (_direction _sfx_volume) (`Timeline|T_GasLeakVolume`)
    (:`Update`
      (`AudioComponent.AdjustVolume` (`self.SFX_GasLeak`) 0.0 _sfx_volume "Linear"))))

(fn `UserConstructionScript`)