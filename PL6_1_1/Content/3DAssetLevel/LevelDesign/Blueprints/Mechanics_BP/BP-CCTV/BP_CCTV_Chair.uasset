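; BP_CCTV_Chair is an interactable chair that triggers the CCTV crisis cutscene and gas leak once.
; Interaction briefly disables player input and plays a level sequence.
; Parallel Sequence delays cue BP_CCTV_Screens, then BP_CCTV_Vent and its own Gas component, then restore input.
; Later it adds a faint green camera fade, heavy breathing and a hold-breath tutorial widget, then activates BP_CCTV_LevelEnd.
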(event `self.ReceiveBeginPlay`
  (`ActorComponent.SetActive` (`self.Gas`) false false))

(event `/Game/BP_BO/Inventory/BPI_InteractInterface.InteractWith`
  (params (PlayerCharacter :type "/Game/BP_BO/PlayerCharacter/BP_TPCharacter Object Reference"))
  (`/Engine/EditorBlueprintResources/StandardMacros.DoOnce` false
    (:`Completed`
      ;[1 0.1615 0.2326] CCTV SCREENS & GAS CINEMATIC
      (`self.DisableInput` (`GameplayStatics.GetPlayerCharacter` 0) (`GameplayStatics.GetPlayerController` 0))
      (`self.Play Crisis Cutscene`))))

(event `Play Crisis Cutscene`
  (`|ExecutionSequence`
    (:`then_0`
      ;[1 1 1] LevelSequence Cinematic
      (bind _outactor (`LevelSequencePlayer.CreateLevelSequencePlayer` "/Game/3DAssetLevel/LevelDesign/Cutscenes/LS_CCTV_Crisis.LS_CCTV_Crisis"))
      (`MovieSceneSequencePlayer.Play` (`LevelSequenceActor.SequencePlayer` _outactor)))
    (:`then_1`
      ;[1 1 1] Attivazione Hacking schermi
      (`KismetSystemLibrary.Delay` 0.2)
      (bind _returnvalue (`GameplayStatics.GetActorOfClass` "/Game/3DAssetLevel/LevelDesign/Blueprints/Mechanics_BP/BP-CCTV/BP_CCTV_Screens.BP_CCTV_Screens_C"))
      (`/Game/3DAssetLevel/LevelDesign/Blueprints/Mechanics_BP/BP-CCTV/BP_CCTV_Screens.CinematicStart` _returnvalue))
    (:`then_2`
      ;[1 1 1] Attivazione Gas
      (`KismetSystemLibrary.Delay` 1.0)
      (bind _returnvalue_2 (`GameplayStatics.GetActorOfClass` "/Game/3DAssetLevel/LevelDesign/Blueprints/Mechanics_BP/BP-CCTV/BP_CCTV_Vent.BP_CCTV_Vent_C"))
      (`/Game/3DAssetLevel/LevelDesign/Blueprints/Mechanics_BP/BP-CCTV/BP_CCTV_Vent.GasLeak Start` _returnvalue_2)
      (`ActorComponent.SetActive` (`self.Gas`) true false))
    (:`then_3`
      ;[1 1 1] Stacchiamo i comandi coì il player si sta fermo con le mani
      (`KismetSystemLibrary.Delay` 1.25)
      (`self.EnableInput` (`GameplayStatics.GetPlayerCharacter` 0) (`GameplayStatics.GetPlayerController` 0)))
    (:`then_4`
      ;[1 1 1] Fine Cinematic + Suono di respiro affannoso
      (`KismetSystemLibrary.Delay` 5.0)
      (`PlayerCameraManager.StartCameraFade` (`GameplayStatics.GetPlayerCameraManager` 0) 0.0 0.03 5.0 (struct :`R` 0.121797 :`G` 0.59375 :`B` 0.090336 :`A` 1.0) false true)
      (`GameplayStatics.PlaySound2D` "/Game/SoundDesign/Character_SFX/SoundCues/SC_HeavyBreathing.SC_HeavyBreathing" 1.0 1.0 0.0 null null)
      ;[1 1 1] Widget Tutorial Holdbreath
      (bind _returnvalue_3 (`|CreateWidget` "/Game/Level_0/Environment/Blueprint/Widgets/W_HoldBreath.W_HoldBreath_C"))
      (`UserWidget.AddToViewport` _returnvalue_3 0)
      ;[1 1 1] Attivazione BP Fine Livello
      (`KismetSystemLibrary.Delay` 10.0)
      (bind _returnvalue_4 (`GameplayStatics.GetActorOfClass` "/Game/3DAssetLevel/LevelDesign/Blueprints/Mechanics_BP/BP-CCTV/BP_CCTV_LevelEnd.BP_CCTV_LevelEnd_C"))
      (`/Game/3DAssetLevel/LevelDesign/Blueprints/Mechanics_BP/BP-CCTV/BP_CCTV_LevelEnd.ActivateEnd` _returnvalue_4))))

(fn `LookAt`
  (returns (Message :type Text))
  (return ""))

(fn `UserConstructionScript`)