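; Assembly blueprint for a two-panel AI door that opens, activates an assigned AI character, then closes.
; IAActivated waits briefly, then plays a timeline per door mesh to slide its relative location.
; In the same sequence, the ACAIActivator starts the referenced character with its behavior tree.
; After a further delay, both timelines reverse to shut the door.
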(event `IA Activated`
  (`KismetSystemLibrary.Delay` 2.0)
  (`|ExecutionSequence`
    (:`then_0`
      (bind (_direction _door1track) (`Timeline|T_Door1` :!label _label)
        (:`Update`
          (`SceneComponent.K2_SetRelativeLocation` (`self.DoorMesh_1`) _door1track false false))))
    (:`then_1`
      (bind (_direction_2 _door2track) (`Timeline|T_Door2` :!label _label_2)
        (:`Update`
          (`SceneComponent.K2_SetRelativeLocation` (`self.DoorMesh_2`) _door2track false false))))
    (:`then_2`
      (`/Game/BP_BO/ArtificialIntelligence/AC_AIActivator.Activate AI` (`self.AC_AIActivator`) (`self.AI_Ref`) (`self.BTRef`)))
    (:`then_3`
      (`KismetSystemLibrary.Delay` 3.0)
      (goto _label :!via `Reverse`))
    (:`then_4`
      (`KismetSystemLibrary.Delay` 3.0)
      (goto _label_2 :!via `Reverse`))))

(fn `UserConstructionScript`)