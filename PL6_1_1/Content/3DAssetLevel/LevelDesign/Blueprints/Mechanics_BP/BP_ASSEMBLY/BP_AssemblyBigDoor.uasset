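; Two-panel sliding door for the assembly area that opens on a ButtonClicked event and closes itself after a short delay.
; Two timelines drive the relative locations of the door meshes, playing together to open and reversing to close.
; A longer parallel delay then calls ButtonReset on the BP_ButtonAssembly returned by GetActorOfClass, so it assumes a single button in the level.
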(event `ButtonClicked`
  (`|ExecutionSequence`
    (:`then_0`
      (`|ExecutionSequence`
        (:`then_0`
          (bind (_direction _door1track) (`Timeline|T_Door1` :!label _label)
            (:`Update`
              (`SceneComponent.K2_SetRelativeLocation` (`self.DoorMesh_1`) _door1track false false))))
        (:`then_1`
          (bind (_direction_2 _door2track) (`Timeline|T_Door2` :!label _label_2)
            (:`Update`
              (`SceneComponent.K2_SetRelativeLocation` (`self.DoorMesh_2`) _door2track false false))))))
    (:`then_1`
      (`KismetSystemLibrary.Delay` 3.0)
      (`|ExecutionSequence`
        (:`then_0`
          (goto _label :!via `Reverse`))
        (:`then_1`
          (goto _label_2 :!via `Reverse`))))
    (:`then_2`
      (`KismetSystemLibrary.Delay` 7.0)
      (bind _returnvalue (`GameplayStatics.GetActorOfClass` "/Game/3DAssetLevel/LevelDesign/Blueprints/Mechanics_BP/BP_ASSEMBLY/BP_ButtonAssembly.BP_ButtonAssembly_C"))
      (`/Game/3DAssetLevel/LevelDesign/Blueprints/Mechanics_BP/BP_ASSEMBLY/BP_ButtonAssembly.ButtonReset` _returnvalue))))

(fn `UserConstructionScript`)