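; BP_Monitor is an interactable monitor that opens a tablet-style screen for the player.
; A trigger box toggles custom depth on the monitor mesh to show an outline while the player character overlaps it.
; On interaction it plays a 2D sound, creates a W_COD_Tablet widget with its note texture, opens it on the viewport and flags the tablet as open.
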(event `self.TriggerBox.OnComponentBeginOverlap`
  (params (OverlappedComponent :type "PrimitiveComponent Object Reference") (OtherActor :type "Actor Object Reference") (OtherComp :type "PrimitiveComponent Object Reference") (OtherBodyIndex :type Integer) (bFromSweep :type Boolean) (SweepResult :type "HitResult Structure (by ref)"))
  ;[1 1 1] Attiva/Disattiva l'Outline dell'oggetto
  (if (== OtherActor (`GameplayStatics.GetPlayerCharacter` 0))
    (`PrimitiveComponent.SetRenderCustomDepth` (`self.Monitor`) true)))

(event `self.TriggerBox.OnComponentEndOverlap`
  (params (OverlappedComponent :type "PrimitiveComponent Object Reference") (OtherActor :type "Actor Object Reference") (OtherComp :type "PrimitiveComponent Object Reference") (OtherBodyIndex :type Integer))
  ;[1 1 1] Attiva/Disattiva l'Outline dell'oggetto
  (if (== OtherActor (`GameplayStatics.GetPlayerCharacter` 0))
    (`PrimitiveComponent.SetRenderCustomDepth` (`self.Monitor`) false)))

(event `/Game/BP_BO/Inventory/BPI_InteractInterface.InteractWith`
  (params (PlayerCharacter :type "/Game/BP_BO/PlayerCharacter/BP_TPCharacter Object Reference"))
  (`GameplayStatics.PlaySound2D` "/Game/SoundDesign/Environment_SFX/SoundCues/SC_Widget.SC_Widget" 0.5 1.0 0.0 null null)
  (bind _returnvalue (`|CreateWidget` "/Game/UI/PlayerUI/Tablet_UI/W_COD_Tablet.W_COD_Tablet_C" null (`self.TabletNoteTexture`)))
  (bind _output_get (set `self.Widget` _returnvalue))
  (`CommonActivatableWidget.ActivateWidget` _output_get)
  (`/Game/UI/PlayerUI/Tablet_UI/W_COD_Tablet.Open Tablet` (`self.Widget`))
  (`UserWidget.AddToViewport` (`self.Widget`) 0)
  (set `self.IsTabletOpen` true))

(fn `UserConstructionScript`)