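; BP_AssemblyNewDoor is a two-panel assembly door that opens when its ButtonClicked event fires, then closes itself.
; Two timelines drive the relative location of each door mesh and reverse after a short delay.
; A longer parallel delay resets the BP_ButtonAssembly found with GetActorOfClass.
; The same event immediately deactivates the referenced AI through ACAIActivator, destroys that actor and prints a debug message.
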(event `ButtonClicked`
  (bind _ia_ref (`self.IA Ref`))
  (`|ExecutionSequence`
    (:`then_0`
      (`|ExecutionSequence`
        (:`then_0`
          (bind (_direction _door1track) (`Timeline|Timeline_0` :!label _label)
            (:`Update`
              (`SceneComponent.K2_SetRelativeLocation` (`self.DoorMesh_1`) _door1track false false))))
        (:`then_1`
          (bind (_direction_2 _door2track) (`Timeline|Timeline_1` :!label _label_2)
            (:`Update`
              (`SceneComponent.K2_SetRelativeLocation` (`self.DoorMesh_2`) _door2track false false))))))
    (:`then_1`
      (`KismetSystemLibrary.Delay` 3.0)
      (`|ExecutionSequence`
        (:`then_0`
          (goto _label :!via `Reverse`))
        (:`then_1`
          (goto _label_2 :!via `Reverse`))))
    (:`then_2`
      (`KismetSystemLibrary.Delay` 7.0)
      (bind _returnvalue (`GameplayStatics.GetActorOfClass` "/Game/3DAssetLevel/LevelDesign/Blueprints/Mechanics_BP/BP_ASSEMBLY/BP_ButtonAssembly.BP_ButtonAssembly_C"))
      (`/Game/3DAssetLevel/LevelDesign/Blueprints/Mechanics_BP/BP_ASSEMBLY/BP_ButtonAssembly.ButtonReset` _returnvalue))
    (:`then_3`
      (`/Game/BP_BO/ArtificialIntelligence/AC_AIActivator.De-activate AI` (`self.AC_AIActivator`) _ia_ref)
      (`self.K2_DestroyActor` _ia_ref)
      (`KismetSystemLibrary.PrintText` "ASSEMBLY IA SPENTA"))))

(fn `UserConstructionScript`)