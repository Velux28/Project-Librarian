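; BP_AssemblyDoor is a two-leaf door actor that caches both door meshes on BeginPlay and drives them from Tick.
; Paired opening and closing flags select OpenDoor or CloseDoor, whose bodies are not shown, with closing clearing the opening flags.
; ButtonClicked sets only the first leaf's opening flag when all are clear, while opening requires both.
; A debug "Hello" prints during opening.
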(event `self.ReceiveBeginPlay`
  (set `self.door` (`self.DoorMesh_1`))
  (set `self.door2` (`self.DoorMesh_2`)))

(event `self.ReceiveTick`
  (params (DeltaSeconds :type "Float (single-precision)"))
  (if (and (`self.bIsDoorOpening`) (`self.bIsDoor2Opening`))
    (if (and (`self.bIsDoorClosing`) (`self.bIsDoor2Closing`))
      (set `self.bIsDoorOpening` false)
      (set `self.bIsDoor2Opening` false)
      (else
        (`self.OpenDoor`)
        (`KismetSystemLibrary.PrintString` "Hello")))
    (elif (and (`self.bIsDoorClosing`) (`self.bIsDoor2Closing`))
      (`self.CloseDoor`))))

(event `ButtonClicked`
  (if (or (`self.bIsDoorOpening`) (`self.bIsDoorClosing`))
    _
    (elif (not (or (`self.bIsDoor2Opening`) (`self.bIsDoor2Closing`)))
      (set `self.bIsDoorOpening` true))))

(fn `UserConstructionScript`)