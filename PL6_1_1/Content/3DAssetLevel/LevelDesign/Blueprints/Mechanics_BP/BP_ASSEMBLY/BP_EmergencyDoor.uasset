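; Emergency door that the player forces open by repeatedly interacting with its lever.
; A trigger box shows a "spam E" HUD widget and outlines the lever through custom depth while the door is closed.
; Interact calls count presses up to a threshold, then tilt the lever and, after a short delay, play a timeline that swings the door open with sounds.
; CheckIFInteractable always returns false, and older timeline logic is left unconnected.
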(event `self.ReceiveBeginPlay`
  ;[1 1 1] Widget Management + Outline Management
  (bind _returnvalue (`|CreateWidget` "/Game/UI/PlayerUI/Environment_UI/Interactions/W_HUD_SpamE.W_HUD_SpamE_C"))
  (`UserWidget.AddToViewport` _returnvalue 0)
  (`Widget.SetVisibility` _returnvalue "Hidden"))

(event `self.TriggerBox.OnComponentBeginOverlap`
  (params (OverlappedComponent :type "PrimitiveComponent Object Reference") (OtherActor :type "Actor Object Reference") (OtherComp :type "PrimitiveComponent Object Reference") (OtherBodyIndex :type Integer) (bFromSweep :type Boolean) (SweepResult :type "HitResult Structure (by ref)"))
  ;[1 1 1] Widget Management + Outline Management
  (if (== OtherActor (`GameplayStatics.GetPlayerCharacter` 0))
    (if (not (`self.B_IsOpen`))
      (`Widget.SetVisibility` (stale `self.ReceiveBeginPlay` _returnvalue) "Visible")
      (`PrimitiveComponent.SetRenderCustomDepth` (`self.Leva`) true) ; Outline
    )))

(event `self.TriggerBox.OnComponentEndOverlap`
  (params (OverlappedComponent :type "PrimitiveComponent Object Reference") (OtherActor :type "Actor Object Reference") (OtherComp :type "PrimitiveComponent Object Reference") (OtherBodyIndex :type Integer))
  ;[1 1 1] Widget Management + Outline Management
  (if (== OtherActor (`GameplayStatics.GetPlayerCharacter` 0))
    (`Widget.SetVisibility` (stale `self.ReceiveBeginPlay` _returnvalue) "Hidden")
    (`PrimitiveComponent.SetRenderCustomDepth` (`self.Leva`) false) ; Outline
  ))

(event `/Game/BP_BO/Inventory/BPI_InteractInterface.InteractWith`
  (params (PlayerCharacter :type "/Game/BP_BO/PlayerCharacter/BP_TPCharacter Object Reference"))
  (bind _returnvalue (`SceneComponent.K2_GetComponentLocation` (`self.Door_1`)))
  (if (not (`self.B_IsOpen`))
    ;[1 0 0] Da ottimizzare
    (bind _result (`/Engine/EditorBlueprintResources/StandardMacros.IncrementFloat` (`self.Pressed Amount`))
      (:`  `
        (bind _output_get (set `self.Pressed Amount` _result))
        (if (== _output_get (`self.Presses needed`))
          ;[1 1 1] Abbassamento Leva
          (`GameplayStatics.PlaySoundAtLocation` "/Game/Level_1/Environment/Sounds/METAL_DEBRIS.METAL_DEBRIS" _returnvalue (struct) 1.0 1.0 0.0 null null null null)
          (`SceneComponent.K2_SetRelativeRotation` (`self.Leva`) (struct :`Roll` 30.0) false false)
          ;[1 0 0] ?
          (`KismetSystemLibrary.Delay` 0.2)
          ;[1 1 1] Apertura Porta
          (bind (_direction _doormov) (`Timeline|T_DoorMove`)
            (:`Update`
              (`SceneComponent.K2_SetRelativeRotation` (`self.Door_1`) (`KismetMathLibrary.MakeRotator` 0.0 0.0 _doormov) false false)
              (set `self.B_IsOpen` true))
            (:`SFX Impact Event`
              ;[0.5 0 1] SFX Porta che sbatte
              (`GameplayStatics.PlaySoundAtLocation` "/Game/Level_1/Environment/Sounds/SC_MetalDoor.SC_MetalDoor" _returnvalue (struct) 1.0 1.0 0.0 null null null null))))))))

(fn `Check IF Interactable`
  (returns (`Is NOT Interactable` :type Boolean))
  (return false))

(fn `UserConstructionScript`)