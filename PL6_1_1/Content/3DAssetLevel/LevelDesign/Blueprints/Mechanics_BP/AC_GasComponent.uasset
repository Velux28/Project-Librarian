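; Gas hazard component that kills or heavily damages a player who breathes in gas for too long.
; CheckHoldBreath, meant for repeated external calls, counts the exposure timer down by delta time and applies damage on every call once it is empty.
; Holding breath, read from the player's OLD-prefixed variables, refills the timer up to GasKillTimer.
; It clears the hold flag when the player's breath timer runs out.
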(event `self.ReceiveBeginPlay`
  (set `self.CurrentTimer` (`self.GasKillTimer`)))

(fn `CheckHoldBreath`
  (params (Player :type "/Game/BP_BO/PlayerCharacter/BP_TPCharacter Object Reference"))
  (if (`/Game/BP_BO/PlayerCharacter/BP_TPCharacter.[OLD] IsHoldingBreath` Player)
    (set `self.CurrentTimer` (`KismetMathLibrary.FClamp` (+ (`self.CurrentTimer`) (`GameplayStatics.GetWorldDeltaSeconds`)) 0.0 (`self.GasKillTimer`)))
    (if (<= (`/Game/BP_BO/PlayerCharacter/BP_TPCharacter.[OLD] BreathCurrTimer` (`local.Player`)) 0.0)
      (set `/Game/BP_BO/PlayerCharacter/BP_TPCharacter.[OLD] IsHoldingBreath` false (`local.Player`)))
    (elif (<= (`self.CurrentTimer`) 0.0)
      (`GameplayStatics.ApplyDamage` Player 150.0)
      (cast `/Game/BP_BO/PlayerCharacter/BP_TPCharacter` (`GameplayStatics.GetPlayerCharacter` 0))
      (else
        (set `self.CurrentTimer` (- (`self.CurrentTimer`) (`GameplayStatics.GetWorldDeltaSeconds`)))))))