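; BP_ConductVent1 is an interactable vent whose door is knocked off after a set number of interactions.
; Interactwith counts presses while the vent is not flagged open; on reaching the required count it enables physics on the door, applies an impulse and disables simulation after a short delay.
; IsAllScrewOpen checks whether every screw is open but is not called in these graphs, and LookAt returns an empty string.
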(event `/Game/BP_BO/Inventory/BPI_InteractInterface.InteractWith`
  (params (PlayerCharacter :type "/Game/BP_BO/PlayerCharacter/BP_TPCharacter Object Reference"))
  (bind _pressed_amount (`self.Pressed Amount`))
  (bind _ventdoor3 (`self.VentDoor3`))
  (if (not (`self.B_IsOpen`))
    ;[1 0 0] Da ottimizzare
    (`/Engine/EditorBlueprintResources/StandardMacros.IncrementFloat` _pressed_amount
      (:`  `
        (bind _output_get (set `self.Pressed Amount` _pressed_amount))
        (if (== _output_get (`self.Presses needed`))
          (`PrimitiveComponent.SetSimulatePhysics` _ventdoor3 true)
          (`PrimitiveComponent.AddImpulse` _ventdoor3 (0.0 -100000.0 -100.0) "None" false)
          (`KismetSystemLibrary.Delay` 2.0)
          (`PrimitiveComponent.SetSimulatePhysics` _ventdoor3 false))))))

(fn `Is All Screw Open`
  (returns (Result :type Boolean))
  (for _array_element (`self.Screws`)
    ;[0 0.6429 1] se una vite è ancora avvitata non controllo le altre
    (if (not (`/Game/3DAssetLevel/LevelDesign/Blueprints/Mechanics_BP/BP_Screw.B_ScrewOpen` _array_element))
      (return false)))
  (return true))

(fn `LookAt`
  (returns (Message :type Text))
  (return ""))

(fn `UserConstructionScript`)