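; BP_TUT_Button_A is an interactable button, apparently for the tutorial, that triggers scripted level objects once and reports "Button" as its look-at text.
; Interactwith passes a DoOnce, plays a positive sound, then runs a Sequence that activates the dynamic glass and, after a short delay, the can dispenser.
; Targets are found with GetActorOfClass rather than references; the final branch looks up the freeze pod but calls nothing on it.
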(event `/Game/BP_BO/Inventory/BPI_InteractInterface.InteractWith`
  (params (PlayerCharacter :type "/Game/BP_BO/PlayerCharacter/BP_TPCharacter Object Reference"))
  (`/Engine/EditorBlueprintResources/StandardMacros.DoOnce` false
    (:`Completed`
      (`GameplayStatics.PlaySoundAtLocation` "/Game/SoundDesign/Environment_SFX/SoundCues/SC_Button_Positive.SC_Button_Positive" (`SceneComponent.RelativeLocation` (`self.Button`)) (struct) 1.0 1.0 0.0 null null null null)
      (`|ExecutionSequence`
        (:`then_0`
          ;[1 1 1] Attivazione trasparenza vetro
          (bind _returnvalue (`GameplayStatics.GetActorOfClass` "/Game/3DAssetLevel/LevelDesign/Blueprints/Mechanics_BP/TUT_BP/BP_TUT_DynamicGlass.BP_TUT_DynamicGlass_C"))
          (`/Game/3DAssetLevel/LevelDesign/Blueprints/Mechanics_BP/TUT_BP/BP_TUT_DynamicGlass.GlassActivation` _returnvalue))
        (:`then_1`
          (`KismetSystemLibrary.Delay` 2.0)
          (bind _returnvalue_2 (`GameplayStatics.GetActorOfClass` "/Game/3DAssetLevel/LevelDesign/Blueprints/Mechanics_BP/BP_TUT_CanDispenser.BP_TUT_CanDispenser_C"))
          (`/Game/3DAssetLevel/LevelDesign/Blueprints/Mechanics_BP/BP_TUT_CanDispenser.Dispenser Activated` _returnvalue_2))
        (:`then_2`
          (`GameplayStatics.GetActorOfClass` "/Game/3DAssetLevel/LevelDesign/Blueprints/Mechanics_BP/TUT_BP/BP_TUT_FreezePod.BP_TUT_FreezePod_C"))))))

(fn `LookAt`
  (returns (Message :type Text))
  (return "Button"))

(fn `UserConstructionScript`)