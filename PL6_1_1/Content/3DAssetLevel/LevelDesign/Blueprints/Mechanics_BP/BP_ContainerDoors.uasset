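; BP_ContainerDoors is a shipping-container door actor that can be switched from closed to damaged during play.
; On BeginPlay the damaged door mesh is hidden with collision disabled.
; The OpenContainer event destroys both closed door components, then reveals the damaged door with full collision and plays a metal door sound at its location.
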(event `self.ReceiveBeginPlay`
  (bind _damageddoor (`self.DamagedDoor`))
  (`SceneComponent.SetVisibility` _damageddoor false true)
  (`PrimitiveComponent.SetCollisionEnabled` _damageddoor "NoCollision"))

(event `Open Container`
  (bind _damageddoor (`self.DamagedDoor`))
  (`ActorComponent.K2_DestroyComponent` (`self.ClosedDoor`))
  (`ActorComponent.K2_DestroyComponent` (`self.ClosedDoor2`))
  (`SceneComponent.SetVisibility` _damageddoor true true)
  (`PrimitiveComponent.SetCollisionEnabled` _damageddoor "QueryAndPhysics")
  (`GameplayStatics.PlaySoundAtLocation` "/Game/Level_1/Environment/Sounds/SC_MetalDoor.SC_MetalDoor" (`SceneComponent.K2_GetComponentLocation` (`self.DamagedDoor`)) (struct) 1.0 1.0 0.0 null null null null))

(fn `UserConstructionScript`)