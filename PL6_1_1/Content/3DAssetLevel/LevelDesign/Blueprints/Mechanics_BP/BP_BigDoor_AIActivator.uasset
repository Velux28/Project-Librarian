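; BP_BigDoor_AIActivator is a trigger-driven double door that also activates an AI character.
; Any overlap with the Box plays two timelines that move the door meshes' relative locations; ending the overlap reverses them.
; The first timeline's Update calls ACAIActivator's ActivateAI with the referenced character and behavior tree and prints a debug message, so activation repeats every update rather than firing once.
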(event `self.Box.OnComponentBeginOverlap`
  (params (OverlappedComponent :type "PrimitiveComponent Object Reference") (OtherActor :type "Actor Object Reference") (OtherComp :type "PrimitiveComponent Object Reference") (OtherBodyIndex :type Integer) (bFromSweep :type Boolean) (SweepResult :type "HitResult Structure (by ref)"))
  (`|ExecutionSequence`
    (:`then_0`
      (bind (_direction _door1track) (`Timeline|T_Door1` :!label _label)
        (:`Update`
          (`SceneComponent.K2_SetRelativeLocation` (`self.DoorMesh_1`) _door1track false false)
          (`/Game/BP_BO/ArtificialIntelligence/AC_AIActivator.Activate AI` (`self.AC_AIActivator`) (`self.AIRef`) (`self.BTRef`))
          (`KismetSystemLibrary.PrintString` "AI Attivata"))))
    (:`then_1`
      (bind (_direction_2 _door2track) (`Timeline|T_Door2` :!label _label_2)
        (:`Update`
          (`SceneComponent.K2_SetRelativeLocation` (`self.DoorMesh_2`) _door2track false false))))))

(event `self.Box.OnComponentEndOverlap`
  (params (OverlappedComponent :type "PrimitiveComponent Object Reference") (OtherActor :type "Actor Object Reference") (OtherComp :type "PrimitiveComponent Object Reference") (OtherBodyIndex :type Integer))
  (`|ExecutionSequence`
    (:`then_0`
      (goto _label :!via `Reverse`))
    (:`then_1`
      (goto _label_2 :!via `Reverse`))))

(fn `UserConstructionScript`)