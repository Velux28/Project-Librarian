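; Interactable CCTV chair that triggers a one-time crisis cinematic, with a trigger box toggling its outline while usable.
; Interaction removes the inventory HUD, locks input, hides the player, disables a button and plays a Level Sequence.
; Timed delays fire the screens and server events and zero the player's cans, then dialogue starts and control returns as the sequence ends.
; An unwired fainting and level-load ending remains.
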(event `/Game/BP_BO/Inventory/BPI_InteractInterface.InteractWith`
  (params (PlayerCharacter :type "/Game/BP_BO/PlayerCharacter/BP_TPCharacter Object Reference"))
  (set `self.Player Character` PlayerCharacter)
  (`/Engine/EditorBlueprintResources/StandardMacros.DoOnce` false
    (:`Completed`
      ;[1 1 1] Spengo player HUD per il resto della permanenza in CCTV.
      ; Verrà ricaricato col BeginPlay in Submap_1
      (`Widget.RemoveFromParent` (`/Game/UI/PlayerUI/Basic_UI/W_PlayerHUD.W_HUD_Inventory` (`/Game/BP_BO/PlayerCharacter/BP_TPCharacter.HUD` (`self.Player Character`))))
      ;[1 1 1] Disable Player Input
      (`self.DisableInput` (`self.Player Character`) (`GameplayStatics.GetPlayerController` 0))
      ;[1 1 1] Turn Off Player Visibility
      ; Player Mesh can't be seen during Cinematic
      (`SceneComponent.SetVisibility` (`Character.Mesh` (`self.Player Character`)) false true)
      ;[1 1 1] Turn Off Exit Button
      (`/Game/BP_BO/Puzzles/BPI_Unlockable.SetButtonUnusable_Red` (`self.Button to Disable`))
      ;[1 1 1] LevelSequence Cinematic - Camera Pan across Screens
      (bind _outactor (`LevelSequencePlayer.CreateLevelSequencePlayer` "/Game/3DAssetLevel/LevelDesign/Cutscenes/LS_CCTV_Crisis.LS_CCTV_Crisis"))
      (bind _sequenceplayer (`LevelSequenceActor.SequencePlayer` _outactor))
      (`MovieSceneSequencePlayer.Play` _sequenceplayer)
      (`|ExecutionSequence`
        (:`then_0`
          ;[1 1 1] Screens going Red + Audio Cue
          (`KismetSystemLibrary.Delay` 0.4)
          (bind _returnvalue (`GameplayStatics.GetActorOfClass` "/Game/3DAssetLevel/LevelDesign/Blueprints/Mechanics_BP/BP_CCTV/BP_CCTV_Screens.BP_CCTV_Screens_C"))
          (`/Game/3DAssetLevel/LevelDesign/Blueprints/Mechanics_BP/BP_CCTV/BP_CCTV_Screens.CinematicStart` _returnvalue)
          ;[1 1 1] Levo le lattine al player così non lancia un cazzo
          (set `/Game/BP_BO/PlayerCharacter/BP_TPCharacter.Number of Cans` 0 (`self.Player Character`))
          ;[1 0.5 0] Server Activation
          (`KismetSystemLibrary.Delay` 4.6)
          (bind _returnvalue_2 (`GameplayStatics.GetActorOfClass` "/Game/BP_BO/Environment/BP_CCTVServer.BP_CCTVServer_C"))
          (`/Game/BP_BO/Environment/BP_CCTVServer.Cinematic` _returnvalue_2))
        (:`then_1`
          (`KismetSystemLibrary.Delay` (`TimeManagementBlueprintLibrary.Conv_QualifiedFrameTimeToSeconds` (`MovieSceneSequencePlayer.GetEndTime` _sequenceplayer))) ; Tempo necessario a finire \nla cinematic
          ;[1 1 1] Start monologue
          (`/Game/BP_BO/PlayerCharacter/BP_TPCharacter.StartDialogue` (`self.Player Character`) (`self.Dialogue Key`) null)
          ;[1 1 1] Enable Player Input
          (`self.EnableInput` (`self.Player Character`) (`GameplayStatics.GetPlayerController` 0))
          ;[1 1 1] Return Player Visibility
          (`SceneComponent.SetVisibility` (`Character.Mesh` (`self.Player Character`)) true false)
          (set `self.Is NOT Interactable` true)
          ;[1 1 1] Attiva/Disattiva l'Outline dell'oggetto
          (`PrimitiveComponent.SetRenderCustomDepth` (`self.Chair`) false :!label _label))))))

(event `self.TriggerBox.OnComponentBeginOverlap`
  (params (OverlappedComponent :type "PrimitiveComponent Object Reference") (OtherActor :type "Actor Object Reference") (OtherComp :type "PrimitiveComponent Object Reference") (OtherBodyIndex :type Integer) (bFromSweep :type Boolean) (SweepResult :type "HitResult Structure (by ref)"))
  ;[1 1 1] Attiva/Disattiva l'Outline dell'oggetto
  (if (== OtherActor (`GameplayStatics.GetPlayerCharacter` 0))
    (if (not (`self.Is NOT Interactable`))
      (`PrimitiveComponent.SetRenderCustomDepth` (`self.Chair`) true))))

(event `self.TriggerBox.OnComponentEndOverlap`
  (params (OverlappedComponent :type "PrimitiveComponent Object Reference") (OtherActor :type "Actor Object Reference") (OtherComp :type "PrimitiveComponent Object Reference") (OtherBodyIndex :type Integer))
  ;[1 1 1] Attiva/Disattiva l'Outline dell'oggetto
  (if (== OtherActor (`GameplayStatics.GetPlayerCharacter` 0))
    (goto _label)))

(fn `Check IF Interactable`
  (returns (`Is NOT Interactable` :type Boolean))
  (return (`self.Is NOT Interactable`)))

(fn `UserConstructionScript`)