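; An interactable button that turns a specific AI character on or off when the player interacts with it.
; On interaction it runs the parent interact logic, then, if working and its AI activator component is valid, checks the ActivateAI flag.
; The flag selects either activating the referenced AI with its behavior tree or deactivating it through that component.
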(event `/Game/BP_BO/Inventory/BPI_InteractInterface.InteractWith`
  (params (PlayerCharacter :type "/Game/BP_BO/PlayerCharacter/BP_TPCharacter Object Reference"))
  (`parent.InteractWith` PlayerCharacter)
  (if (`self.IsWorking`)
    (bind _ac_aiactivator (`self.AC_AIActivator`)
      (:`then`
        (if (`self.ActivateAI`)
          (`/Game/BP_BO/ArtificialIntelligence/AC_AIActivator.Activate AI` _ac_aiactivator (`self.AIRef`) (`self.BTRef`))
          (else
            (`/Game/BP_BO/ArtificialIntelligence/AC_AIActivator.De-activate AI` _ac_aiactivator (`self.AIRef`)))))
      (:`else`))))

(fn `UserConstructionScript`)