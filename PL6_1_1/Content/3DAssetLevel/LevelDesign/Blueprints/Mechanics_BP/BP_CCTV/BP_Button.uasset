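; Interactable button that opens a linked CCTV, control or assembly door and shows "Button" as its look-at text.
; On interaction it plays a positive or negative sound depending on its busy state.
; A DoOnce gate sets it busy and casts DoorToOpen through the three door types to trigger it.
; It resets five seconds after triggering a door, but stays busy if no valid door matches.
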(event `/Game/BP_BO/Inventory/BPI_InteractInterface.InteractWith`
  (params (PlayerCharacter :type "/Game/BP_BO/PlayerCharacter/BP_TPCharacter Object Reference"))
  (if (`self.IsBusy`)
    (`GameplayStatics.PlaySoundAtLocation` "/Game/SoundDesign/Environment_SFX/SoundCues/SC_ButtonNegative.SC_ButtonNegative" (`SceneComponent.RelativeLocation` (`self.Button`)) (struct) 1.0 1.0 0.0 null null null null)
    (else
      (`GameplayStatics.PlaySoundAtLocation` "/Game/SoundDesign/Environment_SFX/SoundCues/SC_Button_Positive.SC_Button_Positive" (`SceneComponent.RelativeLocation` (`self.Button`)) (struct) 1.0 1.0 0.0 null null null null)
      (`/Engine/EditorBlueprintResources/StandardMacros.DoOnce` false :!label _label
        (:`Completed`
          (set `self.IsBusy` true)
          (bind _doortoopen (`self.DoorToOpen`)
            (:`then`
              (bind _asbp_cctv_door (cast `/Game/3DAssetLevel/LevelDesign/Blueprints/Mechanics_BP/BP_CCTV/BP-CCTV_Door` _doortoopen)
                (:`then`
                  (`/Game/3DAssetLevel/LevelDesign/Blueprints/Mechanics_BP/BP_CCTV/BP-CCTV_Door.ButtonClicked` _asbp_cctv_door))
                (:`CastFailed`
                  (bind _asbp_control_door (cast `/Game/3DAssetLevel/LevelDesign/Blueprints/Mechanics_BP/BP_STORAGE/BP_ControlDoor` _doortoopen)
                    (:`then`
                      (`/Game/3DAssetLevel/LevelDesign/Blueprints/Mechanics_BP/BP_STORAGE/BP_ControlDoor.ButtonClicked` _asbp_control_door))
                    (:`CastFailed`
                      (bind _asbp_assembly_door (cast `/Game/3DAssetLevel/LevelDesign/Blueprints/Mechanics_BP/BP_ASSEMBLY/BP_AssemblyDoor` _doortoopen))
                      (`ASlidingDoor.OpenDoor` _asbp_assembly_door)))))
              (`KismetSystemLibrary.Delay` 5.0)
              (`self.ButtonReset`))
            (:`else`)))))))

(event `ButtonReset`
  (set `self.IsBusy` false)
  (goto _label :!via `Reset`))

(fn `LookAt`
  (returns (Message :type Text))
  (return "Button"))

(fn `UserConstructionScript`)