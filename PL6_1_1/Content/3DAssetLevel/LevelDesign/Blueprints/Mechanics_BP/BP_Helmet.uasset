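; BP_Helmet is an interactable helmet pickup, apparently intended to activate the HUD, which is not yet implemented.
; A trigger box toggles custom depth on the helmet mesh to show an outline while the player character overlaps it.
; The Interactwith event prints a red placeholder message and destroys the actor.
; Its CheckIFInteractable function always returns false.
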(event `self.TriggerBox.OnComponentBeginOverlap`
  (params (OverlappedComponent :type "PrimitiveComponent Object Reference") (OtherActor :type "Actor Object Reference") (OtherComp :type "PrimitiveComponent Object Reference") (OtherBodyIndex :type Integer) (bFromSweep :type Boolean) (SweepResult :type "HitResult Structure (by ref)"))
  ;[1 1 1] Gestione Outline
  (if (== OtherActor (`GameplayStatics.GetPlayerCharacter` 0))
    (`PrimitiveComponent.SetRenderCustomDepth` (`self.Helmet`) true)))

(event `self.TriggerBox.OnComponentEndOverlap`
  (params (OverlappedComponent :type "PrimitiveComponent Object Reference") (OtherActor :type "Actor Object Reference") (OtherComp :type "PrimitiveComponent Object Reference") (OtherBodyIndex :type Integer))
  ;[1 1 1] Gestione Outline
  (if (== OtherActor (`GameplayStatics.GetPlayerCharacter` 0))
    (`PrimitiveComponent.SetRenderCustomDepth` (`self.Helmet`) false)))

(event `/Game/BP_BO/Inventory/BPI_InteractInterface.InteractWith`
  (params (PlayerCharacter :type "/Game/BP_BO/PlayerCharacter/BP_TPCharacter Object Reference"))
  (`KismetSystemLibrary.PrintString` "ATTIVAZIONE HUD - DA IMPLEMENTARE" true true (struct :`R` 1.0 :`A` 1.0) 10.0)
  (`self.K2_DestroyActor`))

(fn `Check IF Interactable`
  (returns (`Is NOT Interactable` :type Boolean))
  (return false))

(fn `UserConstructionScript`)