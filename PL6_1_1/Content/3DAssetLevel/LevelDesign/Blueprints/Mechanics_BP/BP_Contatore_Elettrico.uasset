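; Interactable electrical box that the player opens and then switches on, in two separate interactions.
; The first interaction plays two timelines that swing the doors open, with a delay before flagging them as open.
; The next flips the switch with a sound, swaps the red light for the OK light and changes the lamp material.
; It then destroys its interaction component, and DoOnce gates keep each step from repeating.
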(event `/Game/BP_BO/Inventory/BPI_InteractInterface.InteractWith`
  (params (PlayerCharacter :type "/Game/BP_BO/PlayerCharacter/BP_TPCharacter Object Reference"))
  (if (`self.B_AreDoorsOpen`)
    (`/Engine/EditorBlueprintResources/StandardMacros.DoOnce` false
      (:`Completed`
        ;[1 1 1] Switch rotation e SFX
        (`SceneComponent.K2_SetRelativeRotation` (`self.SM_ElectricBox_Switch`) (struct :`Yaw` 90.0 :`Roll` 50.0) false false)
        (`GameplayStatics.PlaySoundAtLocation` "/Engine/VREditor/Sounds/UI/Flashlight_Switch.Flashlight_Switch" (`SceneComponent.RelativeLocation` (`self.SM_ElectricBox_Body`)) (struct) 1.0 1.0 0.0 null null null null)
        ;[1 1 1] Cambiamento luce
        (`SceneComponent.SetVisibility` (`self.RectLight-RED`) false false)
        (`SceneComponent.SetVisibility` (`self.RectLight-OK`) true false)
        (`PrimitiveComponent.SetMaterial` (`self.Lamp`) 1 "/Game/3DAssetLevel/LevelDesign/Materials/ENR_Mats/Instances/MI_ColdLight.MI_ColdLight")
        (`ActorComponent.K2_DestroyComponent` (`self.BP_InteractionComponent`))))
    (else
      (`/Engine/EditorBlueprintResources/StandardMacros.DoOnce` false
        (:`Completed`
          (`|ExecutionSequence`
            (:`then_0`
              ;[1 1 1] Apertura sportelli
              (bind (_direction _rotatortrack) (`Timeline|T_DoorB_Opener`)
                (:`Update`
                  (`SceneComponent.K2_SetRelativeRotation` (`self.SM_ElectricBox_Door_B`) (`KismetMathLibrary.MakeRotator` 0.0 0.0 _rotatortrack) false false)
                  (`KismetSystemLibrary.Delay` 1.0)
                  (set `self.B_AreDoorsOpen` true))))
            (:`then_1`
              (bind (_direction_2 _rotatortrack_2) (`Timeline|T_DoorA_Opener`)
                (:`Update`
                  (`SceneComponent.K2_SetRelativeRotation` (`self.SM_ElectricBox_Door_A`) (`KismetMathLibrary.MakeRotator` 0.0 0.0 _rotatortrack_2) false false))))))))))

(fn `LookAt`
  (returns (Message :type Text))
  (return ""))

(fn `UserConstructionScript`)