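; BP_RoboArm is a one-shot triggered set piece in which a robotic arm moves, then breaks loose.
; Overlapping the trigger destroys it, plays a sliding sound and starts a timeline that drives the arm's relative location.
; When the timeline finishes, the arm switches to physics simulation with impact and delayed debris sounds.
; Its light flickers via a light function before going dark, and actor collision is disabled after a short delay.
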(event `self.Trigger.OnComponentBeginOverlap`
  (params (OverlappedComponent :type "PrimitiveComponent Object Reference") (OtherActor :type "Actor Object Reference") (OtherComp :type "PrimitiveComponent Object Reference") (OtherBodyIndex :type Integer) (bFromSweep :type Boolean) (SweepResult :type "HitResult Structure (by ref)"))
  (bind _armlight (`self.ArmLight`))
  (`ActorComponent.K2_DestroyComponent` (`self.Trigger`))
  (`GameplayStatics.PlaySoundAtLocation` "/Game/BO_Custom/SOUNDS/TUT_LEV/Cues/SC_SlidingDoor.SC_SlidingDoor" (`SceneComponent.K2_GetComponentLocation` (`self.RoboArm`)) (struct) 1.0 1.0 0.0 null null null null)
  (bind (_direction _roboarmtrack) (`Timeline|T_RoboArm`)
    (:`Update`
      (`SceneComponent.K2_SetRelativeLocation` (`self.RoboArm`) _roboarmtrack false false))
    (:`Finished`
      (`PrimitiveComponent.SetSimulatePhysics` (`self.RoboArm`) true)
      (`|ExecutionSequence`
        (:`then_0`
          (`KismetSystemLibrary.Delay` 1.0)
          (`self.SetActorEnableCollision` false))
        (:`then_1`
          (`GameplayStatics.PlaySound2D` "/Game/Level_1/Environment/Sounds/METAL_DOOR_IMPACT.METAL_DOOR_IMPACT" 1.0 1.0 0.0 null null)
          (`KismetSystemLibrary.Delay` 1.0)
          (`GameplayStatics.PlaySound2D` "/Game/Level_1/Environment/Sounds/METAL_DEBRIS.METAL_DEBRIS" 1.0 1.0 0.0 null null))
        (:`then_2`
          (`LightComponent.SetLightFunctionMaterial` _armlight "/Game/3DAssetLevel/LevelDesign/Materials/LightFunctionMats/LF_Flickering.LF_Flickering")
          (`KismetSystemLibrary.Delay` 1.0)
          (`LightComponent.SetIntensity` _armlight 0.0))))))

(fn `UserConstructionScript`)