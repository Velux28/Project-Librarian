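; Interactable emergency switch in the storage level that opens the exit and container doors, wakes an NPC and powers the lamps.
; On interaction it opens the referenced exit, calls the container doors actor, plays a flickering sound and activates every storage lamp.
; After a short delay it activates the referenced AI with a fixed-patrol behavior tree and seeds its blackboard with the first patrol point.
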(event `/Game/BP_BO/Inventory/BPI_InteractInterface.InteractWith`
  (params (PlayerCharacter :type "/Game/BP_BO/PlayerCharacter/BP_TPCharacter Object Reference"))
  (bind _ai_reference (`self.AI_Reference`))
  (bind _doorref (`self.DoorRef`))
  (`|ExecutionSequence`
    (:`then_0`
      (`/Engine/EditorBlueprintResources/StandardMacros.IsValid` _doorref
        (:`Is Valid`
          (`/Game/3DAssetLevel/LevelDesign/Blueprints/Mechanics_BP/BP_GENERIC/BP_VertDoor_EXIT.Open Exit` _doorref))))
    (:`then_1`
      (bind _returnvalue (`GameplayStatics.GetActorOfClass` "/Game/3DAssetLevel/LevelDesign/Blueprints/Mechanics_BP/BP_STORAGE/BP_ContainerDoors.BP_ContainerDoors_C"))
      (`/Game/3DAssetLevel/LevelDesign/Blueprints/Mechanics_BP/BP_STORAGE/BP_ContainerDoors.Open Container` _returnvalue))
    (:`then_2`
      (`KismetSystemLibrary.Delay` 3.0)
      ;[1 1 1] Attivazione Udito I.A.
      (`/Game/BP_BO/ArtificialIntelligence/AC_AIActivator.Activate AI` (`self.AC_AIActivator`) _ai_reference "/Game/BP_BO/ArtificialIntelligence/BT_NPC_FixedPatrol.BT_NPC_FixedPatrol")
      (bind _asai_npc (cast `/Game/BP_BO/ArtificialIntelligence/AI_NPC` (`Pawn.GetController` _ai_reference)))
      (bind _keys (`BlueprintMapLibrary.Map_Keys` (`/Game/BP_BO/ArtificialIntelligence/AI_AC_Behaviour.PatrolPath` (`/Game/BP_BO/ArtificialIntelligence/BP_NPC.AI_AC_Behaviour` _ai_reference))))
      (`BlackboardComponent.SetValueAsVector` (`AIController.Blackboard` _asai_npc) "CurrPatrolPos" (`self.K2_GetActorLocation` (`|GetArrayItem` _keys))))
    (:`then_3`
      ;[1 1 1] Accensione Luci
      (`GameplayStatics.PlaySoundAtLocation` "/Game/3DAssetLevel/NewRoom/Sound/FlickeringLight.FlickeringLight" (`SceneComponent.K2_GetComponentLocation` (`self.EmergencySwitch`)) (struct) 1.0 1.0 0.0 null null null null)
      (bind _outactors (`GameplayStatics.GetAllActorsOfClass` "/Game/3DAssetLevel/LevelDesign/Blueprints/Mechanics_BP/BP_STORAGE/BP_StorageLamp.BP_StorageLamp_C"))
      (`/Game/3DAssetLevel/LevelDesign/Blueprints/Mechanics_BP/BP_STORAGE/BP_StorageLamp.EV_LampsActivation` _outactors))))

(fn `LookAt`
  (returns (Message :type Text))
  (return ""))

(fn `UserConstructionScript`)