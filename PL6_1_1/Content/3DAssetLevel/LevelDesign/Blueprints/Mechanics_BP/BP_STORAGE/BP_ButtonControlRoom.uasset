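; BP_ButtonControlRoom is an interactable control room button that ends the lockdown, usable only once.
; On interaction it plays a shutdown sound at the button and waits briefly.
; It then finds the control monitor, alarm and door button actors by class, calling the lockdown-off event on the first two and clearing the door button's lockdown flag.
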(event `/Game/BP_BO/Inventory/BPI_InteractInterface.InteractWith`
  (params (PlayerCharacter :type "/Game/BP_BO/PlayerCharacter/BP_TPCharacter Object Reference"))
  (`/Engine/EditorBlueprintResources/StandardMacros.DoOnce` false
    (:`Completed`
      (`GameplayStatics.PlaySoundAtLocation` "/Engine/VREditor/Sounds/SC_LockdownShutdown.SC_LockdownShutdown" (`SceneComponent.K2_GetComponentLocation` (`self.Button`)) (struct) 1.0 1.0 0.0 null null null null)
      (`KismetSystemLibrary.Delay` 2.0)
      (`|ExecutionSequence`
        (:`then_0`
          (bind _returnvalue (`GameplayStatics.GetActorOfClass` "/Game/3DAssetLevel/LevelDesign/Blueprints/Mechanics_BP/BP_STORAGE/BP_ControlMonitor.BP_ControlMonitor_C"))
          (`/Game/3DAssetLevel/LevelDesign/Blueprints/Mechanics_BP/BP_STORAGE/BP_ControlMonitor.EV_LockdownOff` _returnvalue))
        (:`then_1`
          (bind _returnvalue_2 (`GameplayStatics.GetActorOfClass` "/Game/3DAssetLevel/LevelDesign/Blueprints/Mechanics_BP/BP_STORAGE/BP_ControlAlarm.BP_ControlAlarm_C"))
          (`/Game/3DAssetLevel/LevelDesign/Blueprints/Mechanics_BP/BP_STORAGE/BP_ControlAlarm.EV_LockdownOff` _returnvalue_2))
        (:`then_2`
          (bind _returnvalue_3 (`GameplayStatics.GetActorOfClass` "/Game/3DAssetLevel/LevelDesign/Blueprints/Mechanics_BP/BP_STORAGE/BP_Control_DoorButton.BP_Control_DoorButton_C"))
          (set `/Game/3DAssetLevel/LevelDesign/Blueprints/Mechanics_BP/BP_STORAGE/BP_Control_DoorButton.IsLockdown` false _returnvalue_3))))))

(fn `LookAt`
  (returns (Message :type Text))
  (return ""))

(fn `UserConstructionScript`)