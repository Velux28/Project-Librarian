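; A one-shot lamp event that flickers on briefly and then dies, triggered when something overlaps its box.
; The point light starts hidden, and the first overlap destroys the trigger box so it cannot fire again.
; It then plays a flickering sound, reveals the light and gives the lamp mesh a flicker material.
; After a short delay it destroys the light and turns the lamp material black.
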(event `self.ReceiveBeginPlay`
  (`SceneComponent.SetVisibility` (`self.pointLight_0`) false false))

(event `self.Box.OnComponentBeginOverlap`
  (params (OverlappedComponent :type "PrimitiveComponent Object Reference") (OtherActor :type "Actor Object Reference") (OtherComp :type "PrimitiveComponent Object Reference") (OtherBodyIndex :type Integer) (bFromSweep :type Boolean) (SweepResult :type "HitResult Structure (by ref)"))
  (`ActorComponent.K2_DestroyComponent` (`self.Box`))
  (`GameplayStatics.PlaySoundAtLocation` "/Game/3DAssetLevel/NewRoom/Sound/FlickeringLight.FlickeringLight" (`SceneComponent.K2_GetComponentLocation` (`self.pointLight_0`)) (struct) 1.0 1.0 0.0 null null null null)
  (`SceneComponent.SetVisibility` (`self.pointLight_0`) true false)
  (`PrimitiveComponent.SetMaterial` (`self.LAMP`) 0 "/Game/Level_1/Environment/Lighting/M_LightFunction_Flicker.M_LightFunction_Flicker")
  (`KismetSystemLibrary.Delay` 2.0)
  (`ActorComponent.K2_DestroyComponent` (`self.pointLight_0`))
  (`PrimitiveComponent.SetMaterial` (`self.LAMP`) 0 "/Game/StarterContent/Materials/M_BLACK.M_BLACK"))

(fn `UserConstructionScript`)