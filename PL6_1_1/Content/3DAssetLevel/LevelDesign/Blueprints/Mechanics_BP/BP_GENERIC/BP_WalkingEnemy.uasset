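; BP_WalkingEnemy is a scripted robot enemy that walks along a spline path and then removes itself.
; STARTWALK sets the walking flag, loops the walk animation on the Enemy mesh and destroys the actor after a fixed delay.
; While walking, Tick advances the distance along EnemyPath by SplineSpeed and moves the mesh to that local spline transform, with a yaw offset to correct its facing.
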(event `START  WALK`
  (set `self.IsWalking` true)
  (`SkeletalMeshComponent.PlayAnimation` (`self.Enemy`) "/Game/3DAssetLevel/LevelDesign/Animations/NPC_IA/Robot_A/Anim/ANIM_Robot_Walk_2.ANIM_Robot_Walk_2" true)
  (`KismetSystemLibrary.Delay` 8.0)
  (`self.K2_DestroyActor`))

(event `self.ReceiveTick`
  (params (DeltaSeconds :type "Float (single-precision)"))
  (bind _enemy (`self.Enemy`))
  (bind _distancealongspline (`self.DistanceAlongSpline`))
  (bind _returnvalue (`SplineComponent.GetTransformAtDistanceAlongSpline` (`self.EnemyPath`) _distancealongspline "Local" false))
  (if (`self.IsWalking`)
    (set `self.DistanceAlongSpline` (+ (* DeltaSeconds (`self.SplineSpeed`)) _distancealongspline))
    (`SceneComponent.K2_SetRelativeTransform` _enemy (`KismetMathLibrary.MakeTransform` (`KismetMathLibrary.MakeVector` (.x (.location _returnvalue)) (.y (.location _returnvalue)) (.z (.location _returnvalue))) (`KismetMathLibrary.MakeRotator` (.roll (.rotation _returnvalue)) (.pitch (.rotation _returnvalue)) (+ (.yaw (.rotation _returnvalue)) -90.0)) (`SceneComponent.RelativeScale3D` _enemy)) false false)))

(fn `UserConstructionScript`)