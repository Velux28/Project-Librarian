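; Small sliding door Blueprint that closes once when either of its two trigger boxes is overlapped.
; The overlap destroys both triggers, plays the sliding sound and runs a timeline that drives the door's relative Y position.
; The RectLight is destroyed after a short delay to save performance without going dark too early.
; A deprecated, disconnected branch would play an NPC animation intended to cast a shadow.
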(event `self.TriggerBox.OnComponentBeginOverlap`
  (params (OverlappedComponent :type "PrimitiveComponent Object Reference") (OtherActor :type "Actor Object Reference") (OtherComp :type "PrimitiveComponent Object Reference") (OtherBodyIndex :type Integer) (bFromSweep :type Boolean) (SweepResult :type "HitResult Structure (by ref)"))
  (`ActorComponent.K2_DestroyComponent` (`self.TriggerBox`) :!label _label)
  (`ActorComponent.K2_DestroyComponent` (`self.TriggerBox1`))
  (`|ExecutionSequence`
    (:`then_0`)
    (:`then_1`
      ;[1 1 1] Chiudo la porta
      (`GameplayStatics.PlaySoundAtLocation` "/Game/BO_Custom/SOUNDS/TUT_LEV/Cues/SC_SlidingDoor.SC_SlidingDoor" (`SceneComponent.K2_GetComponentLocation` (`self.DefaultSceneRoot`)) (struct) 1.0 1.0 0.2 null null null null)
      (bind (_direction _doorclosing) (`Timeline|T_CloseDoor`)
        (:`Update`
          (`SceneComponent.K2_SetRelativeLocation` (`self.ContDoor`) (`KismetMathLibrary.MakeVector` -200.0 _doorclosing) false false))))
    (:`then_2`
      ;[1 1 1] Distruggo la RecLight (anche per le performance)
      (`KismetSystemLibrary.Delay` 0.6) ; Serve per non spegnerla presto
      (`ActorComponent.K2_DestroyComponent` (`self.RectLight`)))))

(event `self.TriggerBox1.OnComponentBeginOverlap`
  (params (OverlappedComponent :type "PrimitiveComponent Object Reference") (OtherActor :type "Actor Object Reference") (OtherComp :type "PrimitiveComponent Object Reference") (OtherBodyIndex :type Integer) (bFromSweep :type Boolean) (SweepResult :type "HitResult Structure (by ref)"))
  (goto _label))

(fn `UserConstructionScript`)