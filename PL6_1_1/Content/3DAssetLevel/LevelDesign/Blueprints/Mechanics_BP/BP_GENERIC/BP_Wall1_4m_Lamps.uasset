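; BP_Wall1_4m_Lamps is a generic 4m wall piece with three lamps that can be powered on.
; The EV_LampsPowerOn event swaps the lamp meshes to a cold emissive-style light material and makes the RectLight visible, with no matching power-off logic.
; The construction script optionally creates a dynamic instance of the wall material to apply a custom MetalColor.
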(event `EV_LampsPowerOn`
  (`PrimitiveComponent.SetMaterial` (`self.Lamp2`) 1 "/Game/3DAssetLevel/3DArt/Materials/MaterialInstances/GenericLighting/MI_Light_Cold.MI_Light_Cold")
  (`PrimitiveComponent.SetMaterial` (`self.Lamp`) 1 "/Game/3DAssetLevel/3DArt/Materials/MaterialInstances/GenericLighting/MI_Light_Cold.MI_Light_Cold")
  (`PrimitiveComponent.SetMaterial` (`self.Lamp1`) 1 "/Game/3DAssetLevel/3DArt/Materials/MaterialInstances/GenericLighting/MI_Light_Cold.MI_Light_Cold")
  (`SceneComponent.SetVisibility` (`self.RectLight`) true false))

(fn `UserConstructionScript`
  (if (`self.B_MetalColor`)
    (bind _returnvalue (`PrimitiveComponent.CreateDynamicMaterialInstance` (`self.StaticMesh`) 0 "/Game/3DAssetLevel/3DArt/Materials/MaterialInstances/MI_Muro1.MI_Muro1" "None"))
    (`MaterialInstanceDynamic.SetVectorParameterValue` _returnvalue "MetalColor" (`self.B_MetalColor_0`))))