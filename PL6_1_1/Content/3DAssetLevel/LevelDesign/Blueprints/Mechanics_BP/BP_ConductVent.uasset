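; BP_ConductVent is a ventilation duct cover that can open only after all four of its screws are removed.
; On BeginPlay it collects its BP_Screw child actors into an array.
; The OpenVent event checks that array and, once every screw is open, runs two chained timelines that move the door along Y, then slide it along X.
; A DoOnce keeps the opening from replaying, and the LookAt function returns an empty string.
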(event `self.ReceiveBeginPlay`
  (`|ExecutionSequence`
    (:`then_0`
      ;[1 1 1] Aggiungo le viti ad una lista per controllarle
      (bind _asbp_screw (cast `/Game/3DAssetLevel/LevelDesign/Blueprints/Mechanics_BP/BP_Screw` (`ChildActorComponent.ChildActor` (`self.BP_Screw`))))
      (`KismetArrayLibrary.Array_Add` (`self.Screws`) _asbp_screw))
    (:`then_1`
      (bind _asbp_screw_2 (cast `/Game/3DAssetLevel/LevelDesign/Blueprints/Mechanics_BP/BP_Screw` (`ChildActorComponent.ChildActor` (`self.BP_Screw1`))))
      (`KismetArrayLibrary.Array_Add` (`self.Screws`) _asbp_screw_2))
    (:`then_2`
      (bind _asbp_screw_3 (cast `/Game/3DAssetLevel/LevelDesign/Blueprints/Mechanics_BP/BP_Screw` (`ChildActorComponent.ChildActor` (`self.BP_Screw2`))))
      (`KismetArrayLibrary.Array_Add` (`self.Screws`) _asbp_screw_3))
    (:`then_3`
      (bind _asbp_screw_4 (cast `/Game/3DAssetLevel/LevelDesign/Blueprints/Mechanics_BP/BP_Screw` (`ChildActorComponent.ChildActor` (`self.BP_Screw3`))))
      (`KismetArrayLibrary.Array_Add` (`self.Screws`) _asbp_screw_4))))

(event `OpenVent`
  ;[0 0.7137 1] Se il condotto è chiuso e tutte le viti sono svitate lo apro
  (if (`self.B_IsOpen`)
    _
    (elif (`self.Is All Screw Open`)
      (`/Engine/EditorBlueprintResources/StandardMacros.DoOnce` false
        (:`Completed`
          (bind (_direction _openvent) (`Timeline|T_OpenVent`)
            (:`Update`
              (`SceneComponent.K2_SetRelativeLocation` (`self.VentDoor3`) (`KismetMathLibrary.MakeVector` 130.0 _openvent 130.0) false false))
            (:`Finished`
              (`KismetSystemLibrary.Delay` 0.2)
              (bind (_direction_2 _openvent_2) (`Timeline|T_SideMovement`)
                (:`Update`
                  (`SceneComponent.K2_SetRelativeLocation` (`self.VentDoor3`) (`KismetMathLibrary.MakeVector` _openvent_2 -12.0 130.0) false false)
                  (set `self.B_IsOpen` true))))))))))

(fn `Is All Screw Open`
  (returns (Result :type Boolean))
  (for _array_element (`self.Screws`)
    ;[0 0.6429 1] se una vite è ancora avvitata non controllo le altre
    (if (not (`/Game/3DAssetLevel/LevelDesign/Blueprints/Mechanics_BP/BP_Screw.B_ScrewOpen` _array_element))
      (return false)))
  (return true))

(fn `LookAt`
  (returns (Message :type Text))
  (return ""))

(fn `UserConstructionScript`)