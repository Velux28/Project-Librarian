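; BP_ElectricalBox is an interactable electrical box that opens linked level doors and activates an AI patrol.
; The first interaction plays two timelines that swing the box doors open and sets a flag when finished.
; A later interaction flips the switch with sound, swaps the red light for the OK light, and opens both target doors.
; After a short delay, ACAIActivator starts the assigned AI's fixed-patrol behavior tree, with each stage gated by DoOnce.
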(event `/Game/BP_BO/Inventory/BPI_InteractInterface.InteractWith`
  (params (PlayerCharacter :type "/Game/BP_BO/PlayerCharacter/BP_TPCharacter Object Reference"))
  (if (`self.B_AreDoorsOpen`)
    (`/Engine/EditorBlueprintResources/StandardMacros.DoOnce` false
      (:`Completed`
        (`|ExecutionSequence`
          (:`then_0`
            ;[1 1 1] Switch rotation e SFX
            (`SceneComponent.K2_SetRelativeRotation` (`self.SM_ElectricBox_Switch`) (struct :`Yaw` 90.0 :`Roll` 90.0) false false)
            (`GameplayStatics.PlaySoundAtLocation` "/Engine/VREditor/Sounds/UI/Flashlight_Switch.Flashlight_Switch" (`SceneComponent.RelativeLocation` (`self.SM_ElectricBox_Body`)) (struct) 1.0 1.0 0.0 null null null null)
            ;[1 1 1] Cambiamento luce
            (`SceneComponent.SetVisibility` (`self.RectLight-RED`) false false)
            (`SceneComponent.SetVisibility` (`self.RectLight-OK`) true false)
            (`PrimitiveComponent.SetMaterial` (`self.Lamp`) 1 "/Game/3DAssetLevel/LevelDesign/Materials/ENR_Mats/Instances/MI_ColdLight.MI_ColdLight")
            (`/Game/BP_BO/Puzzles/BPI_Unlockable.OpenTargetDoor` (`self.DoorToOpen`) self)
            (`/Game/BP_BO/Puzzles/BPI_Unlockable.OpenTargetDoor` (`self.DoorToOpen_0`) self))
          (:`then_1`
            ;[1 1 1] AI ACTIVATION
            (`KismetSystemLibrary.Delay` 1.0)
            (`/Game/BP_BO/ArtificialIntelligence/AC_AIActivator.Activate AI` (`self.AC_AIActivator`) (`self.AI to be activated`) "/Game/BP_BO/ArtificialIntelligence/BT_NPC_FixedPatrol.BT_NPC_FixedPatrol")))))
    (else
      (`/Engine/EditorBlueprintResources/StandardMacros.DoOnce` false
        (:`Completed`
          (`|ExecutionSequence`
            (:`then_0`
              ;[1 1 1] Apertura sportelli
              (bind (_direction _rotatortrack) (`Timeline|T_DoorB_Opener`)
                (:`Update`
                  (`SceneComponent.K2_SetRelativeRotation` (`self.SM_ElectricBox_Door_B`) (`KismetMathLibrary.MakeRotator` 0.0 0.0 _rotatortrack) false false))))
            (:`then_1`
              (bind (_direction_2 _rotatortrack_2) (`Timeline|T_DoorA_Opener`)
                (:`Update`
                  (`SceneComponent.K2_SetRelativeRotation` (`self.SM_ElectricBox_Door_A`) (`KismetMathLibrary.MakeRotator` 0.0 0.0 _rotatortrack_2) false false))
                (:`Finished`
                  (set `self.B_AreDoorsOpen` true))))))))))

(fn `UserConstructionScript`)