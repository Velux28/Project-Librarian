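; Interactable screw that can be removed once the screwdriver is collected, opening a conduct vent.
; A CollectedScrewdriver event sets the flag that lets Interactwith run a one-time sequence of two timelines, rotating the screw mesh and sliding it out along Z.
; When the exit finishes, a short delay precedes calling OpenVent on the BP_ConductVent found by class lookup and enabling physics on the screw.
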(event `CollectedScrewdriver`
  (set `self.B_HasScrewdriver` true))

(event `/Game/BP_BO/Inventory/BPI_InteractInterface.InteractWith`
  (params (PlayerCharacter :type "/Game/BP_BO/PlayerCharacter/BP_TPCharacter Object Reference"))
  (bind _sm_cylinder1 (`self.SM_Cylinder1`))
  (if (`self.B_HasScrewdriver`)
    (`/Engine/EditorBlueprintResources/StandardMacros.DoOnce` false
      (:`Completed`
        (`|ExecutionSequence`
          (:`then_0`
            (bind (_direction _screwrotation) (`Timeline|T_RotateScrew`)
              (:`Update`
                (`SceneComponent.K2_SetRelativeRotation` _sm_cylinder1 (`KismetMathLibrary.MakeRotator` 0.0 0.0 _screwrotation) false false))))
          (:`then_1`
            (bind (_direction_2 _driveexit) (`Timeline|T_ScrewExit`)
              (:`Update`
                (`SceneComponent.K2_SetRelativeLocation` _sm_cylinder1 (`KismetMathLibrary.MakeVector` 0.0 0.0 _driveexit) false false))
              (:`Finished`
                (`KismetSystemLibrary.Delay` 0.2)
                (bind _returnvalue (`GameplayStatics.GetActorOfClass` "/Game/3DAssetLevel/LevelDesign/Blueprints/Mechanics_BP/BP_ConductVent.BP_ConductVent_C"))
                (`/Game/3DAssetLevel/LevelDesign/Blueprints/Mechanics_BP/BP_ConductVent.OpenVent` _returnvalue)
                (`PrimitiveComponent.SetSimulatePhysics` (`self.SM_Cylinder1`) true)))))))))

(fn `LookAt`
  (returns (Message :type Text))
  (return ""))

(fn `UserConstructionScript`)