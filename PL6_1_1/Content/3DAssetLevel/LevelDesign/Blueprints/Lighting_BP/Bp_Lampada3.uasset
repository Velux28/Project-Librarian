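; Lamp actor with a rect light and a point light whose look is set by a selectable LampType preset.
; When AllowTypes is on, the construction script calls ClearElements to reset materials, intensity, temperature and light functions, then applies off, cold, warm, cold or warm flicker, or red.
; Presets swap the mesh material and drive both lights, with flicker using a light function material and red setting light color directly.
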(fn `ClearElements`
  (bind _rectlight (`self.RectLight`))
  (`PrimitiveComponent.SetMaterial` (`self.StaticMesh`) 0 null)
  (`LightComponent.SetIntensity` _rectlight 0.0)
  (`LightComponent.SetIntensity` (`self.PointLight`) 0.0)
  (`LightComponent.SetTemperature` _rectlight 0.0)
  (`LightComponent.SetTemperature` (`self.PointLight`) 0.0)
  (`LightComponent.SetLightFunctionMaterial` _rectlight null)
  (`LightComponent.SetLightFunctionMaterial` (`self.PointLight`) null)
  (set `self.StandardIntensity` (`self.StandardIntensity`))
  (set `self.LowIntensity` (`self.LowIntensity`)))

(fn `UserConstructionScript`
  (locals (NewLocalVar_0 :type Boolean :default false))
  (bind _rectlight (`self.RectLight`))
  (bind _rectlight_2 (`self.RectLight`))
  (bind _rectlight_3 (`self.RectLight`))
  (bind _rectlight_4 (`self.RectLight`))
  (bind _rectlight_5 (`self.RectLight`))
  (if (`self.Allow Types`)
    (if (`|EnumEquality` "NewEnumerator5" (`self.Lamp Type`))
      (`self.ClearElements`)
      (`PrimitiveComponent.SetMaterial` (`self.StaticMesh`) 1 "/Game/StarterContent/Materials/M_BLACK.M_BLACK")
      (`LightComponent.SetIntensity` (`self.RectLight`) 0.0)
      (`LightComponent.SetIntensity` (`self.PointLight`) 0.0)
      (elif (`|EnumEquality` "NewEnumerator0" (`self.Lamp Type`))
        (`self.ClearElements`)
        (`PrimitiveComponent.SetMaterial` (`self.StaticMesh`) 1 "/Game/3DAssetLevel/3DArt/Materials/MaterialInstances/GenericLighting/MI_Light_Cold.MI_Light_Cold")
        (`LightComponent.SetIntensity` _rectlight_4 (`self.StandardIntensity`))
        (`LightComponent.SetTemperature` _rectlight_4 10000.0)
        (`LightComponent.SetTemperature` (`self.PointLight`) 10000.0)
        (`LightComponent.SetIntensity` (`self.PointLight`) 40.0)
        (elif (`|EnumEquality` "NewEnumerator1" (`self.Lamp Type`))
          (`self.ClearElements`)
          (`PrimitiveComponent.SetMaterial` (`self.StaticMesh`) 1 "/Game/3DAssetLevel/3DArt/Materials/MaterialInstances/GenericLighting/MI_Light_Warm.MI_Light_Warm")
          (`LightComponent.SetIntensity` _rectlight_2 (`self.StandardIntensity`))
          (`LightComponent.SetTemperature` _rectlight_2 4000.0)
          (`LightComponent.SetTemperature` (`self.PointLight`) 4000.0)
          (`LightComponent.SetIntensity` (`self.PointLight`) 40.0)
          (elif (`|EnumEquality` "NewEnumerator2" (`self.Lamp Type`))
            (`self.ClearElements`)
            (`PrimitiveComponent.SetMaterial` (`self.StaticMesh`) 1 "/Game/3DAssetLevel/3DArt/Materials/MaterialInstances/GenericLighting/MI_ColdLight_Flicker.MI_ColdLight_Flicker")
            (`LightComponent.SetIntensity` _rectlight_3 (`self.StandardIntensity`))
            (`LightComponent.SetTemperature` _rectlight_3 10000.0)
            (`LightComponent.SetTemperature` (`self.PointLight`) 10000.0)
            (`LightComponent.SetLightFunctionMaterial` _rectlight_3 "/Game/3DAssetLevel/LevelDesign/Materials/LightFunctionMats/LF_Flickering.LF_Flickering")
            (`LightComponent.SetLightFunctionMaterial` (`self.PointLight`) "/Game/3DAssetLevel/LevelDesign/Materials/LightFunctionMats/LF_Flickering.LF_Flickering")
            (`LightComponent.SetIntensity` (`self.PointLight`) 40.0)
            (elif (`|EnumEquality` "NewEnumerator3" (`self.Lamp Type`))
              (`self.ClearElements`)
              (`PrimitiveComponent.SetMaterial` (`self.StaticMesh`) 1 "/Game/3DAssetLevel/3DArt/Materials/MaterialInstances/GenericLighting/MI_WarmLight_Flicker.MI_WarmLight_Flicker")
              (`LightComponent.SetIntensity` _rectlight_5 (`self.StandardIntensity`))
              (`LightComponent.SetTemperature` _rectlight_5 4000.0)
              (`LightComponent.SetTemperature` (`self.PointLight`) 4000.0)
              (`LightComponent.SetLightFunctionMaterial` _rectlight_5 "/Game/3DAssetLevel/LevelDesign/Materials/LightFunctionMats/LF_Flickering.LF_Flickering")
              (`LightComponent.SetLightFunctionMaterial` (`self.PointLight`) "/Game/3DAssetLevel/LevelDesign/Materials/LightFunctionMats/LF_Flickering.LF_Flickering")
              (`LightComponent.SetIntensity` (`self.PointLight`) 40.0)
              (elif (`|EnumEquality` "NewEnumerator4" (`self.Lamp Type`))
                (`self.ClearElements`)
                (`PrimitiveComponent.SetMaterial` (`self.StaticMesh`) 1 "/Game/C_MSF_Office/Materials/Lights/MI_Light_Red_LOW.MI_Light_Red_LOW")
                (`LightComponent.SetIntensity` _rectlight (`self.LowIntensity`))
                (`LightComponent.SetIntensity` (`self.PointLight`) (`self.LowIntensity`))
                (`LightComponent.SetLightColor` _rectlight (struct :`R` 1.0 :`A` 1.0) true)
                (`LightComponent.SetLightColor` (`self.PointLight`) (struct :`R` 1.0 :`A` 1.0) true)))))))))