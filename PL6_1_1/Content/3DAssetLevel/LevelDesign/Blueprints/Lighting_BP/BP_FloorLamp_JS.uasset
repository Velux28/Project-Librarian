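; Floor lamp jump scare that flickers once, the first time anything begins overlapping its trigger box.
; A sequence dims the point light and applies a flickering material as its light function and on the lamp mesh, while playing a flicker sound at the lamp.
; After the jump scare duration, the light brightens and both light and mesh switch to the cold light material.
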(event `self.TriggerBox.OnComponentBeginOverlap`
  (params (OverlappedComponent :type "PrimitiveComponent Object Reference") (OtherActor :type "Actor Object Reference") (OtherComp :type "PrimitiveComponent Object Reference") (OtherBodyIndex :type Integer) (bFromSweep :type Boolean) (SweepResult :type "HitResult Structure (by ref)"))
  (bind _jumpscare_duration (`self.JumpScare_Duration`))
  (bind _pointlight (`self.PointLight`))
  (bind _placeholderlamp (`self.PlaceholderLamp`))
  (`/Engine/EditorBlueprintResources/StandardMacros.DoOnce` false
    (:`Completed`
      (`|ExecutionSequence`
        (:`then_0`
          (`LightComponent.SetIntensity` _pointlight 12000.0)
          (`LightComponent.SetLightFunctionMaterial` _pointlight "/Game/3DAssetLevel/LevelDesign/Materials/LightFunctionMats/LF_Flickering.LF_Flickering")
          (`KismetSystemLibrary.Delay` _jumpscare_duration)
          (`LightComponent.SetIntensity` _pointlight 15000.0)
          (`LightComponent.SetLightFunctionMaterial` _pointlight "/Game/3DAssetLevel/LevelDesign/Materials/ENR_Mats/Instances/MI_ColdLight.MI_ColdLight"))
        (:`then_1`
          (`PrimitiveComponent.SetMaterial` _placeholderlamp 0 "/Game/3DAssetLevel/LevelDesign/Materials/LightFunctionMats/LF_Flickering.LF_Flickering")
          (`KismetSystemLibrary.Delay` _jumpscare_duration)
          (`PrimitiveComponent.SetMaterial` _placeholderlamp 0 "/Game/3DAssetLevel/LevelDesign/Materials/ENR_Mats/Instances/MI_ColdLight.MI_ColdLight"))
        (:`then_2`
          (`GameplayStatics.PlaySoundAtLocation` "/Game/StarterContent/Blueprints/Light_Flicker.Light_Flicker" (`SceneComponent.K2_GetComponentLocation` (`self.DefaultSceneRoot`)) (struct) 1.0 1.0 0.0 "/Game/SoundDesign/SA_BasicAttenuation.SA_BasicAttenuation" null null null))))))

(fn `UserConstructionScript`)