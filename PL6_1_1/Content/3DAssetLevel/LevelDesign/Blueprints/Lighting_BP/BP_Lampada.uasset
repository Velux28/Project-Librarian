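; BP_Lampada is a placeable lamp that pairs a static mesh with a rect light for level lighting.
; When IsManualEditable is set, the Construction Script reads the LampType enum to apply an off, cold, warm, cold flicker, warm flicker or red look.
; ClearElements resets the lamp first, then each look sets the mesh material and light intensity, plus temperature or color as needed.
; Flicker variants use the LF_Flickering light function material.
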(fn `ClearElements`
  (bind _rectlight (`self.RectLight`))
  (`PrimitiveComponent.SetMaterial` (`self.StaticMesh`) 0 null)
  (`LightComponent.SetIntensity` _rectlight 0.0)
  (`LightComponent.SetTemperature` _rectlight 0.0)
  (`LightComponent.SetLightFunctionMaterial` _rectlight null))

(fn `UserConstructionScript`
  (bind _rectlight (`self.RectLight`))
  (bind _rectlight_2 (`self.RectLight`))
  (bind _rectlight_3 (`self.RectLight`))
  (bind _rectlight_4 (`self.RectLight`))
  (bind _rectlight_5 (`self.RectLight`))
  (if (`self.IsManualEditable`)
    (if (`|EnumEquality` "NewEnumerator5" (`self.Lamp Type`))
      (`self.ClearElements`)
      (`PrimitiveComponent.SetMaterial` (`self.StaticMesh`) 0 "/Game/3DAssetLevel/3DArt/Materials/MaterialInstances/Roof_OvalLamp/MI_LuceOvale_spenta.MI_LuceOvale_spenta")
      (`LightComponent.SetIntensity` (`self.RectLight`) 0.0)
      (elif (`|EnumEquality` "NewEnumerator0" (`self.Lamp Type`))
        (`self.ClearElements`)
        (`PrimitiveComponent.SetMaterial` (`self.StaticMesh`) 0 "/Game/3DAssetLevel/3DArt/Materials/MaterialInstances/Roof_OvalLamp/MI_LuceOvale.MI_LuceOvale")
        (`LightComponent.SetIntensity` _rectlight_4 75.0)
        (`LightComponent.SetTemperature` _rectlight_4 10000.0)
        (elif (`|EnumEquality` "NewEnumerator1" (`self.Lamp Type`))
          (`self.ClearElements`)
          (`PrimitiveComponent.SetMaterial` (`self.StaticMesh`) 0 "/Game/3DAssetLevel/3DArt/Materials/MaterialInstances/Roof_OvalLamp/MI_LuceOvale_Warm.MI_LuceOvale_Warm")
          (`LightComponent.SetIntensity` _rectlight_2 75.0)
          (`LightComponent.SetTemperature` _rectlight_2 4000.0)
          (elif (`|EnumEquality` "NewEnumerator2" (`self.Lamp Type`))
            (`self.ClearElements`)
            (`PrimitiveComponent.SetMaterial` (`self.StaticMesh`) 0 "/Game/3DAssetLevel/3DArt/Materials/MaterialInstances/Roof_OvalLamp/MI_LuceOvale_Flick.MI_LuceOvale_Flick")
            (`LightComponent.SetIntensity` _rectlight_3 75.0)
            (`LightComponent.SetTemperature` _rectlight_3 10000.0)
            (`LightComponent.SetLightFunctionMaterial` _rectlight_3 "/Game/3DAssetLevel/LevelDesign/Materials/LightFunctionMats/LF_Flickering.LF_Flickering")
            (elif (`|EnumEquality` "NewEnumerator3" (`self.Lamp Type`))
              (`self.ClearElements`)
              (`PrimitiveComponent.SetMaterial` (`self.StaticMesh`) 0 "/Game/3DAssetLevel/3DArt/Materials/MaterialInstances/Roof_OvalLamp/MI_LuceOvale_Flick_Warm.MI_LuceOvale_Flick_Warm")
              (`LightComponent.SetIntensity` _rectlight_5 75.0)
              (`LightComponent.SetTemperature` _rectlight_5 4000.0)
              (`LightComponent.SetLightFunctionMaterial` _rectlight_5 "/Game/3DAssetLevel/LevelDesign/Materials/LightFunctionMats/LF_Flickering.LF_Flickering")
              (elif (`|EnumEquality` "NewEnumerator4" (`self.Lamp Type`))
                (`self.ClearElements`)
                (`PrimitiveComponent.SetMaterial` (`self.StaticMesh`) 0 "/Game/3DAssetLevel/3DArt/Materials/MaterialInstances/Roof_OvalLamp/MI_LuceOvale_RED.MI_LuceOvale_RED")
                (`LightComponent.SetIntensity` _rectlight 40.0)
                (`LightComponent.SetLightColor` _rectlight (struct :`R` 1.0 :`A` 1.0) true)))))))))