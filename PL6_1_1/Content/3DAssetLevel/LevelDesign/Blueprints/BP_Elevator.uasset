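; BP_Elevator is an elevator that runs a one-off automatic descent and door opening at level start.
; After a short delay on BeginPlay, a timeline drives the relative location of the MSElevator component.
; That timeline's Update output also feeds a longer Delay, which starts two door timelines that move LiftDoor1 and LiftDoor2 along relative X.
; No trigger or player input is involved.
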(event `self.ReceiveBeginPlay`
  (`KismetSystemLibrary.Delay` 1.5)
  ;[1 1 1] Discesa
  (bind (_direction _elevatortrack) (`Timeline|T_Elevator`)
    (:`Update`
      (`SceneComponent.K2_SetRelativeLocation` (`self.MS_Elevator`) _elevatortrack false false)
      ;[1 1 1] "Apertura porte"
      (`KismetSystemLibrary.Delay` 5.5)
      (`|ExecutionSequence`
        (:`then_0`
          (bind (_direction_2 _door1_open) (`Timeline|T_DoorOpen_1`)
            (:`Update`
              (`SceneComponent.K2_SetRelativeLocation` (`self.LiftDoor_1`) (`KismetMathLibrary.MakeVector` _door1_open) false false))))
        (:`then_1`
          (bind (_direction_3 _door1_open_2) (`Timeline|T_DoorOpen_2`)
            (:`Update`
              (`SceneComponent.K2_SetRelativeLocation` (`self.LiftDoor_2`) (`KismetMathLibrary.MakeVector` _door1_open_2) false false))))))))

(fn `UserConstructionScript`)