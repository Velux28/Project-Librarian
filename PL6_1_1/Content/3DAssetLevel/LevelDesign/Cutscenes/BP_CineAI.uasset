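; BP_CineAI is a trigger actor that plays the game's final cutscene of the AI awakening angry.
; On player overlap it removes the trigger, hides the character mesh, disables input, and starts LS_FinalCutscene with fake footstep sounds.
; A parallel Delay-timed chain flickers blue and red lights with face material swaps and sounds, ending in an alarm face and animation.
; It then stops the sequence and destroys the player character.
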(event `self.TriggerBox.OnComponentBeginOverlap`
  (params (OverlappedComponent :type "PrimitiveComponent Object Reference") (OtherActor :type "Actor Object Reference") (OtherComp :type "PrimitiveComponent Object Reference") (OtherBodyIndex :type Integer) (bFromSweep :type Boolean) (SweepResult :type "HitResult Structure (by ref)"))
  (bind _returnvalue (`GameplayStatics.GetPlayerCharacter` 0))
  ;[1 0.5 0] TriggerBox behavior
  (if (== OtherActor _returnvalue)
    (`|ExecutionSequence`
      (:`then_0`
        (`ActorComponent.K2_DestroyComponent` (`self.TriggerBox`))
        (`SceneComponent.SetVisibility` (`Character.Mesh` _returnvalue) false false)
        (`self.DisableInput` (`GameplayStatics.GetPlayerCharacter` 0) null))
      (:`then_1`
        ;;[1 1 1] LevelSequence
        (bind (_outactor _returnvalue_2) (`LevelSequencePlayer.CreateLevelSequencePlayer` "/Game/3DAssetLevel/LevelDesign/Cutscenes/LS_FinalCutscene.LS_FinalCutscene"))
        (`MovieSceneSequencePlayer.Play` _returnvalue_2)
        ;;[0.6057 0 1] Suono passi fake
        (`GameplayStatics.PlaySound2D` "/Game/SoundDesign/SoundWaves/Character_Walkstep_3.Character_Walkstep_3" 1.0 1.0 0.0 null null)
        (`KismetSystemLibrary.Delay` 1.0)
        (`GameplayStatics.PlaySound2D` "/Game/SoundDesign/SoundWaves/Character_Walkstep_2.Character_Walkstep_2" 1.0 1.0 0.0 null null)
        (`KismetSystemLibrary.Delay` 1.2)
        (`GameplayStatics.PlaySound2D` "/Game/SoundDesign/SoundWaves/Character_Walkstep_4.Character_Walkstep_4" 1.0 1.0 0.0 null null))
      (:`then_2`
        (`KismetSystemLibrary.Delay` 5.0) ; Tempo di zoom cinematic
        ;;[1 1 1] Primo sfarfallio
        (`PrimitiveComponent.SetMaterial` (`self.SK_AI`) 16 "/Game/3DAssetLevel/NewRoom/Material/M_BlueLight.M_BlueLight")
        (`SceneComponent.SetVisibility` (`self.BlueLight`) true false)
        (`GameplayStatics.PlaySound2D` "/Engine/VREditor/Sounds/VR_click1.VR_click1" 1.0 1.0 0.0 null null)
        (`KismetSystemLibrary.Delay` 0.2)
        (`PrimitiveComponent.SetMaterial` (`self.SK_AI`) 16 "/Game/StarterContent/Materials/M_BLACK.M_BLACK")
        (`SceneComponent.SetVisibility` (`self.BlueLight`) false false)
        (`KismetSystemLibrary.Delay` 1.8) ; Tempo di zoom cinematic
        ;;[1 1 1] Secondo sfarfallio
        (`PrimitiveComponent.SetMaterial` (`self.SK_AI`) 16 "/Game/C_MSF_Office/Materials/Lights/MI_Light_Red.MI_Light_Red")
        (`SceneComponent.SetVisibility` (`self.RedLight`) true false)
        (`GameplayStatics.PlaySound2D` "/Game/SoundDesign/SoundWaves/SFX_AI_Glitching_2.SFX_AI_Glitching_2" 0.2 1.0 0.0 null null)
        (`KismetSystemLibrary.Delay` 0.4)
        (`PrimitiveComponent.SetMaterial` (`self.SK_AI`) 16 "/Game/StarterContent/Materials/M_BLACK.M_BLACK")
        (`SceneComponent.SetVisibility` (`self.RedLight`) false false)
        (`KismetSystemLibrary.Delay` 0.2)
        (`PrimitiveComponent.SetMaterial` (`self.SK_AI`) 16 "/Game/C_MSF_Office/Materials/Lights/MI_Light_Red.MI_Light_Red")
        (`SceneComponent.SetVisibility` (`self.RedLight`) true false)
        (`KismetSystemLibrary.Delay` 0.6)
        (`PrimitiveComponent.SetMaterial` (`self.SK_AI`) 16 "/Game/StarterContent/Materials/M_BLACK.M_BLACK")
        (`SceneComponent.SetVisibility` (`self.RedLight`) false false)
        (`KismetSystemLibrary.Delay` 1.0) ; Tempo di zoom cinematic
        ;;[1 1 1] "Scena finale"
        (`PrimitiveComponent.SetMaterial` (`self.SK_AI`) 16 "/Game/3DAssetLevel/3DArt/Characters/Robot_V3/Materials/M_Face_panel_Alarm.M_Face_panel_Alarm")
        (`SceneComponent.SetVisibility` (`self.RedLight`) true false)
        (`GameplayStatics.PlaySound2D` "/Game/SoundDesign/SoundWaves/IA_Angry.IA_Angry" 1.0 1.0 0.0 null null) ; ANGRY AI SOUND
        (`SkeletalMeshComponent.SetAnimation` (`self.SK_AI`) "/Game/3DAssetLevel/3DArt/Characters/Robot_V3/Animations/TEST_Ugly/ANIM_TEST_Online.ANIM_TEST_Online")
        (`KismetSystemLibrary.Delay` 2.0)
        ;;[1 1 1] FINE GIOCO
        (`MovieSceneSequencePlayer.Stop` _returnvalue_2)
        (`self.K2_DestroyActor` (`GameplayStatics.GetPlayerCharacter` 0))))))

(fn `UserConstructionScript`)