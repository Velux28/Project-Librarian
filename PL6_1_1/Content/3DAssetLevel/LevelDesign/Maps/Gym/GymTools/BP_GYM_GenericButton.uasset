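; BP_GYM_GenericButton is a multipurpose test button for the gym map, with one action per instance chosen by boolean flags.
; On interact, it checks the flags in priority order to reset the QTE monitor, remove or spawn cans, or change directional light intensity or temperature.
; The AI switch branch forces the selected state on both showcase AI actors.
; Spawn and light actions use DoOnce with a short delay as a cooldown.
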(event `/Game/BP_BO/Inventory/BPI_InteractInterface.InteractWith`
  (params (PlayerCharacter :type "/Game/BP_BO/PlayerCharacter/BP_TPCharacter Object Reference"))
  (bind _e_aistates (`self.E_AIStates`))
  (bind _e_aistates_2 (`self.E_AIStates`))
  (bind _returnvalue_location (`KismetMathLibrary.BreakTransform` (`self.GetTransform` (`self.SpawnRef`))))
  (bind _lightcomponent (`Light.LightComponent` (`self.DirectionaLight`)))
  ;[0 0.4667 1] QTE RESET
  (if (`self.B_IsQTE_Reset`)
    (bind _returnvalue (`GameplayStatics.GetActorOfClass` "/Game/BP_BO/Puzzles/QTE_Puzzle/BP_QTE_Monitor.BP_QTE_Monitor_C"))
    (`/Game/BP_BO/Puzzles/QTE_Puzzle/BP_QTE_Monitor.Reset QTE` _returnvalue)
    (else
      ;[0 1 0.2667] ALL CANS REMOVAL
      (if (`self.B_IsCanRemoval`)
        (bind _outactors (`GameplayStatics.GetAllActorsOfClass` "/Game/BP_BO/Inventory/Items/BP_ThrowCan.BP_ThrowCan_C"))
        (`self.K2_DestroyActor` _outactors)
        (else
          ;[0 1 0.2667] CAN SPAWNER
          (if (`self.B_IsCanSpawner`)
            (`/Engine/EditorBlueprintResources/StandardMacros.DoOnce` false :!label _label
              (:`Completed`
                (`|SpawnActorFromClass` "/Game/BP_BO/Inventory/Items/BP_EnvCan.BP_EnvCan_C" (`KismetMathLibrary.MakeTransform` _returnvalue_location) "DontSpawnIfColliding" "OverrideRootScale" null null)
                (`KismetSystemLibrary.Delay` 0.5)
                (goto _label :!via `Reset`)))
            (else
              ;[1 0.9358 0.5417] TURN ON LIGHT
              (if (`self.B_IsLightSwitch_ON`)
                (`/Engine/EditorBlueprintResources/StandardMacros.DoOnce` false :!label _label_2
                  (:`Completed`
                    (`LightComponent.SetIntensity` _lightcomponent 10.0)
                    (`KismetSystemLibrary.Delay` 0.5)
                    (goto _label_2 :!via `Reset`)))
                (else
                  ;[1 0.9358 0.5417] TURN ON LIGHT
                  (if (`self.B_IsLightSwitch_OFF`)
                    (`/Engine/EditorBlueprintResources/StandardMacros.DoOnce` false :!label _label_3
                      (:`Completed`
                        (`LightComponent.SetIntensity` _lightcomponent 0.0)
                        (`KismetSystemLibrary.Delay` 0.5)
                        (goto _label_3 :!via `Reset`)))
                    (else
                      ;[1 0.9358 0.5417] SET TEMPERATURE
                      (if (`self.B_IsLightSwitch_TEMP`)
                        (`/Engine/EditorBlueprintResources/StandardMacros.DoOnce` false :!label _label_4
                          (:`Completed`
                            (`LightComponent.SetTemperature` _lightcomponent (`self.Light Temperature`))
                            (`KismetSystemLibrary.Delay` 0.5)
                            (goto _label_4 :!via `Reset`)))
                        (else
                          ;[1 0.9358 0.5417] SET TEMPERATURE
                          (if (`self.B_IsLightSwitch_RESET`)
                            (`/Engine/EditorBlueprintResources/StandardMacros.DoOnce` false :!label _label_5
                              (:`Completed`
                                (`LightComponent.SetTemperature` _lightcomponent 6500.0)
                                (`KismetSystemLibrary.Delay` 0.5)
                                (goto _label_5 :!via `Reset`)))
                            (else
                              ;[1 0.1779 0] AI STATES SIMULATION
                              (if (`self.IsAI_Switch`)
                                (`|ExecutionSequence`
                                  (:`then_0`
                                    (bind _returnvalue_2 (`GameplayStatics.GetActorOfClass` "/Game/3DAssetLevel/LevelDesign/Animations/NPC_IA/Robot_New/BP_AI_Showcase.BP_AI_Showcase_C"))
                                    (if (`|EnumEquality` _e_aistates "NewEnumerator0")
                                      (`/Game/3DAssetLevel/LevelDesign/Animations/NPC_IA/Robot_New/BP_AI_Showcase.Patrol` _returnvalue_2)
                                      (elif (`|EnumEquality` _e_aistates "NewEnumerator7")
                                        (`/Game/3DAssetLevel/LevelDesign/Animations/NPC_IA/Robot_New/BP_AI_Showcase.SoundHeard` _returnvalue_2)
                                        (elif (`|EnumEquality` _e_aistates "NewEnumerator1")
                                          (`/Game/3DAssetLevel/LevelDesign/Animations/NPC_IA/Robot_New/BP_AI_Showcase.Hunt` _returnvalue_2)
                                          (elif (`|EnumEquality` _e_aistates "NewEnumerator2")
                                            (`/Game/3DAssetLevel/LevelDesign/Animations/NPC_IA/Robot_New/BP_AI_Showcase.Scan` _returnvalue_2)
                                            (elif (`|EnumEquality` _e_aistates "NewEnumerator3")
                                              (`/Game/3DAssetLevel/LevelDesign/Animations/NPC_IA/Robot_New/BP_AI_Showcase.Spotted` _returnvalue_2)
                                              (elif (`|EnumEquality` _e_aistates "NewEnumerator4")
                                                (`/Game/3DAssetLevel/LevelDesign/Animations/NPC_IA/Robot_New/BP_AI_Showcase.Chase` _returnvalue_2)
                                                (elif (`|EnumEquality` _e_aistates "NewEnumerator6")
                                                  (`/Game/3DAssetLevel/LevelDesign/Animations/NPC_IA/Robot_New/BP_AI_Showcase.Attack` _returnvalue_2)))))))))
                                  (:`then_1`
                                    ;[1 0.1779 0] AI STATES SIMULATION
                                    (bind _returnvalue_3 (`GameplayStatics.GetActorOfClass` "/Game/3DAssetLevel/3DArt/Characters/Robot_V3/BP_AI_V3_Showcase.BP_AI_V3_Showcase_C"))
                                    (if (`|EnumEquality` _e_aistates_2 "NewEnumerator0")
                                      (`/Game/3DAssetLevel/3DArt/Characters/Robot_V3/BP_AI_V3_Showcase.Patrol` _returnvalue_3)
                                      (elif (`|EnumEquality` _e_aistates_2 "NewEnumerator7")
                                        (`/Game/3DAssetLevel/3DArt/Characters/Robot_V3/BP_AI_V3_Showcase.SoundHeard` _returnvalue_3)
                                        (elif (`|EnumEquality` _e_aistates_2 "NewEnumerator1")
                                          (`/Game/3DAssetLevel/3DArt/Characters/Robot_V3/BP_AI_V3_Showcase.Hunt` _returnvalue_3)
                                          (elif (`|EnumEquality` _e_aistates_2 "NewEnumerator2")
                                            (`/Game/3DAssetLevel/3DArt/Characters/Robot_V3/BP_AI_V3_Showcase.Scan` _returnvalue_3)
                                            (elif (`|EnumEquality` _e_aistates_2 "NewEnumerator3")
                                              (`/Game/3DAssetLevel/3DArt/Characters/Robot_V3/BP_AI_V3_Showcase.Spotted` _returnvalue_3)
                                              (elif (`|EnumEquality` _e_aistates_2 "NewEnumerator4")
                                                (`/Game/3DAssetLevel/3DArt/Characters/Robot_V3/BP_AI_V3_Showcase.Chase` _returnvalue_3)
                                                (elif (`|EnumEquality` _e_aistates_2 "NewEnumerator6")
                                                  (`/Game/3DAssetLevel/3DArt/Characters/Robot_V3/BP_AI_V3_Showcase.Attack` _returnvalue_3))))))))))))))))))))))))))

(fn `Check IF Interactable`
  (returns (`Is NOT Interactable` :type Boolean))
  (return false))

(fn `UserConstructionScript`)