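; BP_Gym_SaveSwitcher is a gym test tool actor that toggles whether the gym game mode loads a save file.
; On BeginPlay it casts the current game mode to BP_GymGamemode and caches it.
; Each Interactwith event flips that game mode's LoadSaveFile flag, then swaps the cube's material to green when enabled or red when disabled.
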(event `self.ReceiveBeginPlay`
  (bind _asbp_gym_gamemode (cast `/Game/BP_BO/GameModes/BP_GymGamemode` (`GameplayStatics.GetGameMode`)))
  (set `self.As BP Gym Gamemode` _asbp_gym_gamemode))

(event `/Game/BP_BO/Inventory/BPI_InteractInterface.InteractWith`
  (params (PlayerCharacter :type "/Game/BP_BO/PlayerCharacter/BP_TPCharacter Object Reference"))
  (bind _cube (`self.Cube`))
  (bind _as_bp_gym_gamemode (`self.As BP Gym Gamemode`)
    (:`then`
      (bind _output_get (set `/Game/BP_BO/GameModes/BP_GymGamemode.LoadSaveFile` (not (`/Game/BP_BO/GameModes/BP_GymGamemode.LoadSaveFile` _as_bp_gym_gamemode)) _as_bp_gym_gamemode))
      (if _output_get
        (`PrimitiveComponent.SetMaterial` _cube 0 "/Game/StarterContent/Materials/M_GREEN.M_GREEN")
        (else
          (`PrimitiveComponent.SetMaterial` _cube 0 "/Game/StarterContent/Materials/M_RED.M_RED"))))
    (:`else`)))

(fn `UserConstructionScript`)