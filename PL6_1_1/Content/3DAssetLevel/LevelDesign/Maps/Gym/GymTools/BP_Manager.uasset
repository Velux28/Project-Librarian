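; Gym test-level button manager that controls a referenced robot's AI when interacted with, branching on its button type.
; The activator type starts the robot's chosen behavior tree through ACAIActivator; other handled types only print out-of-service or "Nothing happens" messages.
; DoOnce gates and cross-calling reset events link activation, deactivation and respawn at a spawn reference.
; Author notes flag reset and deactivation as broken because the AI cannot be reactivated afterward.
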(event `EV_Reset_Reset`
  ;[1 0 0] Non va - non si riesce poi a farlo ripartire dal bottone Activator
  (`/Engine/EditorBlueprintResources/StandardMacros.DoOnce` false :!via `Reset`
    (:`Completed`
      (`self.K2_SetActorLocation` (`self.Robot Reference`) (`SceneComponent.K2_GetComponentLocation` (`/Game/3DAssetLevel/LevelDesign/Maps/Gym/GymTools/BP_SpawnRef.RefMesh` (`self.SpwnRef`))) false false)
      (bind _robot_reference (`self.Robot Reference`)
        (:`then`
          (`/Game/BP_BO/ArtificialIntelligence/AC_AIActivator.De-activate AI` (`self.AC_AIActivator`) _robot_reference)
          (`self.EV_Reset_Activator`))
        (:`else`)))))

(event `/Game/BP_BO/Inventory/BPI_InteractInterface.InteractWith`
  (params (PlayerCharacter :type "/Game/BP_BO/PlayerCharacter/BP_TPCharacter Object Reference"))
  (if (`|EnumEquality` (`self.ButtonType`) "NewEnumerator0")
    (`KismetSystemLibrary.PrintText` "OUT OF SERVICE - LOOK AT BP" true false (struct :`R` 1.0 :`G` 0.025803 :`A` 1.0) 4.0)
    (elif (`|EnumEquality` (`self.ButtonType`) "NewEnumerator7")
      (`KismetSystemLibrary.PrintText` "Nothing happens..." true false (struct :`R` 1.0 :`G` 0.025803 :`A` 1.0) 4.0)
      (elif (`|EnumEquality` (`self.ButtonType`) "NewEnumerator1")
        (`KismetSystemLibrary.PrintText` "OUT OF SERVICE - LOOK AT BP" true false (struct :`R` 1.0 :`G` 0.025803 :`A` 1.0) 4.0)
        (elif (`|EnumEquality` (`self.ButtonType`) "NewEnumerator8")
          (`/Engine/EditorBlueprintResources/StandardMacros.DoOnce` false :!label _label
            (:`Completed`
              (bind _robot_reference (`self.Robot Reference`)
                (:`then`
                  (`/Game/BP_BO/ArtificialIntelligence/AC_AIActivator.Activate AI` (`self.AC_AIActivator`) _robot_reference (`self.Desired BT`))
                  (`self.EV_Reset_Reset`)
                  (`self.EV_Reset_Deactivator`))
                (:`else`)))))))))

(event `EV_Reset_Deactivator`
  ;[1 0 0] Non va - spegne l'IA ma poi non la si può più riattivare col bottone Activator
  (`/Engine/EditorBlueprintResources/StandardMacros.DoOnce` false :!via `Reset`
    (:`Completed`
      (bind _robot_reference (`self.Robot Reference`)
        (:`then`
          (`/Game/BP_BO/ArtificialIntelligence/AC_AIActivator.De-activate AI` (`self.AC_AIActivator`) _robot_reference)
          (`self.EV_Reset_Activator`))
        (:`else`)))))

(event `EV_Reset_Activator`
  (goto _label :!via `Reset`))

(fn `Check IF Interactable`
  (returns (`Is NOT Interactable` :type Boolean))
  (return false))

(fn `UserConstructionScript`)