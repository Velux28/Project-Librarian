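; Conveyor assembly line that carries randomly chosen static meshes along a spline.
; BeginPlay scales SpawnDelay by Speed, and a Tick-driven Delay repeatedly spawns plain Actors with runtime-added mesh components.
; A shared Timer advances by Speed, placing each item on the spline offset by its array index.
; Box overlaps destroy anything except non-player BP_NPCs, including the player, and rewind Timer one SpawnDelay to keep spacing.
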(event `self.ReceiveBeginPlay`
  (set `self.SpawnDelay` (* (`self.SpawnDelay`) (`self.Speed`)))
  (`self.SpawnItem` :!label _label))

(event `self.ReceiveTick`
  (params (DeltaSeconds :type "Float (single-precision)"))
  (`|ExecutionSequence`
    (:`then_0`
      (`KismetSystemLibrary.Delay` (`self.SpawnDelay`))
      (goto _label))
    (:`then_1`
      (set `self.Timer` (+ (* DeltaSeconds (`self.Speed`)) (`self.Timer`)))
      (`self.Move Obj`))))

(event `self.Box.OnComponentBeginOverlap`
  (params (OverlappedComponent :type "PrimitiveComponent Object Reference") (OtherActor :type "Actor Object Reference") (OtherComp :type "PrimitiveComponent Object Reference") (OtherBodyIndex :type Integer) (bFromSweep :type Boolean) (SweepResult :type "HitResult Structure (by ref)"))
  (if (not (and (!= OtherActor (`GameplayStatics.GetPlayerCharacter` 0)) (`.bSuccess` (cast `/Game/BP_BO/ArtificialIntelligence/BP_NPC` OtherActor :!pure true))))
    (`self.DestroyItem` OtherActor)))

(fn `DestroyItem`
  (params (ObjToDestroy :type "Actor Object Reference"))
  (`KismetArrayLibrary.Array_RemoveItem` (`self.Items`) ObjToDestroy)
  (set `self.Timer` (- (`self.Timer`) (`self.SpawnDelay`)))
  (`self.K2_DestroyActor` ObjToDestroy))

(fn `Move Obj`
  (for (_array_element _array_index) (`self.Items`)
    (`self.K2_SetActorLocation` _array_element (`SplineComponent.GetLocationAtTime` (`self.Spline`) (`KismetMathLibrary.FMax` (- (`self.Timer`) (* _array_index (`self.SpawnDelay`)))) "World" false) false false)))

(fn `SpawnItem`
  (locals (Temp :type "Actor Object Reference"))
  (bind _objtospawn (`self.ObjToSpawn`))
  (bind _returnvalue (`SplineComponent.GetTransformAtTime` (`self.Spline`) 0.0 "World" false false))
  (bind _returnvalue_2 (`|SpawnActorFromClass` "/Script/Engine.Actor" _returnvalue "AlwaysSpawn" "OverrideRootScale" null null))
  (bind _output_get (set `local.Temp` _returnvalue_2))
  (bind _returnvalue_3 (`AddComponent|NODE_AddStaticMeshComponent-1` :`self` _output_get :`RelativeTransform` _returnvalue))
  (`StaticMeshComponent.SetStaticMesh` _returnvalue_3 (`|GetArrayItem` _objtospawn (`KismetMathLibrary.RandomInteger` (`KismetArrayLibrary.Array_Length` _objtospawn))))
  (`KismetArrayLibrary.Array_Add` (`self.Items`) (`local.Temp`))
  (return))

(fn `UserConstructionScript`)