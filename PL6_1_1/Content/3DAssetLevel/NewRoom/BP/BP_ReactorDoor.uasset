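; Reactor door Blueprint built to slide its Door component open along X, though none of its graph logic is connected to a triggering event.
; The OpeningDoor timeline's update lerps the door position, sets materials on four lamps of an actor found by class, spawns an actor and calls PositionEvent on another found actor.
; A separate spawn node is also unreachable, and the construction script is empty.
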(fn `UserConstructionScript`)