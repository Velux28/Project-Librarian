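; BP_Reactor is an interactable reactor that opens the reactor doors once enough items are collected.
; CollectItem increments a counter, and Interactwith checks it for an exact match with ItemNeeded.
; On a match it calls OpenDoor on every BP_ReactorDoor in the level and swaps its cylinder's material.
; Otherwise it shows the W_NoCacciavite (no screwdriver) widget, then clears all widgets after a short delay.
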(event `self.InteractWith`
  (params (PlayerCharacter :type "Object Object Reference"))
  (if (== (`self.ItemCollected`) (`self.ItemNeeded`))
    (bind _outactors (`GameplayStatics.GetAllActorsOfClass` "/Game/NewRoom/BP/BP_ReactorDoor.BP_ReactorDoor_C"))
    (`/Game/NewRoom/BP/BP_ReactorDoor.OpenDoor` _outactors)
    (`PrimitiveComponent.SetMaterial` (`self.Shape_Cylinder`) 0 "/Game/NewRoom/Material/M_OpenDoor.M_OpenDoor")
    (else
      (bind _returnvalue (`|CreateWidget` "/Game/NewRoom/Widget/W_NoCacciavite.W_NoCacciavite_C"))
      (`UserWidget.AddToViewport` _returnvalue 0)
      (`KismetSystemLibrary.Delay` 2.0)
      (`WidgetLayoutLibrary.RemoveAllWidgets`))))

(event `CollectItem`
  (`/Engine/EditorBlueprintResources/StandardMacros.IncrementInt` (`self.ItemCollected`)))

(fn `UserConstructionScript`)