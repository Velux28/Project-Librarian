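; Trigger volume that makes room lights flicker when the first-person character overlaps it, by swapping their materials to a flicker material.
; Left and right macros find BP_Lights and BP_Lights2 by class and swap their light materials.
; The right macro's DoOnce gates a 2D sound and delayed swaps on two further lights, then exits to switch the BP_WindowLights light after another short delay.
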(event `self.Box.OnComponentBeginOverlap`
  (params (OverlappedComponent :type "PrimitiveComponent Object Reference") (OtherActor :type "Actor Object Reference") (OtherComp :type "PrimitiveComponent Object Reference") (OtherBodyIndex :type Integer) (bFromSweep :type Boolean) (SweepResult :type "HitResult Structure (by ref)"))
  (cast `/Game/FirstPerson/Blueprints/BP_FirstPersonCharacter` OtherActor)
  (`|ExecutionSequence`
    (:`then_0`
      (bind _returnvalue (`GameplayStatics.GetActorOfClass` "/Game/NewRoom/BP/BP_Lights.BP_Lights_C"))
      (`|ExecutionSequence`
        (:`then_0`
          (`PrimitiveComponent.SetMaterial` (`/Game/NewRoom/BP/BP_Lights.Light` _returnvalue) 0 "/Game/NewRoom/Material/M_FlickerWL.M_FlickerWL"))
        (:`then_1`
          (`PrimitiveComponent.SetMaterial` (`/Game/NewRoom/BP/BP_Lights.Light2` _returnvalue) 0 "/Game/NewRoom/Material/M_FlickerWL.M_FlickerWL"))
        (:`then_2`
          (`PrimitiveComponent.SetMaterial` (`/Game/NewRoom/BP/BP_Lights.Light3` _returnvalue) 0 "/Game/NewRoom/Material/M_FlickerWL.M_FlickerWL"))))
    (:`then_1`
      (bind _returnvalue_2 (`GameplayStatics.GetActorOfClass` "/Game/NewRoom/BP/BP_Lights2.BP_Lights2_C"))
      (`|ExecutionSequence`
        (:`then_0`
          (`PrimitiveComponent.SetMaterial` (`/Game/NewRoom/BP/BP_Lights2.Light` _returnvalue_2) 0 "/Game/NewRoom/Material/M_FlickerWL.M_FlickerWL"))
        (:`then_1`
          (`PrimitiveComponent.SetMaterial` (`/Game/NewRoom/BP/BP_Lights2.Light2` _returnvalue_2) 0 "/Game/NewRoom/Material/M_FlickerWL.M_FlickerWL")
          (`/Engine/EditorBlueprintResources/StandardMacros.DoOnce` false
            (:`Completed`
              (`GameplayStatics.PlaySound2D` "/Game/NewRoom/Sound/FlickeringLight.FlickeringLight" 1.0 1.0 0.0 null null)
              (`KismetSystemLibrary.Delay` 1.0)
              (`PrimitiveComponent.SetMaterial` (`/Game/NewRoom/BP/BP_Lights2.Light4` _returnvalue_2) 0 "/Game/NewRoom/Material/M_FlickerWL.M_FlickerWL")
              (`KismetSystemLibrary.Delay` 0.2)
              (`PrimitiveComponent.SetMaterial` (`/Game/NewRoom/BP/BP_Lights2.Light5` _returnvalue_2) 0 "/Game/NewRoom/Material/M_FlickerWL.M_FlickerWL")
              (bind _returnvalue_3 (`GameplayStatics.GetActorOfClass` "/Game/NewRoom/BP/BP_WindowLights.BP_WindowLights_C"))
              (`KismetSystemLibrary.Delay` 0.5)
              (`PrimitiveComponent.SetMaterial` (`/Game/NewRoom/BP/BP_WindowLights.Light` _returnvalue_3) 0 "/Game/NewRoom/Material/M_FlickerWL.M_FlickerWL"))))
        (:`then_2`
          (`PrimitiveComponent.SetMaterial` (`/Game/NewRoom/BP/BP_Lights2.Light3` _returnvalue_2) 0 "/Game/NewRoom/Material/M_FlickerWL.M_FlickerWL"))))))

(fn `UserConstructionScript`)