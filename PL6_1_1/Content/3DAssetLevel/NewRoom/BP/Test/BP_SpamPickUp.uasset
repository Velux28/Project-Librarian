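; Pickup actor that the player collects by rapidly pressing Interact, destroying itself when the press count reaches PressesNeeded.
; Overlap of its Box by BP_TPCharacter enables input and shows a SpamWidget; leaving disables input and removes it.
; Each press increments the count and updates the widget, while a short retriggerable delay after release resets progress when presses stop.
; LookAt returns an empty string.
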(event `InputAction|Interact`
  (params (Key :type "Key Structure"))
  (:`Pressed`
    (bind _result (`/Engine/EditorBlueprintResources/StandardMacros.IncrementFloat` (`self.Pressed Amount`))
      (:`  `
        (bind _output_get (set `self.Pressed Amount` _result))
        (if (== _output_get (`self.Presses Needed`))
          (`self.K2_DestroyActor`)
          (else
            (set `/Game/NewRoom/BP/Test/SpamWidget.Amount Pressed` (stale _output_get_2) (stale `self.Box.OnComponentBeginOverlap` _output_get) :!label _label))))))
  (:`Released`
    (`KismetSystemLibrary.RetriggerableDelay` 0.3)
    (bind _output_get_2 (set `self.Pressed Amount` 0.0))
    (goto _label)))

(event `self.Box.OnComponentBeginOverlap`
  (params (OverlappedComponent :type "PrimitiveComponent Object Reference") (OtherActor :type "Actor Object Reference") (OtherComp :type "PrimitiveComponent Object Reference") (OtherBodyIndex :type Integer) (bFromSweep :type Boolean) (SweepResult :type "HitResult Structure (by ref)"))
  (cast `/Game/BP_BO/PlayerCharacter/BP_TPCharacter` OtherActor)
  (`self.EnableInput` (`GameplayStatics.GetPlayerController` 0))
  (bind _returnvalue (`|CreateWidget` "/Game/NewRoom/BP/Test/SpamWidget.SpamWidget_C"))
  (bind _output_get (set `self.WidgetRef` _returnvalue))
  (`UserWidget.AddToViewport` _output_get 0)
  (set `/Game/NewRoom/BP/Test/SpamWidget.Presses Needed` (`self.Presses Needed`) _output_get))

(event `self.Box.OnComponentEndOverlap`
  (params (OverlappedComponent :type "PrimitiveComponent Object Reference") (OtherActor :type "Actor Object Reference") (OtherComp :type "PrimitiveComponent Object Reference") (OtherBodyIndex :type Integer))
  (cast `/Game/BP_BO/PlayerCharacter/BP_TPCharacter` OtherActor)
  (`self.DisableInput` (`GameplayStatics.GetPlayerController` 0))
  (`Widget.RemoveFromParent` (stale `self.Box.OnComponentBeginOverlap` _returnvalue)))

(fn `LookAt`
  (returns (Message :type Text))
  (return ""))

(fn `UserConstructionScript`)