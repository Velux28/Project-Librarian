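; Interactable generator that the player powers with a Power Cell to activate AI, unlock two buttons and open a target door.
; A trigger box outlines the cell holder while the player overlaps it.
; Successful interaction runs one-time feedback (green light, visible cell, energy beams, sounds) and increments an optional dispenser's count to allow saving again.
; Without a cell, a re-armed DoOnce shows a temporary HUD warning.
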(event `self.TriggerBox.OnComponentBeginOverlap`
  (params (OverlappedComponent :type "PrimitiveComponent Object Reference") (OtherActor :type "Actor Object Reference") (OtherComp :type "PrimitiveComponent Object Reference") (OtherBodyIndex :type Integer) (bFromSweep :type Boolean) (SweepResult :type "HitResult Structure (by ref)"))
  ;[1 1 1] Attiva/Disattiva l'Outline dell'oggetto
  (if (== OtherActor (`GameplayStatics.GetPlayerCharacter` 0))
    (`PrimitiveComponent.SetRenderCustomDepth` (`self.CellHolder 2`) true)))

(event `self.TriggerBox.OnComponentEndOverlap`
  (params (OverlappedComponent :type "PrimitiveComponent Object Reference") (OtherActor :type "Actor Object Reference") (OtherComp :type "PrimitiveComponent Object Reference") (OtherBodyIndex :type Integer))
  ;[1 1 1] Attiva/Disattiva l'Outline dell'oggetto
  (if (== OtherActor (`GameplayStatics.GetPlayerCharacter` 0))
    (`PrimitiveComponent.SetRenderCustomDepth` (`self.CellHolder 2`) false)))

(event `/Game/BP_BO/Inventory/BPI_InteractInterface.InteractWith`
  (params (PlayerCharacter :type "/Game/BP_BO/PlayerCharacter/BP_TPCharacter Object Reference"))
  (bind _light (`self.Light`))
  (if (`/Game/BP_BO/PlayerCharacter/BP_TPCharacter.HasPowerCell` PlayerCharacter)
    (`|ExecutionSequence`
      (:`then_0`
        ;[1 1 1] COSA ACCADE ALLA ACCENSIONE DEL GENERATORE?  [Es. aprire porte, accendere luci]
        (`/Game/BP_BO/ArtificialIntelligence/AC_AIActivator.Activate AI` (`self.AC_AIActivator`) (`self.AICharacter`) (`self.AIBT`)) ; Attivazione IA Assembly
        (`/Game/BP_BO/Puzzles/BPI_Unlockable.SetButtonUsable_Blue` (`self.ButtonToUnlock`) null) ; Bottone stanza dei generatori
        (`/Game/BP_BO/Puzzles/BPI_Unlockable.SetButtonUsable_Blue` (`self.ButtonToUnlock_2`) null) ; Bottone porta per MainHall
        (message `/Game/BP_BO/Puzzles/BPI_Unlockable.OpenTargetDoor` (`self.DoorToOpen`) self))
      (:`then_1`
        ;[0 1 0.9855] COME REAGISCE IL GENERATORE ALL'ATTIVAZIONE
        (`/Engine/EditorBlueprintResources/StandardMacros.DoOnce` false
          (:`Completed`
            (`PrimitiveComponent.SetMaterial` _light 0 "/Game/C_MSF_Props/Materials/AlarmLight/MI_AlarmLight_Glass_GREEN.MI_AlarmLight_Glass_GREEN")
            (`PrimitiveComponent.SetMaterial` _light 1 "/Game/3DAssetLevel/3DArt/Materials/MaterialInstances/GenericLighting/MI_GreenLight.MI_GreenLight")
            (`PrimitiveComponent.SetMaterial` _light 2 "/Game/C_MSF_Props/Materials/AlarmLight/MI_AlarmLight_GREEN.MI_AlarmLight_GREEN")
            ;;[1 1 1] Disabilito permanentemente l'Outline
            (`ActorComponent.K2_DestroyComponent` (`self.TriggerBox`))
            (`PrimitiveComponent.SetRenderCustomDepth` (`self.CellHolder 2`) false)
            (`GameplayStatics.PlaySound2D` "/Game/3DAssetLevel/NewRoom/New_Audio/big-metal-knock-001-11345.big-metal-knock-001-11345" 0.5 1.0 0.0 null null false)
            (`SceneComponent.SetVisibility` (`self.Cell 2`) true false)
            (`KismetSystemLibrary.Delay` 1.0)
            (`GameplayStatics.PlaySoundAtLocation` "/Game/SoundDesign/SoundCues/SFX_BP/SC_PowerUp.SC_PowerUp" (`SceneComponent.K2_GetComponentLocation` (`self.Generator`)) (struct) 1.0 1.0 0.0 "/Game/SoundDesign/SA_BasicAttenuation.SA_BasicAttenuation" null null null)
            (`SceneComponent.SetVisibility` (`self.EnergyBeam`) true false)
            (`SceneComponent.SetVisibility` (`self.EnergyBeam1`) true false)
            ;;[1 1 1] Permette di salvare nuovamente
            (bind _dispencer (`self.Dispencer`)
              (:`then`
                (`/Game/BP_BO/Environment/BP_CanDispenser.Increment Can Number` _dispencer))
              (:`else`))))))
    (else
      ;[1 0 0] COME REAGISCE IL GENERATORE ALLA MANCATA ATTIVAZIONE
      (`/Engine/EditorBlueprintResources/StandardMacros.DoOnce` false :!label _label
        (:`Completed`
          (`GameplayStatics.PlaySound2D` null 1.0 1.0 0.0 null null)
          (bind _returnvalue (`|CreateWidget` "/Game/UI/PlayerUI/Environment_UI/Objectives/W_HUD_NoScrewdriver.W_HUD_NoScrewdriver_C"))
          (`UserWidget.AddToViewport` _returnvalue 0)
          (`KismetSystemLibrary.Delay` 2.0)
          (`Widget.RemoveFromParent` _returnvalue)
          (goto _label :!via `Reset`))))))

(fn `Check IF Interactable`
  (returns (`Is NOT Interactable` :type Boolean))
  (return false))

(fn `UserConstructionScript`)