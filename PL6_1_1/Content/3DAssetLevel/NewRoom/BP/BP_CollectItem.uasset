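; BP_CollectItem is an interactable pickup that reports its collection to BP_Generator and triggers a scare cue.
; On Interactwith it calls CollectItem on every BP_Generator in the level and destroys itself.
; It then switches the four BP_LampChipRoom lamps to a flickering light-function material and plays a creepy 2D sound.
; LookAt returns empty text, and a disconnected branch for restoring white light after a delay never runs.
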(event `/Game/BP_BO/Inventory/BPI_InteractInterface.InteractWith`
  (params (PlayerCharacter :type "/Game/BP_BO/PlayerCharacter/BP_TPCharacter Object Reference"))
  (bind _outactors (`GameplayStatics.GetAllActorsOfClass` "/Game/3DAssetLevel/NewRoom/BP/BP_Generator.BP_Generator_C"))
  (`/Game/3DAssetLevel/NewRoom/BP/BP_Generator.CollectItem` _outactors)
  (`self.K2_DestroyActor`)
  (`|ExecutionSequence`
    (:`then_0`
      (bind _returnvalue (`GameplayStatics.GetActorOfClass` "/Game/3DAssetLevel/LevelDesign/Blueprints/Mechanics_BP/BP_ASSEMBLY/BP_LampChipRoom.BP_LampChipRoom_C"))
      (`PrimitiveComponent.SetMaterial` (`/Game/3DAssetLevel/LevelDesign/Blueprints/Mechanics_BP/BP_ASSEMBLY/BP_LampChipRoom.Lamp2` _returnvalue) 0 "/Game/Level_1/Environment/Lighting/M_LightFunction_Flicker.M_LightFunction_Flicker")
      (`PrimitiveComponent.SetMaterial` (`/Game/3DAssetLevel/LevelDesign/Blueprints/Mechanics_BP/BP_ASSEMBLY/BP_LampChipRoom.Lamp3` _returnvalue) 0 "/Game/Level_1/Environment/Lighting/M_LightFunction_Flicker.M_LightFunction_Flicker")
      (`PrimitiveComponent.SetMaterial` (`/Game/3DAssetLevel/LevelDesign/Blueprints/Mechanics_BP/BP_ASSEMBLY/BP_LampChipRoom.Lamp1` _returnvalue) 0 "/Game/Level_1/Environment/Lighting/M_LightFunction_Flicker.M_LightFunction_Flicker")
      (`PrimitiveComponent.SetMaterial` (`/Game/3DAssetLevel/LevelDesign/Blueprints/Mechanics_BP/BP_ASSEMBLY/BP_LampChipRoom.Lamp4` _returnvalue) 0 "/Game/Level_1/Environment/Lighting/M_LightFunction_Flicker.M_LightFunction_Flicker"))
    (:`then_1`
      (`GameplayStatics.PlaySound2D` "/Game/3DAssetLevel/NewRoom/Sound/227578-Just-Transitions-Creepy-068.227578-Just-Transitions-Creepy-068" 1.0 1.0 0.0 null null))))

(fn `LookAt`
  (returns (Message :type Text))
  (return ""))

(fn `UserConstructionScript`)