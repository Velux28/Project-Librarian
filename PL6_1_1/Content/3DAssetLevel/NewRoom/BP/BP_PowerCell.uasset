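; BP_PowerCell is a power cell pickup that the player collects by interacting with it.
; Its TriggerBox toggles custom depth rendering on the Cell component as the player character enters and leaves, showing or hiding an outline.
; The Interactwith event sets HasPowerCell on the passed PlayerCharacter and destroys the actor.
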(event `self.TriggerBox.OnComponentBeginOverlap`
  (params (OverlappedComponent :type "PrimitiveComponent Object Reference") (OtherActor :type "Actor Object Reference") (OtherComp :type "PrimitiveComponent Object Reference") (OtherBodyIndex :type Integer) (bFromSweep :type Boolean) (SweepResult :type "HitResult Structure (by ref)"))
  ;[1 1 1] Attiva/Disattiva l'Outline dell'oggetto
  (if (== OtherActor (`GameplayStatics.GetPlayerCharacter` 0))
    (`PrimitiveComponent.SetRenderCustomDepth` (`self.Cell`) true)))

(event `self.TriggerBox.OnComponentEndOverlap`
  (params (OverlappedComponent :type "PrimitiveComponent Object Reference") (OtherActor :type "Actor Object Reference") (OtherComp :type "PrimitiveComponent Object Reference") (OtherBodyIndex :type Integer))
  ;[1 1 1] Attiva/Disattiva l'Outline dell'oggetto
  (if (== (stale `self.TriggerBox.OnComponentBeginOverlap` OtherActor) (`GameplayStatics.GetPlayerCharacter` 0))
    (`PrimitiveComponent.SetRenderCustomDepth` (`self.Cell`) false)))

(event `/Game/BP_BO/Inventory/BPI_InteractInterface.InteractWith`
  (params (PlayerCharacter :type "/Game/BP_BO/PlayerCharacter/BP_TPCharacter Object Reference"))
  (set `/Game/BP_BO/PlayerCharacter/BP_TPCharacter.HasPowerCell` true PlayerCharacter)
  (`self.K2_DestroyActor`)
  (`|ExecutionSequence`))

(fn `UserConstructionScript`)