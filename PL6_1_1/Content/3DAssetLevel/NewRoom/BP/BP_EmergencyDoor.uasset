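; BP_EmergencyDoor is an emergency door that the player opens by rapidly spamming the Interact input.
; Box overlap with BP_FirstPersonCharacter enables input and shows a W_SpamE widget, removing both on exit.
; Presses count toward PressesNeeded, and a retriggerable delay on release resets the count when presses lapse.
; Reaching the target rotates the lever by timeline, with a delayed second timeline sliding the door open.
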(event `self.Box.OnComponentBeginOverlap`
  (params (OverlappedComponent :type "PrimitiveComponent Object Reference") (OtherActor :type "Actor Object Reference") (OtherComp :type "PrimitiveComponent Object Reference") (OtherBodyIndex :type Integer) (bFromSweep :type Boolean) (SweepResult :type "HitResult Structure (by ref)"))
  (cast `/Game/FirstPerson/Blueprints/BP_FirstPersonCharacter` OtherActor)
  (`self.EnableInput` (`GameplayStatics.GetPlayerController` 0))
  (bind _returnvalue (`|CreateWidget` "/Game/NewRoom/Widget/W_SpamE.W_SpamE_C"))
  (bind _output_get (set `self.SpamWidget` _returnvalue))
  (`UserWidget.AddToViewport` (`self.SpamWidget`) 0)
  (`UserWidget.AddToViewport` _output_get 0)
  (set `/Game/NewRoom/Widget/W_SpamE.Presses_Needed` (`self.Presses needed`) _output_get))

(event `self.Box.OnComponentEndOverlap`
  (params (OverlappedComponent :type "PrimitiveComponent Object Reference") (OtherActor :type "Actor Object Reference") (OtherComp :type "PrimitiveComponent Object Reference") (OtherBodyIndex :type Integer))
  (cast `/Game/FirstPerson/Blueprints/BP_FirstPersonCharacter` OtherActor)
  (`self.DisableInput` (`GameplayStatics.GetPlayerController` 0))
  (`Widget.RemoveFromParent` (stale `self.Box.OnComponentBeginOverlap` _output_get)))

(event `InputAction|Interact`
  (params (Key :type "Key Structure"))
  (:`Pressed`
    (bind _result (`/Engine/EditorBlueprintResources/StandardMacros.IncrementFloat` (`self.Pressed Amount`))
      (:`  `
        (bind _output_get (set `self.Pressed Amount` _result))
        (if (== _output_get (`self.Presses needed`))
          (bind (_direction _pulldown) (`Timeline|PullDown`)
            (:`Update`
              (`SceneComponent.K2_SetRelativeRotation` (`self.Leva`) (`KismetMathLibrary.RLerp` (struct :`Pitch` 28.182673) (struct :`Pitch` -40.0) _pulldown) false false)
              (`KismetSystemLibrary.Delay` 2.0)
              (bind (_direction_2 _x) (`Timeline|OpenDoor_X`)
                (:`Update`
                  (`SceneComponent.K2_SetRelativeLocation` (`self.E_Door`) (`KismetMathLibrary.VLerp` (0.0 0.0 0.0) (0.0 95.0 0.0) _x) false false)))))
          (else
            (set `/Game/NewRoom/Widget/W_SpamE.Pressed Amount` 0.0 (stale `self.Box.OnComponentBeginOverlap` _output_get)))))))
  (:`Released`
    (`KismetSystemLibrary.RetriggerableDelay` 0.3)
    (set `self.Pressed Amount` 0.0)))

(fn `UserConstructionScript`)