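; BP_Alberto is an actor that moves along a scripted, non-looping patrol through preset positions, stopping to scan with a swiping beam.
; PositionEvent handles initial placement; Patrol_1 starts chained events through Patrol6, neither triggered here.
; Timelines lerp root location and rotation, and three stops briefly spawn BP_ScanFX_SwipingBeam.
; Sequencing hangs Delays and next-leg calls off timeline Update pins rather than Finished.
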(event `PositionEvent`
  (bind (_direction _positioning) (`Timeline|Positioning`)
    (:`Update`
      (`SceneComponent.K2_SetWorldLocation` (`self.DefaultSceneRoot`) (`KismetMathLibrary.VLerp` (`self.PosA`) (`self.PosB`) _positioning) false false))))

(event `Patrol_1`
  (bind (_direction _patrolling1) (`Timeline|Patrolling1`)
    (:`Update`
      (`SceneComponent.K2_SetWorldLocation` (`self.DefaultSceneRoot`) (`KismetMathLibrary.VLerp` (`self.PosB`) (`self.PosC`) _patrolling1) false false)
      (`KismetSystemLibrary.Delay` 3.0)
      (bind (_direction_2 _rotation1) (`Timeline|Rotation1`)
        (:`Update`
          (`SceneComponent.K2_SetRelativeRotation` (`self.DefaultSceneRoot`) (`KismetMathLibrary.RLerp` (struct :`Yaw` 270.0) (struct :`Yaw` 180.0) _rotation1) false false)
          (`KismetSystemLibrary.Delay` 0.5)
          (bind _returnvalue (`|SpawnActorFromClass` "/Game/ScanFX/Blueprints/BP_ScanFX_SwipingBeam.BP_ScanFX_SwipingBeam_C" (`KismetMathLibrary.MakeTransform` (`self.SpawnBeam`) (struct :`Yaw` -90.0)) "Undefined" "OverrideRootScale" null null))
          (`KismetSystemLibrary.Delay` 3.0)
          (`self.K2_DestroyActor` _returnvalue)
          (`self.Patrol2`))))))

(event `Patrol2`
  (bind (_direction _patrolling2) (`Timeline|Patrolling2`)
    (:`Update`
      (`SceneComponent.K2_SetWorldLocation` (`self.DefaultSceneRoot`) (`KismetMathLibrary.VLerp` (`self.PosC`) (`self.PosD`) _patrolling2) false false)
      (`KismetSystemLibrary.Delay` 2.5)
      (bind (_direction_2 _rotation2) (`Timeline|Rotation2`)
        (:`Update`
          (`SceneComponent.K2_SetWorldRotation` (`self.DefaultSceneRoot`) (`KismetMathLibrary.RLerp` (struct :`Yaw` 180.0) (struct) _rotation2) false false)
          (`KismetSystemLibrary.Delay` 1.0)
          (`self.Patrol3`))))))

(event `Patrol3`
  (bind (_direction _patrolling3) (`Timeline|Patrolling3`)
    (:`Update`
      (`SceneComponent.K2_SetWorldLocation` (`self.DefaultSceneRoot`) (`KismetMathLibrary.VLerp` (`self.PosD`) (`self.PosC`) _patrolling3) false false)
      (`KismetSystemLibrary.Delay` 2.5)
      (bind (_direction_2 _rotation3) (`Timeline|Rotation3`)
        (:`Update`
          (`SceneComponent.K2_SetWorldRotation` (`self.DefaultSceneRoot`) (`KismetMathLibrary.RLerp` (struct) (struct :`Yaw` -90.0) _rotation3) false false)
          (`KismetSystemLibrary.Delay` 0.5)
          (bind _returnvalue (`|SpawnActorFromClass` "/Game/ScanFX/Blueprints/BP_ScanFX_SwipingBeam.BP_ScanFX_SwipingBeam_C" (`KismetMathLibrary.MakeTransform` (`self.SpawnBeam2`)) "Undefined" "OverrideRootScale" null null))
          (`KismetSystemLibrary.Delay` 3.0)
          (`self.K2_DestroyActor` _returnvalue)
          (`self.Patrol4`))))))

(event `Patrol4`
  (bind (_direction _patrolling4) (`Timeline|Patrolling4`)
    (:`Update`
      (`SceneComponent.K2_SetWorldLocation` (`self.DefaultSceneRoot`) (`KismetMathLibrary.VLerp` (`self.PosC`) (`self.PosE`) _patrolling4) false false)
      (`KismetSystemLibrary.Delay` 2.0)
      (bind (_direction_2 _rotation4) (`Timeline|Rotation4`)
        (:`Update`
          (`SceneComponent.K2_SetWorldRotation` (`self.DefaultSceneRoot`) (`KismetMathLibrary.RLerp` (struct) (struct :`Yaw` 90.0) _rotation4) false false)
          (`self.Patrol5`))))))

(event `Patrol5`
  (bind (_direction _patrolling5) (`Timeline|Patrolling5`)
    (:`Update`
      (`SceneComponent.K2_SetWorldLocation` (`self.DefaultSceneRoot`) (`KismetMathLibrary.VLerp` (`self.PosE`) (`self.PosF`) _patrolling5) false false)
      (`KismetSystemLibrary.Delay` 2.0)
      (bind (_direction_2 _rotation5) (`Timeline|Rotation5`)
        (:`Update`
          (`SceneComponent.K2_SetWorldRotation` (`self.DefaultSceneRoot`) (`KismetMathLibrary.RLerp` (struct :`Yaw` 90.0) (struct :`Yaw` 180.0) _rotation5) false false)
          (`self.Patrol6`))))))

(event `Patrol6`
  (bind (_direction _patrolling6) (`Timeline|Patrolling76`)
    (:`Update`
      (`SceneComponent.K2_SetWorldLocation` (`self.DefaultSceneRoot`) (`KismetMathLibrary.VLerp` (`self.PosF`) (`self.PosG`) _patrolling6) false false)
      (`KismetSystemLibrary.Delay` 2.0)
      (bind (_direction_2 _rotation6) (`Timeline|Rotation6`)
        (:`Update`
          (`SceneComponent.K2_SetWorldRotation` (`self.DefaultSceneRoot`) (`KismetMathLibrary.RLerp` (struct :`Yaw` 180.0) (struct :`Yaw` 90.0) _rotation6) false false)
          (`KismetSystemLibrary.Delay` 0.5)
          (bind _returnvalue (`|SpawnActorFromClass` "/Game/ScanFX/Blueprints/BP_ScanFX_SwipingBeam.BP_ScanFX_SwipingBeam_C" (`KismetMathLibrary.MakeTransform` (`self.SpawnBeam3`) (struct :`Yaw` 270.0)) "Undefined" "OverrideRootScale" null null))
          (`KismetSystemLibrary.Delay` 3.0)
          (`self.K2_DestroyActor` _returnvalue))))))

(fn `UserConstructionScript`)