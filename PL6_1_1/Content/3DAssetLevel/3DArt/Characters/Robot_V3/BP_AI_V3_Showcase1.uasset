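; Showcase Blueprint for the V3 robot AI that roughly simulates its state changes to display animations on a stationary mesh.
; Each state event drives the cached ABP_RobotAI_V3: most reset it, and Spotted raises HasSeenPlayer for a timed delay.
; Patrol, Chase and Attack play montages, then restore AnimationBlueprint mode, since ground speed alone does not animate the stationary robot.
; SoundHeard, Hunt and Scan only reset; their further logic is disconnected.
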(event `self.ReceiveBeginPlay`
  (bind _asabp_robot_ai_v3 (cast `/Game/3DAssetLevel/3DArt/Characters/Robot_V3/Animations/ABP_RobotAI_V3` (`SkeletalMeshComponent.GetAnimInstance` (`self.AI_SkeletalMesh`))))
  (set `self.ABP REF` _asabp_robot_ai_v3))

(event `Patrol`
  (bind _abp_ref (`self.ABP REF`))
  ;[1 0.1779 0] Simulazione grossolana del cambio di stato dell'IA
  (`/Game/3DAssetLevel/3DArt/Characters/Robot_V3/Animations/ABP_RobotAI_V3.ResetAll` _abp_ref)
  (set `/Game/3DAssetLevel/3DArt/Characters/Robot_V3/Animations/ABP_RobotAI_V3.GroundSpeed` 100.0 _abp_ref)
  ;[1 0 0] Dovrebbe fare la Walk in automatico, ma dato che è ferma sul posto la sua velocità e 0 e anche cambiandole la GroundSpeed non cammina perchè è ferma
  (`|PlayMontage` (`self.AI_SkeletalMesh`) "/Game/3DAssetLevel/LevelDesign/Animations/NPC_IA/Robot_New/Montages/MONT_AI_Walk.MONT_AI_Walk" ; Necessario il Montage per non "scaricare" l'ABP
    (:`OnCompleted`
      (`SkeletalMeshComponent.SetAnimationMode` (`self.AI_SkeletalMesh`) "AnimationBlueprint") ; Serve se no rimane bloccato nell'animazione
    )))

(event `SoundHeard`
  ;[1 0.1779 0] Simulazione grossolana del cambio di stato dell'IA
  (`/Game/3DAssetLevel/3DArt/Characters/Robot_V3/Animations/ABP_RobotAI_V3.ResetAll` (`self.ABP REF`)))

(event `Hunt`
  ;[1 0.1779 0] Simulazione grossolana del cambio di stato dell'IA
  (`/Game/3DAssetLevel/3DArt/Characters/Robot_V3/Animations/ABP_RobotAI_V3.ResetAll` (`self.ABP REF`)))

(event `Scan`
  ;[1 0.1779 0] Simulazione grossolana del cambio di stato dell'IA
  (`/Game/3DAssetLevel/3DArt/Characters/Robot_V3/Animations/ABP_RobotAI_V3.ResetAll` (`self.ABP REF`)))

(event `Spotted`
  (bind _abp_ref (`self.ABP REF`))
  ;[1 0.1779 0] Simulazione grossolana del cambio di stato dell'IA
  (`/Game/3DAssetLevel/3DArt/Characters/Robot_V3/Animations/ABP_RobotAI_V3.ResetAll` _abp_ref)
  (set `/Game/3DAssetLevel/3DArt/Characters/Robot_V3/Animations/ABP_RobotAI_V3.HasSeenPlayer` true _abp_ref)
  ;;[1 0 0] Questo passaggio non mi piace, vorrei che l'ABP prima di tornare in Idle o in Locomotion aspettasse da sola di terminare le animazioni che sta eseguendo, non so come si possa fare, oppure non so magari evitare i delay
  (`KismetSystemLibrary.Delay` 4.0)
  (set `/Game/3DAssetLevel/3DArt/Characters/Robot_V3/Animations/ABP_RobotAI_V3.HasSeenPlayer` false _abp_ref))

(event `Chase`
  (bind _abp_ref (`self.ABP REF`))
  ;[1 0.1779 0] Simulazione grossolana del cambio di stato dell'IA
  (`/Game/3DAssetLevel/3DArt/Characters/Robot_V3/Animations/ABP_RobotAI_V3.ResetAll` _abp_ref)
  (set `/Game/3DAssetLevel/3DArt/Characters/Robot_V3/Animations/ABP_RobotAI_V3.GroundSpeed` 400.0 _abp_ref)
  ;[1 0 0] Dovrebbe fare la Run in automatico, ma dato che è ferma sul posto la sua velocità e 0 e anche cambiandole la GroundSpeed non cammina perchè è ferma (credo)
  (`|PlayMontage` (`self.AI_SkeletalMesh`) "/Game/3DAssetLevel/LevelDesign/Animations/NPC_IA/Robot_New/Montages/MONT_AI_Run.MONT_AI_Run" ; Necessario il Montage per non "scaricare" l'ABP
    (:`OnCompleted`
      (`SkeletalMeshComponent.SetAnimationMode` (`self.AI_SkeletalMesh`) "AnimationBlueprint") ; Serve se no rimane bloccato nell'animazione
    )))

(event `Attack`
  ;[1 1 1] Questa si attiva ogni volta perchè è così che la farei dalla BP dell' IA, dato che serve solo quando muore il Player, è come una cinematic
  (`|PlayMontage` (`self.AI_SkeletalMesh`) "/Game/3DAssetLevel/LevelDesign/Animations/NPC_IA/Robot_New/Montages/MONT_AI_Attack.MONT_AI_Attack" ; Necessario il Montage per non "scaricare" l'ABP
    (:`OnCompleted`
      (`SkeletalMeshComponent.SetAnimationMode` (`self.AI_SkeletalMesh`) "AnimationBlueprint") ; Serve se no rimane bloccato nell'animazione
    )))

(fn `UserConstructionScript`)