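; Decal actor that shows one tile from a configurable texture atlas, set per instance.
; The construction script creates a dynamic instance of MI_Decals on the decal, then applies the tile settings, and BeginPlay reapplies them.
; ChangeTexture sets any valid tile, opacity and normal textures plus the row and column counts.
; ChangeTile sets the tile offsets, and both store absolute values back into the variables.
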(event `self.ReceiveBeginPlay`
  (`self.Change Texture` (`self.Tile`) (`self.Opacity`) (`self.Normal`) (`self.N_Row`) (`self.N_Col`))
  (`self.Change Tile` (`self.OffsetX`) (`self.OffsetY`)))

(fn `Change Texture`
  (params (NewTile :type "Texture Object Reference") (NewOpacity :type "Texture Object Reference") (NewNormal :type "Texture Object Reference") (NRow :type Integer) (NCol :type Integer))
  (bind _newtile (`local.NewTile`))
  (bind _newopacity (`local.NewOpacity`))
  (bind _newnormal (`local.NewNormal`))
  (bind _returnvalue (`KismetMathLibrary.Abs_Int` (`self.N_Col`)))
  (bind _returnvalue_2 (`KismetMathLibrary.Abs_Int` (`self.N_Row`)))
  (`|ExecutionSequence`
    (:`then_0`
      (`/Engine/EditorBlueprintResources/StandardMacros.IsValid` _newtile
        (:`Is Valid`
          (`MaterialInstanceDynamic.SetTextureParameterValue` (`self.MID_Decal`) "Tile" _newtile)
          (set `self.Tile` _newtile))))
    (:`then_1`
      (`/Engine/EditorBlueprintResources/StandardMacros.IsValid` _newopacity
        (:`Is Valid`
          (`MaterialInstanceDynamic.SetTextureParameterValue` (`self.MID_Decal`) "Opacity" _newopacity)
          (set `self.Opacity` _newopacity))))
    (:`then_2`
      (`/Engine/EditorBlueprintResources/StandardMacros.IsValid` _newnormal
        (:`Is Valid`
          (`MaterialInstanceDynamic.SetTextureParameterValue` (`self.MID_Decal`) "Normal" _newnormal)
          (set `self.Normal` _newnormal))))
    (:`then_3`
      (`MaterialInstanceDynamic.SetScalarParameterValue` (`self.MID_Decal`) "TilesX" (`KismetMathLibrary.Conv_IntToDouble` _returnvalue))
      (`MaterialInstanceDynamic.SetScalarParameterValue` (`self.MID_Decal`) "TilesY" (`KismetMathLibrary.Conv_IntToDouble` _returnvalue_2))
      (set `self.N_Col` _returnvalue)
      (set `self.N_Row` _returnvalue_2))))

(fn `Change Tile`
  (params (Offsetx :type Integer) (Offsety :type Integer))
  (bind _returnvalue (`KismetMathLibrary.Abs_Int` Offsetx))
  (bind _returnvalue_2 (`KismetMathLibrary.Abs_Int` Offsety))
  (`MaterialInstanceDynamic.SetScalarParameterValue` (`self.MID_Decal`) "OffsetX" (`KismetMathLibrary.Conv_IntToDouble` _returnvalue))
  (`MaterialInstanceDynamic.SetScalarParameterValue` (`self.MID_Decal`) "OffsetY" (`KismetMathLibrary.Conv_IntToDouble` _returnvalue_2))
  (set `self.OffsetX` _returnvalue)
  (set `self.OffsetY` _returnvalue_2))

(fn `UserConstructionScript`
  (bind _returnvalue (`KismetMaterialLibrary.CreateDynamicMaterialInstance` "/Game/3DAssetLevel/3DArt/Materials/MI_Decals.MI_Decals"))
  (bind _output_get (set `self.MID_Decal` _returnvalue))
  (`DecalComponent.SetDecalMaterial` (`self.Decal`) _output_get)
  (`self.Change Texture` (`self.Tile`) (`self.Opacity`) (`self.Normal`) (`self.N_Row`) (`self.N_Col`))
  (`self.Change Tile` (`self.OffsetX`) (`self.OffsetY`)))