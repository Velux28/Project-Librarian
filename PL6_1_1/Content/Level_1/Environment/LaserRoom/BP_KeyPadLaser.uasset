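; Laser room keypad actor that opens a keypad UI or moves the exit door when the player character overlaps its box.
; If IsCorrect is already set, it relocates the mesh of BP_DoorLaserRoomToMH; otherwise it creates W_Keypad, shows the cursor and focuses input on it.
; Leaving the box removes all widgets without restoring cursor or input mode.
; LookAt returns an empty string.
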(event `self.Box.OnComponentBeginOverlap`
  (params (OverlappedComponent :type "PrimitiveComponent Object Reference") (OtherActor :type "Actor Object Reference") (OtherComp :type "PrimitiveComponent Object Reference") (OtherBodyIndex :type Integer) (bFromSweep :type Boolean) (SweepResult :type "HitResult Structure (by ref)"))
  (bind _returnvalue (`GameplayStatics.GetPlayerController` 0))
  (cast `/Game/BP_BO/PlayerCharacter/BP_TPCharacter` OtherActor)
  (if (`self.IsCorrect`)
    (bind _returnvalue_2 (`GameplayStatics.GetActorOfClass` "/Game/Level_1/Environment/LaserRoom/BP_DoorLaserRoomToMH.BP_DoorLaserRoomToMH_C"))
    (`SceneComponent.K2_SetRelativeLocation` (`StaticMeshActor.StaticMeshComponent` _returnvalue_2) (`self.New Location`) false false)
    (else
      (bind _returnvalue_3 (`|CreateWidget` "/Game/UI/PlayerUI/Environment_UI/Interactions/W_Keypad.W_Keypad_C"))
      (`UserWidget.AddToViewport` _returnvalue_3 0)
      (`WidgetBlueprintLibrary.SetInputMode_UIOnlyEx` null null)
      (set `PlayerController.bShowMouseCursor` true _returnvalue)
      (`WidgetBlueprintLibrary.SetInputMode_GameAndUIEx` _returnvalue _returnvalue_3))))

(event `self.Box.OnComponentEndOverlap`
  (params (OverlappedComponent :type "PrimitiveComponent Object Reference") (OtherActor :type "Actor Object Reference") (OtherComp :type "PrimitiveComponent Object Reference") (OtherBodyIndex :type Integer))
  (cast `/Game/BP_BO/PlayerCharacter/BP_TPCharacter` OtherActor)
  (`WidgetLayoutLibrary.RemoveAllWidgets`))

(fn `LookAt`
  (returns (Message :type Text))
  (return ""))

(fn `UserConstructionScript`)