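; BP_Scientist is an NPC scientist in the Level 1 laser room that plays a scripted three-part dialogue when interacted with.
; Interactwith creates three dialogue widgets hidden, then shows each in turn for a fixed delay.
; A DoOnce blocks retriggering until the sequence and a short cooldown finish; LookAt returns an empty string.
; An older index-based dialogue path using a TalkText widget remains unconnected.
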(event `/Game/BP_BO/Inventory/BPI_InteractInterface.InteractWith`
  (params (PlayerCharacter :type "/Game/BP_BO/PlayerCharacter/BP_TPCharacter Object Reference"))
  ;[0.4507 0 1] DIALOGO NPC
  (`/Engine/EditorBlueprintResources/StandardMacros.DoOnce` false :!label _label
    (:`Completed`
      (`self.ScienziatUno`)
      (`self.ScienziatoDue`)
      (`self.ScienziatoTre`)
      (`Widget.SetVisibility` (`self.Scienziato1`) "Visible")
      (`KismetSystemLibrary.Delay` 2.0)
      (`Widget.SetVisibility` (`self.Scienziato1`) "Collapsed")
      (`Widget.SetVisibility` (`self.Scienziato2`) "Visible")
      (`KismetSystemLibrary.Delay` 10.0)
      (`Widget.SetVisibility` (`self.Scienziato2`) "Collapsed")
      (`Widget.SetVisibility` (`self.Scienziato3`) "Visible")
      (`KismetSystemLibrary.Delay` 6.0)
      (`Widget.SetVisibility` (`self.Scienziato3`) "Collapsed")
      (`KismetSystemLibrary.Delay` 4.0)
      (goto _label :!via `Reset`))))

(fn `LookAt`
  (returns (Message :type Text))
  (return ""))

(fn `ScienziatoDue`
  (bind _returnvalue (`|CreateWidget` "/Game/Level_1/Environment/LaserRoom/W_Dial2.W_Dial2_C"))
  (bind _output_get (set `self.Scienziato2` _returnvalue))
  (`UserWidget.AddToViewport` _output_get 0)
  (`Widget.SetVisibility` (`self.Scienziato2`) "Collapsed"))

(fn `ScienziatoTre`
  (bind _returnvalue (`|CreateWidget` "/Game/Level_1/Environment/LaserRoom/W_DIal3.W_DIal3_C"))
  (bind _output_get (set `self.Scienziato3` _returnvalue))
  (`UserWidget.AddToViewport` _output_get 0)
  (`Widget.SetVisibility` (`self.Scienziato3`) "Collapsed"))

(fn `ScienziatUno`
  (bind _returnvalue (`|CreateWidget` "/Game/Level_1/Environment/LaserRoom/W_Dial1.W_Dial1_C"))
  (bind _output_get (set `self.Scienziato1` _returnvalue))
  (`UserWidget.AddToViewport` _output_get 0)
  (`Widget.SetVisibility` (`self.Scienziato1`) "Collapsed"))

(fn `UserConstructionScript`)