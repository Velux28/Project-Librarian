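; BP_TestRoomCan is a can prop in the test room that makes noise when hit.
; Its Hit event runs once, plays the can sound at the actor and reports an AI noise event attributed to the player, then destroys the actor after a short delay.
; The noise location is hardcoded rather than taken from the can.
; The can reports itself as non-interactable, and FondoCestino only prints a debug message.
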(event `self.ReceiveHit`
  (params (MyComp :type "PrimitiveComponent Object Reference") (Other :type "Actor Object Reference") (OtherComp :type "PrimitiveComponent Object Reference") (bSelfMoved :type Boolean) (HitLocation :type "Vector Structure") (HitNormal :type "Vector Structure") (NormalImpulse :type "Vector Structure") (Hit :type "HitResult Structure (by ref)"))
  (`/Engine/EditorBlueprintResources/StandardMacros.DoOnce` false
    (:`Completed`
      (`GameplayStatics.PlaySoundAtLocation` "/Game/BO_Custom/SOUNDS/GENERIC/SC_Can.SC_Can" (`self.K2_GetActorLocation`) (struct) 1.0 1.0 0.0 null null null null)
      (`AISense_Hearing.ReportNoiseEvent` (1531.0 2183.0 -152.0) 3.0 (`GameplayStatics.GetPlayerController` 0))
      (`KismetSystemLibrary.Delay` 1.0)
      (`self.K2_DestroyActor`))))

(fn `Check IF Interactable`
  (returns (`Is NOT Interactable` :type Boolean))
  (return false))

(fn `FondoCestino`
  (params (Object :type "Object Object Reference"))
  (`KismetSystemLibrary.PrintString` "TESTROOMCAN CALLS FOR FONDOCESTINO " true true (struct :`R` 1.0 :`B` 0.076571 :`A` 1.0) 10.0))

(fn `UserConstructionScript`)