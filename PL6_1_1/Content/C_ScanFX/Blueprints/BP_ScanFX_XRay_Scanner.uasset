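; X-ray scanner effect actor that shows a triangle phantom for each actor overlapping it.
; Actors overlapping at BeginPlay or entering later each get a phantom spawned at their transform, fed the scan dynamic material, unless ignored, already observed or owned by the scanner.
; Observed actors and phantoms sit in index-paired arrays, so ending an overlap destroys and removes the matching phantom.
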(event `self.ReceiveActorBeginOverlap`
  (params (OtherActor :type "Actor Object Reference"))
  ;[0.1 0.1 0.1] Add new actors to the effect when they overlap and remove them when they stop overlapping
  (`self.Add Observed Actor` OtherActor))

(event `self.ReceiveBeginPlay`
  ;[0.1 0.1 0.1] Add all actors that are overlapping at the beginning to the observed actors list
  (`parent.ReceiveBeginPlay`)
  (for _array_element (`self.GetOverlappingActors` "/Script/Engine.Actor")
    (`self.Add Observed Actor` _array_element)))

(event `self.ReceiveActorEndOverlap`
  (params (OtherActor :type "Actor Object Reference"))
  ;[0.1 0.1 0.1] Add new actors to the effect when they overlap and remove them when they stop overlapping
  (`self.Remove Observed Actor` OtherActor))

(event `Add Observed Actor`
  (params (Actor :type "Actor Object Reference"))
  ;[0.1 0.1 0.1] Add an actor to scan
  ;;[0.1 0.1 0.1] Prevent addition of ignored actors
  (if (not (`KismetArrayLibrary.Array_Contains` (`self.Ignored Actors`) Actor))
    ;;[0.1 0.1 0.1] Make sure the actor is not already registered
    (if (and (not (`KismetArrayLibrary.Array_Contains` (`self.Observed Actors`) Actor)) (!= (`self.GetOwner` Actor) self))
      ;;[0.1 0.1 0.1] Spawn new phantom actor
      (bind _returnvalue (`|SpawnActorFromClass` "/Game/C_ScanFX/Blueprints/BP_ScanFX_TrianglePhantomActor.BP_ScanFX_TrianglePhantomActor_C" (`self.GetTransform` Actor) "AlwaysSpawn" "OverrideRootScale" self (`self.Scan MID`) Actor null))
      ;;[0.1 0.1 0.1] Add actors to observation list
      (`/Engine/EditorBlueprintResources/StandardMacros.IsValid` _returnvalue
        (:`Is Valid`
          (`KismetArrayLibrary.Array_Add` (`self.Scan Phantom Actors`) _returnvalue)
          (`KismetArrayLibrary.Array_Add` (`self.Observed Actors`) Actor))))))

(event `Remove Observed Actor`
  (params (Actor :type "Actor Object Reference"))
  (bind _returnvalue (`KismetArrayLibrary.Array_Find` (`self.Observed Actors`) Actor))
  ;[0.1 0.1 0.1] Remove an actor from being scanned
  ;;[0.1 0.1 0.1] Only remove if actor is being scanned
  (if (`KismetArrayLibrary.Array_Contains` (`self.Observed Actors`) Actor)
    ;;[0.1 0.1 0.1] Find and destroy the phantom
    (`self.K2_DestroyActor` (`|GetArrayItem` (`self.Scan Phantom Actors`) _returnvalue))
    ;;[0.1 0.1 0.1] Remove actors from scanning list
    (`KismetArrayLibrary.Array_Remove` (`self.Scan Phantom Actors`) _returnvalue)
    (`KismetArrayLibrary.Array_Remove` (`self.Observed Actors`) _returnvalue)))

(fn `UserConstructionScript`
  (`parent.UserConstructionScript`))