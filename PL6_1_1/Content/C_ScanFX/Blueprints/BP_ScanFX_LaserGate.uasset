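; BP_ScanFX_LaserGate is a laser gate effect that builds a row of evenly spaced laser beams stacked along Z.
; At BeginPlay it adds the configured number of ScanFX laser components, spreading them up to UpperCorner's height.
; Each laser receives the shared material and uses UpperCorner's X as its trace distance.
; The construction script optionally adds a rotating movement component to spin the gate at a configurable rate.
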(event `self.ReceiveBeginPlay`
  (bind (_upper_corner_x _upper_corner_y _upper_corner_z) (`KismetMathLibrary.BreakVector` (`self.Upper Corner`)))
  (bind _upper_corner_x_2 (`KismetMathLibrary.BreakVector` (`self.Upper Corner`)))
  (bind _returnvalue (- (`self.Lasers Count`) 1))
  ;[0.1 0.1 0.1] Create specified amount of laser components and interpolate their positin along Z
  (for _index (range (+ _returnvalue 1))
    (`AddComponent|NODE_AddBP_ScanFX_LaserComponent-0` :`RelativeTransform` (`KismetMathLibrary.MakeTransform` (`KismetMathLibrary.MakeVector` 0.0 0.0 (* _index (/ _upper_corner_z (`KismetMathLibrary.Conv_IntToDouble` _returnvalue))))) :`Trace Distance` _upper_corner_x_2 :`Laser Material` (`self.Laser Material`))))

(fn `UserConstructionScript`
  (if (`self.Lasers Rotate`)
    (bind _returnvalue (`AddComponent|NODE_AddRotatingMovementComponent-0`))
    (set `RotatingMovementComponent.RotationRate` (`KismetMathLibrary.MakeRotator` 0.0 0.0 (`self.Laser Rotation Rate`)) _returnvalue)))