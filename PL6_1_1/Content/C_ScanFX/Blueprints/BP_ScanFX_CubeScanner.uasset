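; Cube scanner variant of a scan FX Blueprint that sweeps a cube vertically through a box volume.
; The construction script sizes the cube to the box footprint at a set height, centers it and applies the scan dynamic material.
; It derives the material's grid scale from laser grid size divided by box extent, compensating for box size.
; UpdateScanPosition extends the parent event, lerping the cube's Z between bottom and top corners by position alpha.
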(event `self.Update Scan Position`
  (params (`Position Alpha` :type "Float (double-precision)"))
  (bind (_bottom_corner_x _bottom_corner_y _bottom_corner_z) (`KismetMathLibrary.BreakVector` (`self.Bottom Corner`)))
  (bind (_top_corner_x _top_corner_y _top_corner_z) (`KismetMathLibrary.BreakVector` (`self.Top Corner`)))
  ;[0.1 0.1 0.1] Move cube up and down
  (`parent.Update Scan Position` `Position Alpha`)
  (`SceneComponent.K2_SetRelativeLocation` (`self.Cube`) (`KismetMathLibrary.MakeVector` (.x (`SceneComponent.RelativeLocation` (`self.Box`))) (.y (`SceneComponent.RelativeLocation` (`self.Box`))) (`KismetMathLibrary.Lerp` _bottom_corner_z _top_corner_z `Position Alpha`)) false false))

(fn `UserConstructionScript`
  (bind _returnvalue (`BoxComponent.GetScaledBoxExtent` (`self.Box`)))
  (bind (_returnvalue_x _returnvalue_y) (`KismetMathLibrary.BreakVector` (* _returnvalue 2.0)))
  (`parent.UserConstructionScript`)
  ;[0.1 0.1 0.1] Tell material how big the scanning box is
  (`MaterialInstanceDynamic.SetVectorParameterValue` (`self.Scan MID`) "Scan Grid Scale" (`KismetMathLibrary.Conv_VectorToLinearColor` (/ (`self.Laser Grid Size`) (* _returnvalue 0.01))))
  ;[0.1 0.1 0.1] Scale cube mesh accordingly
  (`SceneComponent.SetRelativeScale3D` (`self.Cube`) (* (`KismetMathLibrary.MakeVector` _returnvalue_x _returnvalue_y (`self.Cube Height`)) 0.01))
  ;[0.1 0.1 0.1] Position cube mesh to center of box
  (`SceneComponent.K2_SetRelativeLocation` (`self.Cube`) (`SceneComponent.RelativeLocation` (`self.Box`)) false false)
  ;[0.1 0.1 0.1] Apply scan material
  (`PrimitiveComponent.SetMaterial` (`self.Cube`) 0 (`self.Scan MID`)))