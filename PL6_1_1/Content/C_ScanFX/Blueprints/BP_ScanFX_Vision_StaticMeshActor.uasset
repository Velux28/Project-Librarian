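; Static mesh actor that swaps its materials to match the scan vision mode.
; On BeginPlay it caches the mesh's original materials as the default set.
; SetVisionMode applies the thermal or electro material array for those modes and restores the defaults for Night and any other mode, using a helper that sets each slot by index.
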(event `self.ReceiveBeginPlay`
  ;[0.1 0.1 0.1] Save original materials into array for later use
  (for _index (range (`PrimitiveComponent.GetNumMaterials` (`self.StaticMeshComponent`)))
    (`KismetArrayLibrary.Array_Add` (`self.Default Materials`) (`PrimitiveComponent.GetMaterial` (`self.StaticMeshComponent`) _index))))

(event `/Game/C_ScanFX/Blueprints/BP_ScanFX_VisionInterface.Set Vision Mode`
  (params (`New Mode` :type "/Game/C_ScanFX/Data/EScanFXVisionMode Enum" :default "NewEnumerator0"))
  ;[0.1 0.1 0.1] Set material based on vision mode
  (switch `/Game/C_ScanFX/Data/EScanFXVisionMode` `New Mode`
    (:`NewEnumerator0`
      (`self.Apply Materials` (`self.Default Materials`) :!label _label))
    (:`NewEnumerator1`
      (goto _label))
    (:`NewEnumerator2`
      (`self.Apply Materials` (`self.Thermal Materials`)))
    (:`NewEnumerator3`
      (`self.Apply Materials` (`self.Electro Materials`)))))

(event `Apply Materials`
  (params (Materials :type "Array of MaterialInterface Object Reference"))
  ;[0.1 0.1 0.1] Helper method to apply material array
  (for (_array_element _array_index) Materials
    (`PrimitiveComponent.SetMaterial` (`self.StaticMeshComponent`) _array_index _array_element)))

(fn `UserConstructionScript`)