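; Single door Blueprint that switches AI on or off when the player enters its AIBox trigger.
; On overlap by the player character, and only while IsWorking is set, it calls the ACAIActivator component if valid.
; The ActivateAI flag selects between activating AIRef with the BTRef behavior tree and deactivating AIRef.
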(event `self.AIBox.OnComponentBeginOverlap`
  (params (OverlappedComponent :type "PrimitiveComponent Object Reference") (OtherActor :type "Actor Object Reference") (OtherComp :type "PrimitiveComponent Object Reference") (OtherBodyIndex :type Integer) (bFromSweep :type Boolean) (SweepResult :type "HitResult Structure (by ref)"))
  (if (and (`self.IsWorking`) (== OtherActor (`GameplayStatics.GetPlayerCharacter` 0)))
    (bind _ac_aiactivator (`self.AC_AIActivator`)
      (:`then`
        (if (`self.ActivateAI`)
          (`/Game/BP_BO/ArtificialIntelligence/AC_AIActivator.Activate AI` _ac_aiactivator (`self.AIRef`) (`self.BTRef`))
          (else
            (`/Game/BP_BO/ArtificialIntelligence/AC_AIActivator.De-activate AI` _ac_aiactivator (`self.AIRef`)))))
      (:`else`))))

(fn `UserConstructionScript`)