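; Sliding double door Blueprint that opens when the player enters its trigger box and closes on exit, if trigger operation is enabled.
; Two timelines play or reverse to move the door meshes, with a sound for each direction.
; Other actors can call OpenTargetDoor, which opens it, closes it after a delay, enables trigger operation and messages the calling button.
; Debug print functions describing these states are defined but not called here.
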(event `self.Box.OnComponentBeginOverlap`
  (params (OverlappedComponent :type "PrimitiveComponent Object Reference") (OtherActor :type "Actor Object Reference") (OtherComp :type "PrimitiveComponent Object Reference") (OtherBodyIndex :type Integer) (bFromSweep :type Boolean) (SweepResult :type "HitResult Structure (by ref)"))
  ;[1 1 1] When the Player enters the Trigger Box
  (if (== OtherActor (`GameplayStatics.GetPlayerCharacter` 0))
    (if (`self.DoorShouldOperateByTriggerBox`)
      (`self.DoorOpenSequence`))))

(event `DoorOpenSequence`
  ;[1 1 1] Open or Close the Door.
  (`GameplayStatics.PlaySoundAtLocation` "/Game/SoundDesign/Environment_SFX/SoundCues/SC_SlidingDoor_A.SC_SlidingDoor_A" (`SceneComponent.K2_GetComponentLocation` (`self.DoorFrame`)) (struct) 1.0 1.0 0.0 null null null null)
  (`|ExecutionSequence`
    (:`then_0`
      (bind (_direction _door1track) (`Timeline|DoorMesh1_Timeline` :!label _label)
        (:`Update`
          (`SceneComponent.K2_SetRelativeLocation` (`self.DoorMesh_1`) _door1track false false))))
    (:`then_1`
      (bind (_direction_2 _door2track) (`Timeline|DoorMesh2_Timeline` :!label _label_2)
        (:`Update`
          (`SceneComponent.K2_SetRelativeLocation` (`self.DoorMesh_2`) _door2track false false))))))

(event `self.Box.OnComponentEndOverlap`
  (params (OverlappedComponent :type "PrimitiveComponent Object Reference") (OtherActor :type "Actor Object Reference") (OtherComp :type "PrimitiveComponent Object Reference") (OtherBodyIndex :type Integer))
  ;[1 1 1] When the Player leaves the Trigger Box
  (if (== OtherActor (`GameplayStatics.GetPlayerCharacter` 0))
    (if (`self.DoorShouldOperateByTriggerBox`)
      (`self.DoorCloseSequence`))))

(event `DoorCloseSequence`
  ;[1 1 1] Open or Close the Door.
  (`GameplayStatics.PlaySoundAtLocation` "/Game/SoundDesign/Environment_SFX/SoundCues/SC_SlidingDoor_B.SC_SlidingDoor_B" (`SceneComponent.K2_GetComponentLocation` (`self.DoorFrame`)) (struct) 1.0 1.0 0.0 null null null null)
  (`|ExecutionSequence`
    (:`then_0`
      (goto _label :!via `Reverse`))
    (:`then_1`
      (goto _label_2 :!via `Reverse`))))

(event `/Game/BP_BO/Puzzles/BPI_Unlockable.OpenTargetDoor`
  (params (Caller :type "Actor Object Reference"))
  ;[1 1 1] When Called by another Actor
  (set `self.Caller` Caller)
  (`self.DoorOpenSequence`)
  (`KismetSystemLibrary.Delay` 5.0)
  (`self.DoorCloseSequence`)
  (set `self.DoorShouldOperateByTriggerBox` true)
  (message `/Game/BP_BO/Puzzles/BPI_Unlockable.SetButtonUsable_Blue` (`self.Caller`) self))

(fn `TestingString_Close`
  (params (Caller :type "Actor Object Reference") (DoorShouldOperateByTriggerBox :type Boolean))
  (if (== Caller self)
    (if DoorShouldOperateByTriggerBox
      (`KismetSystemLibrary.PrintString` (`KismetStringLibrary.Concat_StrStr` "I am  " (`KismetSystemLibrary.GetDisplayName` self) ". I have been called to CLOSE by my own TriggerBox") true true (struct :`G` 0.66 :`B` 1.0 :`A` 1.0) 10.0)
      (return)
      (else
        (`KismetSystemLibrary.PrintString` (`KismetStringLibrary.Concat_StrStr` "I am  " (`KismetSystemLibrary.GetDisplayName` self) ". I have been called to CLOSE by my own TriggerBox, " "but i cannot, for i am not set to Operate by TriggerBox") true true (struct :`R` 1.0 :`G` 0.5 :`A` 1.0) 10.0)
        (return)))))

(fn `TestingString_Opening`
  (params (Caller :type "Actor Object Reference") (DoorShouldOperateByTriggerBox :type Boolean))
  (if (== Caller self)
    (if DoorShouldOperateByTriggerBox
      (`KismetSystemLibrary.PrintString` (`KismetStringLibrary.Concat_StrStr` "I am  " (`KismetSystemLibrary.GetDisplayName` self) ". I have been called to OPEN by my own TriggerBox") true true (struct :`G` 0.66 :`B` 1.0 :`A` 1.0) 10.0)
      (return)
      (else
        (`KismetSystemLibrary.PrintString` (`KismetStringLibrary.Concat_StrStr` "I am  " (`KismetSystemLibrary.GetDisplayName` self) ". I have been called to OPEN by my own TriggerBox, " "but i cannot, for i am not set to Operate by TriggerBox") true true (struct :`R` 1.0 :`G` 0.5 :`A` 1.0) 10.0)
        (return)))
    (else
      (`KismetSystemLibrary.PrintString` (`KismetStringLibrary.Concat_StrStr` "I am  " (`KismetSystemLibrary.GetDisplayName` self) ". I have been called to OPEN by " (`KismetSystemLibrary.GetDisplayName` Caller) ". I will close automatically in 5 seconds.") true true (struct :`G` 0.66 :`B` 1.0 :`A` 1.0) 10.0)
      (return))))

(fn `TestingString_OpeninOverride`
  (params (Caller :type "Actor Object Reference") (DoorShouldOperateByTriggerBox :type Boolean))
  (if DoorShouldOperateByTriggerBox
    (`KismetSystemLibrary.PrintString` (`KismetStringLibrary.Concat_StrStr` "I am  " (`KismetSystemLibrary.GetDisplayName` self) ", and i already Operate by TriggerBox") true true (struct :`G` 1.0 :`A` 1.0) 10.0)
    (return)
    (else
      (`KismetSystemLibrary.PrintString` (`KismetStringLibrary.Concat_StrStr` "I am  " (`KismetSystemLibrary.GetDisplayName` self) ". I have been now set to Operate by TriggerBox by " (`KismetSystemLibrary.GetDisplayName` Caller)) true true (struct :`G` 1.0 :`A` 1.0) 10.0)
      (return))))

(fn `UserConstructionScript`)