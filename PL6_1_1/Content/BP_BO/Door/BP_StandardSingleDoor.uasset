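; Single door Blueprint that opens automatically when the player enters its box, or on a button request, while it is working.
; BeginPlay assigns the door mesh and disables the box collision for non-automatic doors.
; Tick uses opening and closing flags to call OpenDoor and CloseDoor, defined outside this file, with a three-second delay before closing.
; Lock and Unlock toggle the working state; an older timeline-based opening remains disconnected.
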(event `self.ReceiveBeginPlay`
  (set `self.door` (`self.SM_porta1`))
  (if (not (`self.IsAutomaticDoor`))
    (`PrimitiveComponent.SetCollisionEnabled` (`self.Box`) "NoCollision")))

(event `self.ReceiveTick`
  (params (DeltaSeconds :type "Float (single-precision)"))
  (if (`self.IsWorking`)
    (if (`self.bIsDoorOpening`)
      (if (`self.bIsDoorClosing`)
        (`KismetSystemLibrary.Delay` 3.0)
        (set `self.bIsDoorOpening` false)
        (else
          (`self.OpenDoor`)))
      (elif (`self.bIsDoorClosing`)
        (`self.CloseDoor`)))))

(event `ButtonClicked`
  ;[0.9714 1 0] da rimuovere
  (if (not (or (`self.bIsDoorOpening`) (`self.bIsDoorClosing`)))
    (set `self.bIsDoorOpening` true)))

(event `self.Box.OnComponentBeginOverlap`
  (params (OverlappedComponent :type "PrimitiveComponent Object Reference") (OtherActor :type "Actor Object Reference") (OtherComp :type "PrimitiveComponent Object Reference") (OtherBodyIndex :type Integer) (bFromSweep :type Boolean) (SweepResult :type "HitResult Structure (by ref)"))
  (if (and (`self.IsAutomaticDoor`) (`self.IsWorking`) (== OtherActor (`GameplayStatics.GetPlayerCharacter` 0)))
    (set `self.bIsDoorOpening` true)
    (set `self.bIsDoorClosing` false)))

(event `/Game/BP_BO/Puzzles/BPI_Unlockable.Unlock`
  (set `self.IsWorking` true))

(event `/Game/BP_BO/Puzzles/BPI_Unlockable.Lock`
  (set `self.IsWorking` false))

(fn `Try Open Door With Button`
  (returns (result :type Boolean))
  (if (not (or (`self.bIsDoorOpening`) (`self.bIsDoorClosing`)))
    (set `self.bIsDoorOpening` true))
  (return (`self.bIsDoorOpening`)))

(fn `UserConstructionScript`)