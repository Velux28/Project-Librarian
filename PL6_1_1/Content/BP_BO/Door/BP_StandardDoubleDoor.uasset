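; Sliding double door that opens automatically for the player or through a button, and can be locked or unlocked.
; BeginPlay assigns both door meshes and disables the trigger box unless automatic; player overlap calls TryOpenDoor, which is defined outside this file.
; TryOpenDoorWithButton raises both opening flags when the door is working and idle, and returns the opening state.
; The older timeline, sound and state-driven open/close logic remains in the graph, disconnected.
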(event `self.ReceiveBeginPlay`
  (set `self.door` (`self.DoorMesh_1`))
  (set `self.door2` (`self.DoorMesh_2`))
  (if (not (`self.IsAutomaticDoor`))
    (`PrimitiveComponent.SetCollisionEnabled` (`self.Box`) "NoCollision")))

(event `self.ReceiveTick`
  (params (DeltaSeconds :type "Float (single-precision)")))

(event `self.Box.OnComponentBeginOverlap`
  (params (OverlappedComponent :type "PrimitiveComponent Object Reference") (OtherActor :type "Actor Object Reference") (OtherComp :type "PrimitiveComponent Object Reference") (OtherBodyIndex :type Integer) (bFromSweep :type Boolean) (SweepResult :type "HitResult Structure (by ref)"))
  (if (and (`self.IsAutomaticDoor`) (`self.IsWorking`) (== OtherActor (`GameplayStatics.GetPlayerCharacter` 0)))
    (`self.TryOpenDoor`)))

(event `/Game/BP_BO/Puzzles/BPI_Unlockable.Unlock`
  (set `self.IsWorking` true))

(event `/Game/BP_BO/Puzzles/BPI_Unlockable.Lock`
  (set `self.IsWorking` false))

(fn `Try Open Door With Button`
  (returns (result :type Boolean))
  (if (`self.IsWorking`)
    (if (not (or (`self.bIsDoorOpening`) (`self.bIsDoorClosing`) (`self.bIsDoor2Opening`) (`self.bIsDoor2Closing`)))
      (set `self.bIsDoorOpening` true)
      (set `self.bIsDoor2Opening` true))
    (return (`self.bIsDoorOpening`))
    (else
      (return false))))

(fn `UserConstructionScript`)