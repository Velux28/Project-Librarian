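; Interactable button that opens a linked standard single or double door, with positive or negative sound feedback.
; Interactwith plays the negative sound when not working or busy, otherwise it sets busy through a DoOnce and calls TryOpenDoorWithButton on the cast door.
; After a successful door cast, a short delay calls ButtonReset to clear the busy state and DoOnce.
; Lock and Unlock toggle whether the button works and message the linked door.
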(event `/Game/BP_BO/Inventory/BPI_InteractInterface.InteractWith`
  (params (PlayerCharacter :type "/Game/BP_BO/PlayerCharacter/BP_TPCharacter Object Reference"))
  (bind _returnvalue (`self.K2_GetActorLocation`))
  (if (`self.IsWorking`)
    (if (`self.IsBusy`)
      (`GameplayStatics.PlaySoundAtLocation` "/Game/SoundDesign/Environment_SFX/SoundCues/SC_ButtonNegative.SC_ButtonNegative" _returnvalue (struct) 1.0 1.0 0.0 null null null null :!label _label)
      (else
        (`GameplayStatics.PlaySoundAtLocation` "/Game/SoundDesign/Environment_SFX/SoundCues/SC_Button_Positive.SC_Button_Positive" _returnvalue (struct) 1.0 1.0 0.0 null null null null)
        (`/Engine/EditorBlueprintResources/StandardMacros.DoOnce` false :!label _label_2
          (:`Completed`
            (set `self.IsBusy` true)
            (bind _doortoopen (`self.DoorToOpen`)
              (:`then`
                (bind _asbp_standard_single_door (cast `/Game/BP_BO/Door/BP_StandardSingleDoor` _doortoopen)
                  (:`then`
                    (`/Game/BP_BO/Door/BP_StandardSingleDoor.Try Open Door With Button` _asbp_standard_single_door))
                  (:`CastFailed`
                    (bind _asbp_standard_double_door (cast `/Game/BP_BO/Door/BP_StandardDoubleDoor` _doortoopen))
                    (`/Game/BP_BO/Door/BP_StandardDoubleDoor.Try Open Door With Button` _asbp_standard_double_door)))
                (`KismetSystemLibrary.Delay` 5.0)
                (`self.Button Reset`))
              (:`else`))))))
    (else
      (goto _label))))

(event `/Game/BP_BO/Puzzles/BPI_Unlockable.Unlock`
  (set `self.IsWorking` true)
  (message `/Game/BP_BO/Puzzles/BPI_Unlockable.Unlock` (`self.DoorToOpen`)))

(event `Button Reset`
  (set `self.IsBusy` false)
  (goto _label_2 :!via `Reset`))

(event `/Game/BP_BO/Puzzles/BPI_Unlockable.Lock`
  (set `self.IsWorking` false)
  (message `/Game/BP_BO/Puzzles/BPI_Unlockable.Lock` (`self.DoorToOpen`)))

(fn `LookAt`
  (returns (Message :type Text))
  (return ""))

(fn `UserConstructionScript`)