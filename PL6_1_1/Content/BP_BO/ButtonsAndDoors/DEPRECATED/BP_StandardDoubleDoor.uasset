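; Deprecated double-door Blueprint that hands its two meshes to a parent door class, which handles opening and closing.
; In automatic mode a Box overlap by the player opens and closes it; otherwise the box's collision is disabled.
; IsWorking gates ticking, overlaps and button opening, and is toggled by puzzle success or button-disable events.
; The old timeline-driven sliding and sound logic remains but is disconnected.
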(event `self.ReceiveBeginPlay`
  (`parent.ReceiveBeginPlay`)
  (set `self.door` (`self.DoorMesh_1`))
  (set `self.door2` (`self.DoorMesh_2`))
  (if (not (`self.IsAutomaticDoor`))
    (`PrimitiveComponent.SetCollisionEnabled` (`self.Box`) "NoCollision")))

(event `self.ReceiveTick`
  (params (DeltaSeconds :type "Float (single-precision)"))
  (if (`self.IsWorking`)
    (`parent.ReceiveTick` DeltaSeconds)))

(event `self.Box.OnComponentBeginOverlap`
  (params (OverlappedComponent :type "PrimitiveComponent Object Reference") (OtherActor :type "Actor Object Reference") (OtherComp :type "PrimitiveComponent Object Reference") (OtherBodyIndex :type Integer) (bFromSweep :type Boolean) (SweepResult :type "HitResult Structure (by ref)"))
  (if (and (`self.IsAutomaticDoor`) (`self.IsWorking`) (== OtherActor (`GameplayStatics.GetPlayerCharacter` 0)))
    (set `self.bCanBeClose` false)
    (`self.OpenDoor`)))

(event `/Game/BP_BO/Puzzles/BPI_Unlockable.OpenTargetDoor`
  (params (Caller :type "Actor Object Reference"))
  (set `self.IsWorking` true))

(event `/Game/BP_BO/Puzzles/BPI_Unlockable.SetButtonUnusable_Red`
  (set `self.IsWorking` false))

(event `self.Puzzle Sucsess`
  (`/Game/BP_BO/Puzzles/BPI_Unlockable.OpenTargetDoor` null))

(event `self.Box.OnComponentEndOverlap`
  (params (OverlappedComponent :type "PrimitiveComponent Object Reference") (OtherActor :type "Actor Object Reference") (OtherComp :type "PrimitiveComponent Object Reference") (OtherBodyIndex :type Integer))
  (if (and (`self.IsAutomaticDoor`) (`self.IsWorking`) (== OtherActor (`GameplayStatics.GetPlayerCharacter` 0)))
    (set `self.bCanBeClose` true)
    (`self.CloseDoor`)))

(fn `CloseDoor`
  (returns (ReturnValue :type Boolean))
  ;[1 1 1] Senza questo non si chiude
  (bind _returnvalue (`parent.CloseDoor`))
  (return _returnvalue))

(fn `OpenDoor`
  (returns (ReturnValue :type Boolean))
  ;[1 1 1] Senza questo non si apre
  (bind _returnvalue (`parent.OpenDoor`))
  (return _returnvalue))

(fn `Try Open Door With Button`
  (returns (result :type Boolean))
  (if (`self.IsWorking`)
    (`self.OpenDoor`)
    (return false)
    (else
      (return false))))

(fn `UserConstructionScript`)