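; Single sliding control-room door, a child Blueprint that opens and closes by trigger box or when another actor calls it.
; A timeline plays forward or in reverse to slide the door mesh, with a sound for each direction.
; Player overlaps drive it only while trigger operation is enabled.
; A remote open can auto-close after a delay, then enables trigger operation and messages the caller to set its button usable.
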(event `self.Box.OnComponentBeginOverlap`
  (params (OverlappedComponent :type "PrimitiveComponent Object Reference") (OtherActor :type "Actor Object Reference") (OtherComp :type "PrimitiveComponent Object Reference") (OtherBodyIndex :type Integer) (bFromSweep :type Boolean) (SweepResult :type "HitResult Structure (by ref)"))
  ;[1 1 1] When the Player enters the Trigger Box
  (if (== OtherActor (`GameplayStatics.GetPlayerCharacter` 0))
    (if (`self.Door Should Operate by Trigger Box`)
      (`self.DoorOpenSequence`))))

(event `DoorOpenSequence`
  ;[1 1 1] Open or Close the Door.
  (`GameplayStatics.PlaySoundAtLocation` "/Game/SoundDesign/SoundCues/SFX_BP/SC_SlidingDoor_A.SC_SlidingDoor_A" (`SceneComponent.K2_GetComponentLocation` (`self.DoorFrame`)) (struct) 1.0 1.0 0.0 null null null null)
  (bind (_direction _door1track) (`Timeline|Timeline_0` :!label _label)
    (:`Update`
      (`SceneComponent.K2_SetRelativeLocation` (`self.SM_porta1`) _door1track false false))))

(event `self.Box.OnComponentEndOverlap`
  (params (OverlappedComponent :type "PrimitiveComponent Object Reference") (OtherActor :type "Actor Object Reference") (OtherComp :type "PrimitiveComponent Object Reference") (OtherBodyIndex :type Integer))
  ;[1 1 1] When the Player leaves the Trigger Box
  (if (== OtherActor (`GameplayStatics.GetPlayerCharacter` 0))
    (if (`self.Door Should Operate by Trigger Box`)
      (`self.DoorCloseSequence`))))

(event `DoorCloseSequence`
  ;[1 1 1] Open or Close the Door.
  (`GameplayStatics.PlaySoundAtLocation` "/Game/SoundDesign/SoundCues/SFX_BP/SC_SlidingDoor_B.SC_SlidingDoor_B" (`SceneComponent.K2_GetComponentLocation` (`self.DoorFrame`)) (struct) 1.0 1.0 0.0 null null null null)
  (goto _label :!via `Reverse`))

(event `/Game/BP_BO/Puzzles/BPI_Unlockable.OpenTargetDoor`
  (params (Caller :type "Actor Object Reference"))
  ;[1 1 1] When Called by another Actor
  (set `self.Caller` Caller)
  (`self.DoorOpenSequence`)
  (if (`self.DoorShouldCloseAutomatically`)
    (`KismetSystemLibrary.Delay` 5.0)
    (`self.DoorCloseSequence`)
    (set `self.Door Should Operate by Trigger Box` true)
    (message `/Game/BP_BO/Puzzles/BPI_Unlockable.SetButtonUsable_Blue` (`self.Caller`) self)))

(fn `UserConstructionScript`
  (`parent.UserConstructionScript`))