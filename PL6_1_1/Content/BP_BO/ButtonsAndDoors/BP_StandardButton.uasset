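; Wall-button actor that the player interacts with to open a linked DoorToOpen, with a four-state status: red, orange, gray or blue.
; Only Usable_Blue plays the positive sound, messages the door and switches to gray in-progress; other states play a negative sound.
; The door calls back to restore blue when done, and each state drives display and button materials, also applied at construction.
; Trigger box overlap by the player toggles a custom-depth outline.
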(event `self.TriggerBox.OnComponentBeginOverlap`
  (params (OverlappedComponent :type "PrimitiveComponent Object Reference") (OtherActor :type "Actor Object Reference") (OtherComp :type "PrimitiveComponent Object Reference") (OtherBodyIndex :type Integer) (bFromSweep :type Boolean) (SweepResult :type "HitResult Structure (by ref)"))
  ;[1 1 1] Attiva/Disattiva l'Outline dell'oggetto
  (if (== OtherActor (`GameplayStatics.GetPlayerCharacter` 0))
    (`PrimitiveComponent.SetRenderCustomDepth` (`self.Frame`) true)
    (`PrimitiveComponent.SetRenderCustomDepth` (`self.Button`) true)))

(event `self.TriggerBox.OnComponentEndOverlap`
  (params (OverlappedComponent :type "PrimitiveComponent Object Reference") (OtherActor :type "Actor Object Reference") (OtherComp :type "PrimitiveComponent Object Reference") (OtherBodyIndex :type Integer))
  ;[1 1 1] Attiva/Disattiva l'Outline dell'oggetto
  (if (== (stale `self.TriggerBox.OnComponentBeginOverlap` OtherActor) (`GameplayStatics.GetPlayerCharacter` 0))
    (`PrimitiveComponent.SetRenderCustomDepth` (`self.Frame`) false)
    (`PrimitiveComponent.SetRenderCustomDepth` (`self.Button`) false)))

(event `/Game/BP_BO/Puzzles/BPI_Unlockable.SetButtonUsable_Blue`
  (params (Caller :type "Actor Object Reference"))
  ;[1 1 1] Called to make a Button Usable (DoorToOpen Actors call it when they are done opening, to reset from InProgress_Gray)
  (bind _output_get (set `self.ButtonState` "NewEnumerator2"))
  (`self.ModifyMaterials` _output_get))

(event `/Game/BP_BO/Puzzles/BPI_Unlockable.SetButtonUnusable_Red`
  ;[1 1 1] Called to make a Button Unusable
  (bind _output_get (set `self.ButtonState` "NewEnumerator0"))
  (`self.ModifyMaterials` _output_get))

(event `/Game/BP_BO/Inventory/BPI_InteractInterface.InteractWith`
  (params (PlayerCharacter :type "/Game/BP_BO/PlayerCharacter/BP_TPCharacter Object Reference"))
  ;[1 1 1] Button Interactions. Negative sound for any state but Usable_Blue. When interacted while Usable_Blue, OpenTargetDoor and switch to State InProgress_Grey
  (switch `/Game/BP_BO/ButtonsAndDoors/E_ButtonStates` (`self.ButtonState`)
    (:`NewEnumerator0`
      (`GameplayStatics.PlaySoundAtLocation` "/Game/SoundDesign/Environment_SFX/SoundCues/SC_ButtonNegative.SC_ButtonNegative" (`self.K2_GetActorLocation`) (struct) 1.0 1.0 0.0 null null null null :!label _label))
    (:`NewEnumerator1`
      (goto _label))
    (:`NewEnumerator3`
      (goto _label))
    (:`NewEnumerator2`
      (`GameplayStatics.PlaySoundAtLocation` "/Game/SoundDesign/Environment_SFX/SoundCues/SC_Button_Positive.SC_Button_Positive" (`self.K2_GetActorLocation`) (struct) 1.0 1.0 0.0 null null null null)
      (message `/Game/BP_BO/Puzzles/BPI_Unlockable.OpenTargetDoor` (`self.DoorToOpen`) self)
      (bind _output_get (set `self.ButtonState` "NewEnumerator3"))
      (`self.ModifyMaterials` _output_get))))

(fn `ModifyMaterials`
  (params (NewParam :type "/Game/BP_BO/ButtonsAndDoors/E_ButtonStates Enum" :default "NewEnumerator0"))
  (`PrimitiveComponent.SetMaterial` (`self.HolographicDisplay`) 0 (select `/Game/BP_BO/ButtonsAndDoors/E_ButtonStates` NewParam :`NewEnumerator0` "/Game/3DAssetLevel/3DArt/Materials/M_ButtonDisplay_Red.M_ButtonDisplay_Red" :`NewEnumerator1` "/Game/3DAssetLevel/3DArt/Materials/M_ButtonDisplay_Yellow.M_ButtonDisplay_Yellow" :`NewEnumerator3` "/Game/3DAssetLevel/3DArt/Materials/M_ButtonDisplay_Gray.M_ButtonDisplay_Gray" :`NewEnumerator2` "/Game/3DAssetLevel/3DArt/Materials/M_ButtonDisplay_Blue.M_ButtonDisplay_Blue" :!type "MaterialInterface Object Reference"))
  (`PrimitiveComponent.SetMaterial` (`self.Button`) 0 (select `/Game/BP_BO/ButtonsAndDoors/E_ButtonStates` NewParam :`NewEnumerator0` "/Game/3DAssetLevel/3DArt/Materials/MaterialInstances/MI_Button_Red.MI_Button_Red" :`NewEnumerator1` "/Game/3DAssetLevel/3DArt/Materials/MaterialInstances/MI_Button_Red.MI_Button_Red" :`NewEnumerator3` "/Game/3DAssetLevel/3DArt/Materials/MaterialInstances/MI_Button_Blue.MI_Button_Blue" :`NewEnumerator2` "/Game/3DAssetLevel/3DArt/Materials/MaterialInstances/MI_Button_Blue.MI_Button_Blue" :!type "MaterialInterface Object Reference")))

(fn `UserConstructionScript`
  (`PrimitiveComponent.SetMaterial` (`self.HolographicDisplay`) 0 (select `/Game/BP_BO/ButtonsAndDoors/E_ButtonStates` (`self.ButtonState`) :`NewEnumerator0` "/Game/3DAssetLevel/3DArt/Materials/M_ButtonDisplay_Red.M_ButtonDisplay_Red" :`NewEnumerator1` "/Game/3DAssetLevel/3DArt/Materials/M_ButtonDisplay_Yellow.M_ButtonDisplay_Yellow" :`NewEnumerator3` "/Game/3DAssetLevel/3DArt/Materials/M_ButtonDisplay_Gray.M_ButtonDisplay_Gray" :`NewEnumerator2` "/Game/3DAssetLevel/3DArt/Materials/M_ButtonDisplay_Blue.M_ButtonDisplay_Blue" :!type "MaterialInterface Object Reference"))
  (`PrimitiveComponent.SetMaterial` (`self.Button`) 0 (select `/Game/BP_BO/ButtonsAndDoors/E_ButtonStates` (`self.ButtonState`) :`NewEnumerator0` "/Game/3DAssetLevel/3DArt/Materials/MaterialInstances/MI_Button_Red.MI_Button_Red" :`NewEnumerator1` "/Game/3DAssetLevel/3DArt/Materials/MaterialInstances/MI_Button_Red.MI_Button_Red" :`NewEnumerator3` "/Game/3DAssetLevel/3DArt/Materials/MaterialInstances/MI_Button_Blue.MI_Button_Blue" :`NewEnumerator2` "/Game/3DAssetLevel/3DArt/Materials/MaterialInstances/MI_Button_Blue.MI_Button_Blue" :!type "MaterialInterface Object Reference")))