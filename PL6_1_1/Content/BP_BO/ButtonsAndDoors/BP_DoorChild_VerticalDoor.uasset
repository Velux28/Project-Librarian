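; Vertical door child Blueprint that slides its door mesh open and closed along a timeline.
; The open and close sequences call the parent logic, then play or reverse the timeline, which drives the relative location of SMPorta.
; When another actor triggers OpenTargetDoor, it switches a door frame material and the rect light to light blue before passing the call to the parent.
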(event `DoorOpenSequence`
  ;[1 1 1] Open or Close the Door.
  (`parent.DoorOpenSequence`)
  (bind (_direction _newtrack_1) (`Timeline|Timeline_0` :!label _label)
    (:`Update`
      (`SceneComponent.K2_SetRelativeLocation` (`self.SM_porta`) _newtrack_1 false false))))

(event `DoorCloseSequence`
  ;[1 1 1] Open or Close the Door.
  (`parent.DoorCloseSequence`)
  (goto _label :!via `Reverse`))

(event `/Game/BP_BO/Puzzles/BPI_Unlockable.OpenTargetDoor`
  (params (Caller :type "Actor Object Reference"))
  ;[1 1 1] When Called by another Actor
  (`PrimitiveComponent.SetMaterial` (`self.DoorFrame`) 4 "/Game/C_MSF_Office/Materials/Lights/MI_Light_Blue.MI_Light_Blue")
  (`LightComponent.SetLightColor` (`self.RectLight`) (struct :`G` 0.913726 :`B` 1.0 :`A` 1.0) true)
  (`parent.OpenTargetDoor` Caller))

(fn `UserConstructionScript`
  (`parent.UserConstructionScript`))