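; BP_DoorChild_DoubleDoor is a child door Blueprint for a double door with two panels that open and close.
; The open sequence calls the parent, then plays two timelines that drive the relative locations of SMPorta and SMPorta2 from separate tracks.
; The close sequence calls the parent, then reverses both timelines.
; OpenTargetDoor, triggered by another actor, and the construction script only forward to the parent.
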(event `DoorOpenSequence`
  ;[1 1 1] Open or Close the Door.
  (`parent.DoorOpenSequence`)
  (`|ExecutionSequence`
    (:`then_0`
      (bind (_direction _door1track) (`Timeline|Timeline_0` :!label _label)
        (:`Update`
          (`SceneComponent.K2_SetRelativeLocation` (`self.SM_porta`) _door1track false false))))
    (:`then_1`
      (bind (_direction_2 _door2track) (`Timeline|Timeline_1` :!label _label_2)
        (:`Update`
          (`SceneComponent.K2_SetRelativeLocation` (`self.SM_porta2`) _door2track false false))))))

(event `DoorCloseSequence`
  ;[1 1 1] Open or Close the Door.
  (`parent.DoorCloseSequence`)
  (`|ExecutionSequence`
    (:`then_0`
      (goto _label :!via `Reverse`))
    (:`then_1`
      (goto _label_2 :!via `Reverse`))))

(event `/Game/BP_BO/Puzzles/BPI_Unlockable.OpenTargetDoor`
  (params (Caller :type "Actor Object Reference"))
  ;[1 1 1] When Called by another Actor
  (`parent.OpenTargetDoor` Caller))

(fn `UserConstructionScript`
  (`parent.UserConstructionScript`))