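; Base door Blueprint that opens and closes for the player or NPCs via a trigger box, or on request from a caller.
; Open and close sequences only play sounds at the frame; children supply timeline movement.
; CanAICross gates NPC opening but not closing.
; OpenTargetDoor can auto-close after a delay, then clears that flag and messages the caller to set its button usable.
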(event `self.Box.OnComponentBeginOverlap`
  (params (OverlappedComponent :type "PrimitiveComponent Object Reference") (OtherActor :type "Actor Object Reference") (OtherComp :type "PrimitiveComponent Object Reference") (OtherBodyIndex :type Integer) (bFromSweep :type Boolean) (SweepResult :type "HitResult Structure (by ref)"))
  ;[1 1 1] When the Player enters the Trigger Box
  (if (or (== OtherActor (`GameplayStatics.GetPlayerCharacter` 0)) (and (`self.CanAICross`) (`.bSuccess` (cast `/Game/BP_BO/ArtificialIntelligence/BP_NPC` OtherActor :!pure true))))
    (if (`self.Door Should Operate by Trigger Box`)
      (`self.DoorOpenSequence`))))

(event `self.Box.OnComponentEndOverlap`
  (params (OverlappedComponent :type "PrimitiveComponent Object Reference") (OtherActor :type "Actor Object Reference") (OtherComp :type "PrimitiveComponent Object Reference") (OtherBodyIndex :type Integer))
  ;[1 1 1] When the Player leaves the Trigger Box
  (if (or (== OtherActor (`GameplayStatics.GetPlayerCharacter` 0)) (`.bSuccess` (cast `/Game/BP_BO/ArtificialIntelligence/BP_NPC` OtherActor :!pure true)))
    (if (`self.Door Should Operate by Trigger Box`)
      (`self.DoorCloseSequence`))))

(event `DoorOpenSequence`
  ;[1 1 1] Only Play sound, the child will use their own timeline
  (`GameplayStatics.PlaySoundAtLocation` (`self.DoorOpenSound`) (`SceneComponent.K2_GetComponentLocation` (`self.DoorFrame`)) (struct) 1.0 1.0 0.0 null null null null))

(event `DoorCloseSequence`
  ;[1 1 1] Only Play sound, the child will use their own timeline
  (`GameplayStatics.PlaySoundAtLocation` (`self.DoorCloseSound`) (`SceneComponent.K2_GetComponentLocation` (`self.DoorFrame`)) (struct) 1.0 1.0 0.0 null null null null))

(event `/Game/BP_BO/Puzzles/BPI_Unlockable.OpenTargetDoor`
  (params (Caller :type "Actor Object Reference"))
  (set `self.Caller` Caller)
  (`self.DoorOpenSequence`)
  (if (`self.DoorShouldCloseAutomatically`)
    (`KismetSystemLibrary.Delay` 5.0)
    (`self.DoorCloseSequence`)
    (set `self.DoorShouldCloseAutomatically` false)
    (message `/Game/BP_BO/Puzzles/BPI_Unlockable.SetButtonUsable_Blue` (`self.Caller`) self)))

(fn `UserConstructionScript`)