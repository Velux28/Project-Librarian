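; BP_Scanner is a trigger actor that repositions and activates two referenced scanners, SightScanner and BreathScanner, when another actor overlaps it.
; On overlap it zeroes SightScanner's rotation, sets its maximum scan angle to a fixed value and teleports it to the trigger's location.
; It also moves BreathScanner to the overlapping actor and enables its box collision.
; The node that would disable that collision is unconnected, so this Blueprint never switches it off.
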(event `self.ReceiveBeginPlay`)

(event `self.ReceiveActorBeginOverlap`
  (params (OtherActor :type "Actor Object Reference"))
  (bind _sightscanner (`self.SightScanner`))
  (bind _breathscanner (`self.BreathScanner`))
  (`self.K2_SetActorRotation` :`self` _sightscanner)
  (set `/Game/BP_ScanFX_SwipingBeam.Scan Max Angle` 180.0 _sightscanner)
  (`self.K2_SetActorLocation` _sightscanner (`self.K2_GetActorLocation` self) false true)
  (`self.K2_SetActorLocation` _breathscanner (`self.K2_GetActorLocation` OtherActor) false false)
  (`PrimitiveComponent.SetCollisionEnabled` (`/Game/C_ScanFX/Blueprints/BP_ScanFX_PostProcess_Visualizer.Box` _breathscanner) "QueryAndPhysics"))

(fn `UserConstructionScript`)