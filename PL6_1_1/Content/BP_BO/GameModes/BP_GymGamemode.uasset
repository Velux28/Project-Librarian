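; BP_GymGamemode is a game mode that handles save loading and player death for a checkpoint system.
; On BeginPlay it binds player destruction, optionally loads the save slot, spawns BP_Load and, for a matching map, restores player transform and item flags.
; On death with a spawn set, it spawns and possesses a new character, opens MAP_Gym and shows an items-reset widget.
; Otherwise it opens SUBMAP_Persistent; several leftover node chains never run.
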(event `Destroyed` :!signature `self.OnDestroyed`
  (params (DestroyedActor :type "Actor Object Reference"))
  ;[1 1 1] Non so cosa sia
)

(event `Key|LeftMouseButton`
  (params (Key :type "Key Structure"))
  ;[1 0 0.1651] wip puzzle
)

(event `self.ReceiveBeginPlay`
  (bind _gamefile (`self.GameFile`))
  (bind _playertransform (`SaveGameFile.PlayerTransform` (`self.GameFile`)))
  ;[1 0.45 0] CheckpointSystem
  (bind _asbp_tpcharacter (cast `/Game/BP_BO/PlayerCharacter/BP_TPCharacter` (`GameplayStatics.GetPlayerCharacter` 0)))
  (bind _output_get (set `self.As BP TPCharacter` _asbp_tpcharacter))
  (add `self.OnDestroyed` _output_get (delegate `Player Death`))
  (if (`self.LoadSaveFile`)
    (bind _returnvalue (`GameplayStatics.LoadGameFromSlot` "Slot1"))
    (`/Engine/EditorBlueprintResources/StandardMacros.IsValid` _returnvalue
      (:`Is Valid`
        (bind _assave_game_file (cast `SaveGameFile` _returnvalue))
        (set `self.GameFile` _assave_game_file)
        (bind _returnvalue_2 (`GameplayStatics.GetCurrentLevelName` true))
        (if (`KismetStringLibrary.EqualEqual_StrStr` _returnvalue_2 (`KismetStringLibrary.Conv_NameToString` (`SaveGameFile.CurrMap` _gamefile)))
          (set `self.Load` true)
          (set `self.CurrSectionToLoad` 0)
          (set `self.TotalSectionToLoad` (`KismetArrayLibrary.Array_Length` (`SaveGameFile.CurrSection` _gamefile)))
          (`|SpawnActorFromClass` "/Game/BP_BO/Environment/BP_Load.BP_Load_C" _playertransform "Undefined" "OverrideRootScale" null null)
          (`self.K2_SetActorTransform` (`self.As BP TPCharacter`) _playertransform false true)
          (set `/Game/BP_BO/PlayerCharacter/BP_TPCharacter.HasScrewdriver` (`SaveGameFile.HasScrewdriver` (`self.GameFile`)) (`self.As BP TPCharacter`))
          (set `/Game/BP_BO/PlayerCharacter/BP_TPCharacter.HasPowerCell` (`SaveGameFile.HasPowerCell` (`self.GameFile`)) (`self.As BP TPCharacter`))
          (else
            (`|SpawnActorFromClass` "/Game/BP_BO/Environment/BP_Load.BP_Load_C" (`KismetMathLibrary.MakeTransform` (0.0 0.0 0.0)) "Undefined" "OverrideRootScale" null null :!label _label))))
      (:`Is Not Valid`
        (bind _returnvalue_3 (`GameplayStatics.CreateSaveGameObject` "/Script/PL6_1.SaveGameFile"))
        (set `self.GameFile` _returnvalue_3)
        (goto _label)))))

(event `Player Death` :!signature `self.OnDestroyed`
  (params (DestroyedActor :type "Actor Object Reference"))
  ;[1 0.45 0] CheckpointSystem
  (if (`self.SpawnIsSet`) :!pinned true
    (bind _returnvalue (`|SpawnActorFromClass` "/Game/BP_BO/PlayerCharacter/BP_TPCharacter.BP_TPCharacter_C" (`SaveGameFile.PlayerTransform` (`self.GameFile`)) "AlwaysSpawn" "OverrideRootScale" null null))
    (bind _returnvalue_2 (`GameplayStatics.GetActorOfClass` null))
    (`/Engine/EditorBlueprintResources/StandardMacros.IsValid` _returnvalue_2
      (:`Is Valid`
        _)
      (:`Is Not Valid`
        _))
    (bind _asmy_player_controller (cast `/Game/BP_BO/PlayerCharacter/MyPlayerController` (`GameplayStatics.GetPlayerController` 0)))
    (`/Game/BP_BO/PlayerCharacter/MyPlayerController.OnRespawn` _asmy_player_controller)
    (`KismetSystemLibrary.Delay` 0.2)
    (`Controller.Possess` _asmy_player_controller _returnvalue)
    (`self.Respawn`)
    (bind _returnvalue_3 (`|CreateWidget` "/Game/UI/PlayerUI/Basic_UI/W_ItemsReset.W_ItemsReset_C"))
    (`UserWidget.AddToViewport` _returnvalue_3 0)
    (`Widget.SetVisibility` _returnvalue_3 "Visible")
    (`KismetSystemLibrary.Delay` 3.0)
    (`Widget.SetVisibility` _returnvalue_3 "Hidden")
    (else
      (`KismetSystemLibrary.Delay` 0.2)
      (`GameplayStatics.OpenLevelBySoftObjectPtr` "/Game/3DAssetLevel/LevelDesign/Maps/SUBMAP_Persistent.SUBMAP_Persistent"))))

(event `Respawn`
  (`GameplayStatics.OpenLevelBySoftObjectPtr` "/Game/3DAssetLevel/LevelDesign/Maps/Gym/MAP_gym.MAP_Gym"))

(fn `UserConstructionScript`)