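; BP_SlidingDoor1 is a sliding door that slides its right panel when OpenGate02 fires and starts closing after a six-second delay.
; Separate open and close timelines lerp the panel's relative location between zero and RightPanelV, each accompanied by a sound at a hard-coded world position.
; A DoOnce gates the sequence but resets right after the delay begins, without waiting for the close.
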(event `Open Gate 02`
  (params (PlayerCharacter :type "/Game/BP_BO/PlayerCharacter/BP_TPCharacter Object Reference"))
  (`/Engine/EditorBlueprintResources/StandardMacros.DoOnce` false :!label _label
    (:`Completed`
      (`|ExecutionSequence`
        (:`then_0`
          (`GameplayStatics.PlaySoundAtLocation` "/Game/BO_Custom/SOUNDS/TUT_LEV/Cues/SC_SlidingDoor.SC_SlidingDoor" (-1431.0 5297.0 0.0) (struct) 1.0 1.0 0.0 null "/Game/BO_Custom/SOUNDS/TUT_LEV/Cues/CONC_Environment.CONC_Environment" null null)
          (bind (_direction _newtrack_0) (`Timeline|TML_OPEN` :!via `PlayFromStart`)
            (:`Update`
              (`SceneComponent.K2_SetRelativeLocation` (`self.RightPanel`) (`KismetMathLibrary.VLerp` (0.0 0.0 0.0) (`self.RightPanelV`) _newtrack_0) false false))))
        (:`then_1`
          (`KismetSystemLibrary.Delay` 6.0)
          (`GameplayStatics.PlaySoundAtLocation` "/Game/BO_Custom/SOUNDS/TUT_LEV/Cues/SC_SlidingDoor.SC_SlidingDoor" (-1431.0 5297.0 0.0) (struct) 1.0 1.0 0.0 null "/Game/BO_Custom/SOUNDS/TUT_LEV/Cues/CONC_Environment.CONC_Environment" null null)
          (bind (_direction_2 _newtrack_0_2) (`Timeline|TML_CLOSE` :!via `PlayFromStart`)
            (:`Update`
              (`SceneComponent.K2_SetRelativeLocation` (`self.RightPanel`) (`KismetMathLibrary.VLerp` (0.0 0.0 0.0) (`self.RightPanelV`) _newtrack_0_2) false false))))
        (:`then_2`
          (goto _label :!via `Reset`))))))

(fn `UserConstructionScript`)