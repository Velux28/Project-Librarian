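; BP_SlidingDoor2 is a two-panel sliding door that opens on the OpenGate event and closes after a delay.
; A timeline lerps the left and right panels' relative locations, with a sound played at a hardcoded location.
; A seven-second Delay chained to the timeline's Update, not Finished, replays the sound and reverses the timeline, so reverse updates re-arm it.
; The BP_CardGate lookup is disconnected and never runs.
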(event `Open Gate`
  (params (PlayerCharacter :type "Actor Object Reference"))
  (`GameplayStatics.PlaySoundAtLocation` "/Game/BO_Custom/SOUNDS/TUT_LEV/Cues/SC_SlidingDoor.SC_SlidingDoor" (-24.0 445.0 -29.0) (struct) 1.0 1.0 0.0 null "/Game/BO_Custom/SOUNDS/TUT_LEV/Cues/CONC_Environment.CONC_Environment" null null)
  (bind (_direction _newtrack_0) (`Timeline|OPENING TIMELINE` :!via `PlayFromStart` :!label _label)
    (:`Update`
      (`SceneComponent.K2_SetRelativeLocation` (`self.RightPanel`) (`KismetMathLibrary.VLerp` (-4.0 0.0 0.0) (`self.RightPanelV`) _newtrack_0) false false)
      (`SceneComponent.K2_SetRelativeLocation` (`self.LeftPanel`) (`KismetMathLibrary.VLerp` (4.0 0.0 0.0) (`self.LeftPanelV`) _newtrack_0) false false)
      (`KismetSystemLibrary.Delay` 7.0)
      (`GameplayStatics.PlaySoundAtLocation` "/Game/BO_Custom/SOUNDS/TUT_LEV/Cues/SC_SlidingDoor.SC_SlidingDoor" (-24.0 445.0 -29.0) (struct) 1.0 1.0 0.0 null "/Game/BO_Custom/SOUNDS/TUT_LEV/Cues/CONC_Environment.CONC_Environment" null null)
      (goto _label :!via `Reverse`))))

(fn `UserConstructionScript`)