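; CCTV server prop that shuts down during a cinematic and then serves as the level-ending interaction.
; Cinematic starts a timer that switches random boxes off, reveals sparks at two of them, then enables interaction and randomly toggles sparks.
; Interacting disables input, plays the fainting sequence, fades out, shows a loading screen and opens SUBMAP_Persistent.
; With IsSubmap1 set, all box lights start off.
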(event `/Game/BP_BO/Inventory/BPI_InteractInterface.InteractWith`
  (params (PlayerCharacter :type "/Game/BP_BO/PlayerCharacter/BP_TPCharacter Object Reference"))
  (if (`self.ReadyForInteraction`)
    (`/Engine/EditorBlueprintResources/StandardMacros.DoOnce` false
      (:`Completed`
        (`KismetSystemLibrary.PrintString` "Hai preso la scossa e sei svenuto" true true (struct :`G` 1.0 :`A` 1.0) 10.0)
        (`self.DisableInput` PlayerCharacter (`GameplayStatics.GetPlayerController` 0))
        (`Widget.RemoveFromParent` (`/Game/BP_BO/PlayerCharacter/BP_TPCharacter.Manina` PlayerCharacter))
        ;[1 1 1] Attivazione LevelSequence Fine Livello
        (`SceneComponent.SetVisibility` (`Character.Mesh` (`GameplayStatics.GetPlayerCharacter` 0)) false true)
        (bind _outactor (`LevelSequencePlayer.CreateLevelSequencePlayer` "/Game/3DAssetLevel/LevelDesign/Cutscenes/LS_CCTV_Fainting.LS_CCTV_Fainting"))
        (`MovieSceneSequencePlayer.Play` (`LevelSequenceActor.SequencePlayer` _outactor))
        (`KismetSystemLibrary.Delay` 1.5)
        (`PlayerCameraManager.StartCameraFade` :`self` (`GameplayStatics.GetPlayerCameraManager` 0) :`ToAlpha` 1.0 :`Duration` 2.0 :`bHoldWhenFinished` true)
        (`KismetSystemLibrary.Delay` 2.0)
        (bind _returnvalue (`|CreateWidget` "/Game/UI/PlayerUI/Basic_UI/W_UI_LoadingScreen.W_UI_LoadingScreen_C"))
        (`UserWidget.AddToViewport` _returnvalue 0)
        ;[1 1 1] Passaggio a Level_1
        (`GameplayStatics.OpenLevelBySoftObjectPtr` "/Game/3DAssetLevel/LevelDesign/Maps/SUBMAP_Persistent.SUBMAP_Persistent")))))

(event `Cinematic`
  ;[1 1 1] Chiamato dalla cinematic della CCTV_Chair, metodo eccessivamente complicato per spegnere le lucine dei server (change Material to MI_Server_OFF) e accendere le scintille quando vengono chiamati i pezzi di server corrispondenti (Box5A e Box7B).
  ; Spenti tutti i Box il server diventa interagibile e le scintille si accendono e spengono a intervalli randomici. (fa schifo)
  (bind _returnvalue (`KismetSystemLibrary.K2_SetTimerDelegate` (delegate `CustomEvent_0`) 0.2 true)))

(event `CustomEvent_0`
  (bind _array (`self.Array`))
  ;[1 1 1] Chiamato dalla cinematic della CCTV_Chair, metodo eccessivamente complicato per spegnere le lucine dei server (change Material to MI_Server_OFF) e accendere le scintille quando vengono chiamati i pezzi di server corrispondenti (Box5A e Box7B).
  ; Spenti tutti i Box il server diventa interagibile e le scintille si accendono e spengono a intervalli randomici. (fa schifo)
  (bind _output_get (set `self.Current Gizmo` (`KismetArrayLibrary.Array_Random` (`self.Array`))))
  (`PrimitiveComponent.SetMaterial` _output_get 0 "/Game/C_ScienceLab/Materials/ScientificDevice/MI_Server_OFF.MI_Server_OFF")
  (if (== (`self.Box5A`) (`self.Current Gizmo`))
    (`SceneComponent.SetVisibility` (`self.ParticleSystem`) true false)
    (elif (== (`self.Box7B`) (`self.Current Gizmo`))
      (`SceneComponent.SetVisibility` (`self.ParticleSystem1`) true false)))
  (`KismetArrayLibrary.Array_RemoveItem` _array (`self.Current Gizmo`))
  (if (`KismetArrayLibrary.Array_IsEmpty` _array)
    (`KismetSystemLibrary.K2_ClearAndInvalidateTimerHandle` (stale `Cinematic` _returnvalue))
    (set `self.ReadyForInteraction` true)
    (`KismetSystemLibrary.K2_SetTimerDelegate` (delegate `CustomEvent_1`) (`KismetMathLibrary.FClamp` (`KismetMathLibrary.RandomFloat`) 1.0 3.0) true)))

(event `CustomEvent_1`
  (bind _outitem (`KismetArrayLibrary.Array_Random` (`|MakeArray` (`self.ParticleSystem`) (`self.ParticleSystem1`))))
  ;[1 1 1] Chiamato dalla cinematic della CCTV_Chair, metodo eccessivamente complicato per spegnere le lucine dei server (change Material to MI_Server_OFF) e accendere le scintille quando vengono chiamati i pezzi di server corrispondenti (Box5A e Box7B).
  ; Spenti tutti i Box il server diventa interagibile e le scintille si accendono e spengono a intervalli randomici. (fa schifo)
  (if (`SceneComponent.IsVisible` _outitem)
    (`SceneComponent.SetVisibility` _outitem false false)
    (else
      (`SceneComponent.SetVisibility` _outitem true false))))

(event `self.ReceiveBeginPlay`
  ;[1 1 1] Se siamo in Submap1 spegne le lucette
  (set `self.Array` (`|MakeArray` (`self.Box1A`) (`self.Box2A`) (`self.Box3A`) (`self.Box4A`) (`self.Box5A`) (`self.Box6A`) (`self.Box7A`) (`self.Box1B`) (`self.Box2B`) (`self.Box3B`) (`self.Box4B`) (`self.Box5B`) (`self.Box6B`) (`self.Box7B`) (`self.Box8B`)))
  (if (`self.IsSubmap1`)
    (for _array_element (`self.Array`)
      (`PrimitiveComponent.SetMaterial` _array_element 0 "/Game/C_ScienceLab/Materials/ScientificDevice/MI_Server_OFF.MI_Server_OFF"))))

(fn `UserConstructionScript`)