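; Assembly-line conveyor that carries a looping row of spawned mesh props along a spline.
; BeginPlay spawns a fixed pool of actors with meshes picked randomly or by index from ObjToSpawn.
; Tick advances a speed-scaled timer, placing each item on the spline offset by its array index.
; A box overlap recycles items to the queue's tail, rewinding the timer, and destroys other actors except non-player BP_NPCs.
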(event `self.ReceiveBeginPlay`
  (set `self.SpawnDelay` (* (`self.SpawnDelay`) (`self.Speed`)))
  (for _ (range 21)
    (`self.SpawnItem`)))

(event `self.ReceiveTick`
  (params (DeltaSeconds :type "Float (single-precision)"))
  (`|ExecutionSequence`
    (:`then_1`
      (set `self.Timer` (+ (* DeltaSeconds (`self.Speed`)) (`self.Timer`)))
      (`self.Move Obj`))))

(event `self.Box.OnComponentBeginOverlap`
  (params (OverlappedComponent :type "PrimitiveComponent Object Reference") (OtherActor :type "Actor Object Reference") (OtherComp :type "PrimitiveComponent Object Reference") (OtherBodyIndex :type Integer) (bFromSweep :type Boolean) (SweepResult :type "HitResult Structure (by ref)"))
  (if (not (and (!= OtherActor (`GameplayStatics.GetPlayerCharacter` 0)) (`.bSuccess` (cast `/Game/BP_BO/ArtificialIntelligence/BP_NPC` OtherActor :!pure true))))
    (`self.DestroyItem` OtherActor)))

(fn `DestroyItem`
  (params (ObjToDestroy :type "Actor Object Reference"))
  (bind _items (`self.Items`))
  (bind _returnvalue (`KismetArrayLibrary.Array_RemoveItem` _items ObjToDestroy))
  (if _returnvalue
    (set `self.Timer` (- (`self.Timer`) (`self.SpawnDelay`)))
    (`KismetArrayLibrary.Array_Add` _items ObjToDestroy)
    (else
      (`self.K2_DestroyActor` ObjToDestroy))))

(fn `Move Obj`
  (for (_array_element _array_index) (`self.Items`)
    (`self.K2_SetActorLocation` _array_element (`SplineComponent.GetLocationAtTime` (`self.Spline`) (`KismetMathLibrary.FMax` (- (`self.Timer`) (* _array_index (`self.SpawnDelay`)))) "World" false) false false)))

(fn `SpawnItem`
  (locals (Temp :type "Actor Object Reference"))
  (bind _objindex (`self.ObjIndex`))
  (bind _objtospawn (`self.ObjToSpawn`))
  (bind _returnvalue (`KismetArrayLibrary.Array_Length` _objtospawn))
  (bind _returnvalue_2 (`SplineComponent.GetTransformAtTime` (`self.Spline`) 0.0 "World" false false))
  (bind _returnvalue_3 (`|SpawnActorFromClass` "/Script/Engine.Actor" _returnvalue_2 "AlwaysSpawn" "OverrideRootScale" null null))
  (bind _output_get (set `local.Temp` _returnvalue_3))
  (bind _returnvalue_4 (`AddComponent|NODE_AddStaticMeshComponent-1` :`self` _output_get :`RelativeTransform` _returnvalue_2))
  (`StaticMeshComponent.SetStaticMesh` _returnvalue_4 (`|GetArrayItem` _objtospawn (`KismetMathLibrary.SelectInt` (`KismetMathLibrary.RandomInteger` _returnvalue) (mod _objindex _returnvalue) (<= _objindex -1))))
  (`KismetArrayLibrary.Array_Add` (`self.Items`) (`local.Temp`))
  (return))

(fn `UserConstructionScript`)