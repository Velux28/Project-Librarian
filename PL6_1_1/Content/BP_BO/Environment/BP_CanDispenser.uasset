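; Can dispenser that acts as a save point, giving the player a can and saving the game on interaction.
; Overlapping its trigger toggles a custom-depth outline for the player.
; With stock and saving enabled, it flashes a green grid, waits, hands over a can, saves through ACSaveComponent and sets checkpoint text; when empty, a gated red flash signals failure.
; IncrementCanNumber resets stock to one with a pulsing green material.
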(event `self.TriggerBox.OnComponentBeginOverlap`
  (params (OverlappedComponent :type "PrimitiveComponent Object Reference") (OtherActor :type "Actor Object Reference") (OtherComp :type "PrimitiveComponent Object Reference") (OtherBodyIndex :type Integer) (bFromSweep :type Boolean) (SweepResult :type "HitResult Structure (by ref)"))
  ;[1 1 1] Attiva/Disattiva l'Outline dell'oggetto
  (if (== OtherActor (`GameplayStatics.GetPlayerCharacter` 0))
    (`PrimitiveComponent.SetRenderCustomDepth` (`self.CanDispenser`) true)))

(event `self.TriggerBox.OnComponentEndOverlap`
  (params (OverlappedComponent :type "PrimitiveComponent Object Reference") (OtherActor :type "Actor Object Reference") (OtherComp :type "PrimitiveComponent Object Reference") (OtherBodyIndex :type Integer))
  ;[1 1 1] Attiva/Disattiva l'Outline dell'oggetto
  (if (== OtherActor (`GameplayStatics.GetPlayerCharacter` 0))
    (`PrimitiveComponent.SetRenderCustomDepth` (`self.CanDispenser`) false)))

(event `self.ReceiveBeginPlay`
  (bind _candispenser (`self.CanDispenser`))
  (set `self.Can Number` (`self.Can Capacity`))
  (bind _returnvalue (`PrimitiveComponent.CreateDynamicMaterialInstance` _candispenser 1 (`PrimitiveComponent.GetMaterial` _candispenser 1) "None"))
  (set `self.MID Decals` _returnvalue))

(event `/Game/BP_BO/Inventory/BPI_InteractInterface.InteractWith`
  (params (PlayerCharacter :type "/Game/BP_BO/PlayerCharacter/BP_TPCharacter Object Reference"))
  (if (> (`self.Can Number`) 0)
    (if (`self.ShouldSave`)
      (set `self.IsSaving` true)
      (`PrimitiveComponent.SetMaterial` (`self.CanDispenser`) 2 "/Game/3DAssetLevel/LevelDesign/Materials/BlockoutMats/GridMats/Generic/MI_Grid_GREEN.MI_Grid_GREEN")
      (`KismetSystemLibrary.Delay` (`self.Can Drop Timer`))
      (`/Engine/EditorBlueprintResources/StandardMacros.DecrementInt` (`self.Can Number`)
        (:`  `
          (`/Game/BP_BO/PlayerCharacter/BP_TPCharacter.AddCan` PlayerCharacter)
          ;[1 1 1] Save only if the dispencer has a can
          (`/Game/BP_BO/Environment/AC_SaveComponent.Save` (`self.AC_SaveComponent`) PlayerCharacter)
          (`PrimitiveComponent.SetMaterial` (`self.CanDispenser`) 2 "/Game/3DAssetLevel/LevelDesign/Materials/BlockoutMats/GridMats/Generic/MI_Grid_BLACK.MI_Grid_BLACK")
          (`TextRenderComponent.K2_SetText` (`self.CHECKPOINT`) (`self.MESSAGE TEXT`))
          (set `self.IsSaving` false)))
      (else
        (`KismetSystemLibrary.PrintString` "IL GIOCO SAREBBE STATO SALVATO \nMA \"SHOULD SAVE\" è FALSE" true true (struct :`R` 1.0 :`A` 1.0)) ; Serve in fase di testing per non creare saveslot in Gym
      ))
    (else
      (set `self.IsSaving` false)
      ;[1 1 1] Se non ha lattine, feedback visivo di mancato salvataggio
      (`/Engine/EditorBlueprintResources/StandardMacros.DoOnce` false :!label _label
        (:`Completed`
          (`PrimitiveComponent.SetMaterial` (`self.CanDispenser`) 2 "/Game/3DAssetLevel/LevelDesign/Materials/BlockoutMats/GridMats/Generic/MI_Grid_RED.MI_Grid_RED")
          (`KismetSystemLibrary.Delay` 1.0)
          (`PrimitiveComponent.SetMaterial` (`self.CanDispenser`) 2 "/Game/3DAssetLevel/LevelDesign/Materials/BlockoutMats/GridMats/Generic/MI_Grid_BLACK.MI_Grid_BLACK")
          (goto _label :!via `Reset`))))))

(fn `Check IF Interactable`
  (returns (`Is NOT Interactable` :type Boolean))
  (return false))

(fn `Increment Can Number`
  (set `self.Can Number` 1)
  (`PrimitiveComponent.SetMaterial` (`self.CanDispenser`) 1 "/Game/3DAssetLevel/NewRoom/Material/M_Pulse_green.M_Pulse_green"))

(fn `UserConstructionScript`)