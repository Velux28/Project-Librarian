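; Actor component that saves player progress to a save slot through its Save function.
; Save takes a player reference and writes the player's transform, can count and current level name into the GameFile held by BP_TPGamemode.
; It then saves that object to a single hardcoded slot.
; Nodes for flagging the spawn as set and playing a checkpoint sound are present but disconnected.
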(fn `Save`
  (params (`Player Ref` :type "/Game/BP_BO/PlayerCharacter/BP_TPCharacter Object Reference"))
  (locals (`Game mode` :type "/Game/BP_BO/PlayerCharacter/BP_TPGamemode Object Reference"))
  (bind _gamefile (`/Game/BP_BO/PlayerCharacter/BP_TPGamemode.GameFile` (`local.Game mode`)))
  (`|ExecutionSequence`
    (:`then_0`
      (bind _asbp_tpgamemode (cast `/Game/BP_BO/PlayerCharacter/BP_TPGamemode` (`GameplayStatics.GetGameMode`)))
      (set `local.Game mode` _asbp_tpgamemode)
      (set `SaveGameFile.PlayerTransform` (`Actor.GetTransform` (`local.Player Ref`)) _gamefile)
      (set `SaveGameFile.PlayerItems` (`/Game/BP_BO/PlayerCharacter/BP_TPCharacter.Number of Cans` (`local.Player Ref`)) _gamefile)
      (bind _returnvalue (`GameplayStatics.GetCurrentLevelName` true))
      (set `SaveGameFile.CurrMap` (`KismetStringLibrary.Conv_StringToName` _returnvalue) _gamefile))
    (:`then_1`
      (`GameplayStatics.SaveGameToSlot` (`/Game/BP_BO/PlayerCharacter/BP_TPGamemode.GameFile` (`local.Game mode`)) "Slot1"))))