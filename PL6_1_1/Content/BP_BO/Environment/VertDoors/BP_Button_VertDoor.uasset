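; BP_Button_VertDoor is an interactable button that opens vertical doors in the level.
; On interact, it plays a click sound at a hardcoded world location, then searches all BP_VerticalDoor actors for a GateValue equal to its ButtonValue.
; Matching doors open with the interacting player passed in.
; A DoOnce blocks repeat presses until a nine-second delay after a match resets it; LookAt returns the "Button" label.
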(event `/Game/BP_BO/Inventory/BPI_InteractInterface.InteractWith`
  (params (PlayerCharacter :type "/Game/BP_BO/PlayerCharacter/BP_TPCharacter Object Reference"))
  (`/Engine/EditorBlueprintResources/StandardMacros.DoOnce` false :!label _label
    (:`Completed`
      (`GameplayStatics.PlaySoundAtLocation` "/Game/BO_Custom/SOUNDS/TUT_LEV/Cues/SC_Button.SC_Button" (505.0 7609.0 124.0) (struct) 1.0 1.0 0.0 null null null null)
      (bind _outactors (`GameplayStatics.GetAllActorsOfClass` "/Game/BP_BO/Environment/VertDoors/BP_VerticalDoor.BP_VerticalDoor_C"))
      (for _array_element _outactors
        (if (== (`/Game/BP_BO/Environment/VertDoors/BP_VerticalDoor.Gate Value` _array_element) (`self.ButtonValue`))
          (`/Game/BP_BO/Environment/VertDoors/BP_VerticalDoor.OpenVerticalDoor` _array_element PlayerCharacter)
          (`KismetSystemLibrary.Delay` 9.0)
          (goto _label :!via `Reset`))))))

(fn `LookAt`
  (returns (Message :type Text))
  (return "Button"))

(fn `UserConstructionScript`)