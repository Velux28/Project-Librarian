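; Vertical sliding door that moves its panel 240 units along local Z when the OpenVerticalDoor event fires.
; One timeline drives the panel immediately and a second, meant for closing, runs after a six-second delay, both lerping between the same two positions.
; Each movement plays a sliding sound at a hard-coded world location.
; The DoOnce gate resets in the same sequence without waiting for the delay, so the event can retrigger mid-cycle.
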(event `OpenVerticalDoor`
  (params (PlayerCharacter :type "Actor Object Reference"))
  (`/Engine/EditorBlueprintResources/StandardMacros.DoOnce` false :!label _label
    (:`Completed`
      (`|ExecutionSequence`
        (:`then_0`
          (`GameplayStatics.PlaySoundAtLocation` "/Game/BO_Custom/SOUNDS/TUT_LEV/Cues/SC_SlidingDoor.SC_SlidingDoor" (245.0 7709.0 4.0) (struct) 1.0 -0.5 0.0 null "/Game/BO_Custom/SOUNDS/TUT_LEV/Cues/CONC_Environment.CONC_Environment" null null)
          (bind (_direction _newtrack_0) (`Timeline|SlidingTimeline` :!via `PlayFromStart`)
            (:`Update`
              (`SceneComponent.K2_SetRelativeLocation` (`self.RightPanel`) (`KismetMathLibrary.VLerp` (0.0 0.0 0.0) (0.0 0.0 240.0) _newtrack_0) false false))))
        (:`then_1`
          (`KismetSystemLibrary.Delay` 6.0)
          (`GameplayStatics.PlaySoundAtLocation` "/Game/BO_Custom/SOUNDS/TUT_LEV/Cues/SC_SlidingDoor.SC_SlidingDoor" (245.0 7709.0 4.0) (struct) 1.0 -0.5 0.0 null "/Game/BO_Custom/SOUNDS/TUT_LEV/Cues/CONC_Environment.CONC_Environment" null null)
          (bind (_direction_2 _newtrack_0_2) (`Timeline|Closing Timeline` :!via `PlayFromStart`)
            (:`Update`
              (`SceneComponent.K2_SetRelativeLocation` (`self.RightPanel`) (`KismetMathLibrary.VLerp` (0.0 0.0 0.0) (0.0 0.0 240.0) _newtrack_0_2) false false))))
        (:`then_2`
          (goto _label :!via `Reset`))))))

(fn `UserConstructionScript`)