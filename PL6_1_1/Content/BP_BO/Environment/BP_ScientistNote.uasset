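; BP_ScientistNote is an interactable environment note that opens and closes a notes widget on screen.
; Its Interactwith event drives a FlipFlop: one press creates and shows W_Appunti_1 and locks look and move input, the next collapses the widget and restores input.
; Each reopen creates a new widget instance rather than reusing the collapsed one.
; Its LookAt function returns an empty string.
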(event `/Game/BP_BO/Inventory/BPI_InteractInterface.InteractWith`
  (params (PlayerCharacter :type "/Game/BP_BO/PlayerCharacter/BP_TPCharacter Object Reference"))
  (bind _returnvalue (`GameplayStatics.GetPlayerController` 0))
  (bind _returnvalue_2 (`GameplayStatics.GetPlayerController` 0))
  (`/Engine/EditorBlueprintResources/StandardMacros.FlipFlop`
    (:`A`
      (bind _returnvalue_3 (`|CreateWidget` "/Game/UI/PlayerUI/Environment_UI/Interactions/W_Appunti_1.W_Appunti_1_C"))
      (bind _output_get (set `self.WIDG_Appunti_1` _returnvalue_3))
      (`UserWidget.AddToViewport` _output_get 0)
      (`Controller.SetIgnoreLookInput` _returnvalue_2 true)
      (`Controller.SetIgnoreMoveInput` _returnvalue_2 true))
    (:`B`
      (`Widget.SetVisibility` (`self.WIDG_Appunti_1`) "Collapsed")
      (`Controller.ResetIgnoreMoveInput` _returnvalue)
      (`Controller.ResetIgnoreLookInput` _returnvalue))))

(fn `LookAt`
  (returns (Message :type Text))
  (return ""))

(fn `UserConstructionScript`)