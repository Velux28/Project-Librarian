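; BP_fondocestino is an environment Blueprint that plays a one-time end sequence when its SitEvent fires, ending in a load of LEVEL_1.
; A DoOnce gate clears all widgets, then a chain of Delays shows the launch-end, coffee and sleep widgets in turn.
; The camera fades out and holds before the sleep widget appears and the level opens.
; The construction script is empty.
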(event `SitEvent`
  (`/Engine/EditorBlueprintResources/StandardMacros.DoOnce` false
    (:`Completed`
      (`WidgetLayoutLibrary.RemoveAllWidgets`)
      (bind _returnvalue (`|CreateWidget` "/Game/Level_0/Environment/Blueprint/Widgets/LaunchWidgets/W_LaunchEnd.W_LaunchEnd_C"))
      (bind _output_get (set `self.W_LaunchEnd` _returnvalue))
      (`UserWidget.AddToViewport` _output_get 0)
      (`KismetSystemLibrary.Delay` 1.0)
      (bind _returnvalue_2 (`|CreateWidget` "/Game/Level_0/Environment/Blueprint/Widgets/W_PlayerCoffe.W_PlayerCoffe_C"))
      (bind _output_get_2 (set `self.W_COFFE` _returnvalue_2))
      (`UserWidget.AddToViewport` _output_get_2 0)
      (`KismetSystemLibrary.Delay` 4.0)
      (`PlayerCameraManager.StartCameraFade` :`self` (`GameplayStatics.GetPlayerCameraManager` 0) :`ToAlpha` 1.0 :`Duration` 3.0 :`bHoldWhenFinished` true)
      (`KismetSystemLibrary.Delay` 3.0)
      (bind _returnvalue_3 (`|CreateWidget` "/Game/Level_0/Environment/Blueprint/Widgets/W_PlayerSleep.W_PlayerSleep_C"))
      (bind _output_get_3 (set `self.W_SLEEP` _returnvalue_3))
      (`UserWidget.AddToViewport` _output_get_3 0)
      (`KismetSystemLibrary.Delay` 3.0)
      (`GameplayStatics.OpenLevel` "LEVEL_1"))))

(fn `UserConstructionScript`)