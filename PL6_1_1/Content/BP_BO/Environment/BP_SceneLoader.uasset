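; BP_SceneLoader is an overlap-triggered actor that streams a sublevel in or out when the player's controlled pawn enters it.
; Its LoadUnload flag selects between a non-blocking load, made visible on completion, and a non-blocking unload of the SublevelREF soft reference.
; The load path also writes the sublevel's name to GameFile.CurrSection on BP_TPGamemode.
; Older name-based load and unload nodes using NextLevel remain disconnected.
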(event `self.ReceiveActorBeginOverlap`
  (params (OtherActor :type "Actor Object Reference"))
  (bind _sublevelref (`self.SublevelREF`))
  (if (== OtherActor (`Controller.K2_GetPawn` (`GameplayStatics.GetPlayerController` 0)))
    (if (`self.Load/Unload`)
      (`GameplayStatics.LoadStreamLevelBySoftObjectPtr` _sublevelref true)
      (bind _asbp_tpgamemode (cast `/Game/BP_BO/PlayerCharacter/BP_TPGamemode` (`GameplayStatics.GetGameMode`)))
      (set `SaveGameFile.CurrSection` (`KismetStringLibrary.Conv_StringToName` (`KismetSystemLibrary.GetObjectName` (`|ConvertAsset` _sublevelref))) (`/Game/BP_BO/PlayerCharacter/BP_TPGamemode.GameFile` _asbp_tpgamemode))
      (else
        (`GameplayStatics.UnloadStreamLevelBySoftObjectPtr` _sublevelref)))))

(fn `UserConstructionScript`)