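; Interactable security panel that starts a code or hack puzzle on the player and opens its target door when solved.
; Interaction fires once, passing puzzle type and difficulty to the player, and rearms when PuzzleFailed is received.
; A trigger box toggles the custom depth outline while the player overlaps.
; Solving disables the highlight trigger, swaps the screen material, messages the door and destroys the CodeSlot actors.
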(event `/Game/BP_BO/Inventory/BPI_InteractInterface.InteractWith`
  (params (PlayerCharacter :type "/Game/BP_BO/PlayerCharacter/BP_TPCharacter Object Reference"))
  ;[1 1 1] Upon being interacted with, call for the Player to start the selected type of Puzzle. Can only be done ONCE, reset when the puzzle is failed or cancelled.
  (`/Engine/EditorBlueprintResources/StandardMacros.DoOnce` false :!label _label
    (:`Completed`
      ;;[0.3 0 1] SFX - Puzzle Activation
      (`GameplayStatics.PlaySoundAtLocation` "/Engine/VREditor/Sounds/UI/Dockable_Window_Drop.Dockable_Window_Drop" (`SceneComponent.K2_GetComponentLocation` (`self.SecurityPanel`)) (struct) 1.0 1.0 0.0 null null null null)
      (message `/Game/BP_BO/Puzzles/BPI_PuzzleHandler.Puzzle Start` PlayerCharacter self false (`self.Code Or Hack`) (`self.E_PuzzleDifficulty`) null)
      ;[1 1 1] Attiva/Disattiva l'Outline dell'oggetto
      (`PrimitiveComponent.SetRenderCustomDepth` (`self.SecurityPanel`) false :!label _label_2))))

(event `self.TriggerBox.OnComponentBeginOverlap`
  (params (OverlappedComponent :type "PrimitiveComponent Object Reference") (OtherActor :type "Actor Object Reference") (OtherComp :type "PrimitiveComponent Object Reference") (OtherBodyIndex :type Integer) (bFromSweep :type Boolean) (SweepResult :type "HitResult Structure (by ref)"))
  ;[1 1 1] Attiva/Disattiva l'Outline dell'oggetto
  (if (== OtherActor (`GameplayStatics.GetPlayerCharacter` 0))
    (if (not (`self.Is NOT Interactable`))
      (`PrimitiveComponent.SetRenderCustomDepth` (`self.SecurityPanel`) true :!label _label_3))))

(event `self.TriggerBox.OnComponentEndOverlap`
  (params (OverlappedComponent :type "PrimitiveComponent Object Reference") (OtherActor :type "Actor Object Reference") (OtherComp :type "PrimitiveComponent Object Reference") (OtherBodyIndex :type Integer))
  ;[1 1 1] Attiva/Disattiva l'Outline dell'oggetto
  (if (== OtherActor (`GameplayStatics.GetPlayerCharacter` 0))
    (goto _label_2)))

(event `/Game/BP_BO/Puzzles/BPI_PuzzleHandler.Puzzle Failed`
  (params (`Caller Is QTE?` :type Boolean))
  ;[1 1 1] Upon being interacted with, call for the Player to start the selected type of Puzzle. Can only be done ONCE, reset when the puzzle is failed or cancelled.
  (`|ExecutionSequence`
    (:`then_0`
      (goto _label :!via `Reset`))
    (:`then_1`
      (goto _label_3))))

(event `/Game/BP_BO/Puzzles/BPI_PuzzleHandler.Puzzle Solved`
  (params (`Caller Is QTE?` :type Boolean))
  ;[1 1 1] Upon being notified by the player that the puzzle has been solved correctly, open the target door
  (set `self.Is NOT Interactable` true)
  (`PrimitiveComponent.SetMaterial` (`self.SecurityPanel`) 0 "/Game/3DAssetLevel/LevelDesign/Materials/ENR_Mats/Instances/MI_MoaiScreen.MI_MoaiScreen")
  ;;[0.3 0 1] SFX - Puzzle Solved
  (`GameplayStatics.PlaySoundAtLocation` "/Game/BO_Custom/SOUNDS/TUT_LEV/SE_Verified__VOICE_.SE_Verified__VOICE_" (`SceneComponent.K2_GetComponentLocation` (`self.SecurityPanel`)) (struct) 1.0 1.0 0.0 null null null null)
  (message `/Game/BP_BO/Puzzles/BPI_Unlockable.OpenTargetDoor` (`self.Door To Open`) self)
  (for _array_element (`self.CodeSlot`)
    (`/Engine/EditorBlueprintResources/StandardMacros.IsValid` _array_element
      (:`Is Valid`
        (`self.K2_DestroyActor` _array_element)))))

(event `self.ReceiveTick`
  (params (DeltaSeconds :type "Float (single-precision)"))
  ;[1 0 0] NO
)

(fn `Check IF Interactable`
  (returns (`Is NOT Interactable` :type Boolean))
  (return (`self.Is NOT Interactable`)))

(fn `UserConstructionScript`)