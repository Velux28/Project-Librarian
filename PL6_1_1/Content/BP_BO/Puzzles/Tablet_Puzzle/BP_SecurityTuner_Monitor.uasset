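; Security tuner monitor puzzle prop that opens the player's tablet to a "Hack" screen when interacted with.
; A DoOnce blocks repeat opening until reset, and a failed puzzle resets it while starting a cooldown timer that Tick counts down before interaction works again.
; OpenDoor unlocks the assigned door through the BPI_Unlockable interface.
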(event `self.ReceiveTick`
  (params (DeltaSeconds :type "Float (single-precision)"))
  (if (> (`self.Curr Fail Timer`) 0.0)
    (set `self.Curr Fail Timer` (- (`self.Curr Fail Timer`) DeltaSeconds))))

(event `/Game/BP_BO/Inventory/BPI_InteractInterface.InteractWith`
  (params (PlayerCharacter :type "/Game/BP_BO/PlayerCharacter/BP_TPCharacter Object Reference"))
  (if (<= (`self.Curr Fail Timer`) 0.0)
    (`/Engine/EditorBlueprintResources/StandardMacros.DoOnce` false :!label _label
      (:`Completed`
        (`/Game/BP_BO/PlayerCharacter/BP_TPCharacter.OpenTablet` PlayerCharacter "Hack")))))

(event `Reset Tuning`
  (goto _label :!via `Reset`))

(fn `LookAt`
  (returns (Message :type Text))
  (return ""))

(fn `Open Door`
  (bind _asbpi_unlockable (cast `/Game/BP_BO/Puzzles/BPI_Unlockable` (`self.Door To Open`)))
  (`/Game/BP_BO/Puzzles/BPI_Unlockable.Unlock` _asbpi_unlockable))

(fn `Puzzle Fail`
  (set `self.Curr Fail Timer` (`self.Puzzle Fail Timer`))
  (`self.Reset Tuning`))

(fn `UserConstructionScript`)