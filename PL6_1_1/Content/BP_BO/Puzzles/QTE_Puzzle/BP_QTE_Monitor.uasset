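; Interactable monitor that runs a multi-step QTE puzzle, opening its linked door when solved.
; On interaction it builds the embedded widget's QTEs from the DT_QTE row for its puzzle level and switches input to UI-only.
; Widget presses resolve to continue, win or fail; a timeout also fails, locking the monitor temporarily before retry.
; Player proximity toggles a custom-depth outline, removed permanently after a win.
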(event `self.TriggerBox.OnComponentBeginOverlap`
  (params (OverlappedComponent :type "PrimitiveComponent Object Reference") (OtherActor :type "Actor Object Reference") (OtherComp :type "PrimitiveComponent Object Reference") (OtherBodyIndex :type Integer) (bFromSweep :type Boolean) (SweepResult :type "HitResult Structure (by ref)"))
  ;[1 1 1] Attiva/Disattiva l'Outline dell'oggetto
  (if (== OtherActor (`GameplayStatics.GetPlayerCharacter` 0))
    (`PrimitiveComponent.SetRenderCustomDepth` (`self.Monitor`) true)))

(event `self.TriggerBox.OnComponentEndOverlap`
  (params (OverlappedComponent :type "PrimitiveComponent Object Reference") (OtherActor :type "Actor Object Reference") (OtherComp :type "PrimitiveComponent Object Reference") (OtherBodyIndex :type Integer))
  ;[1 1 1] Attiva/Disattiva l'Outline dell'oggetto
  (if (== (stale `self.TriggerBox.OnComponentBeginOverlap` OtherActor) (`GameplayStatics.GetPlayerCharacter` 0))
    (`PrimitiveComponent.SetRenderCustomDepth` (`self.Monitor`) false)))

(event `self.ReceiveBeginPlay`
  ;[0 0.3317 1] Widget management
  (`Widget.SetVisibility` (`WidgetComponent.GetWidget` (`self.MonitorUI`)) "Hidden")
  (bind _asw_puz_qte_multi (cast `/Game/BP_BO/Puzzles/QTE_Puzzle/W_PUZ_QTE_Multi` (`WidgetComponent.GetWidget` (`self.MonitorUI`))))
  (set `self.QTEWidget` _asw_puz_qte_multi))

(event `/Game/BP_BO/Inventory/BPI_InteractInterface.InteractWith`
  (params (PlayerCharacter :type "/Game/BP_BO/PlayerCharacter/BP_TPCharacter Object Reference"))
  (bind _qtewidget (`self.QTEWidget`))
  ;[1 1 1] Should the Puzzle start?
  (`/Engine/EditorBlueprintResources/StandardMacros.DoOnce` false :!label _label
    (:`Completed`
      (message `/Game/BP_BO/Puzzles/BPI_PuzzleHandler.Puzzle Start` PlayerCharacter self true "None" "NewEnumerator0" self)
      (`KismetSystemLibrary.Delay` 0.5)
      (`self.Set Puzzle`)
      (`WidgetBlueprintLibrary.SetInputMode_UIOnlyEx` (`GameplayStatics.GetPlayerController` 0) _qtewidget "LockAlways")
      (`Widget.SetKeyboardFocus` _qtewidget)
      (set `self.PuzzleNotOngoing` false)
      (`KismetSystemLibrary.Delay` (`self.Puzzle Fail Cooldown`))
      (if (not (`self.PuzzleNotOngoing`))
        (`/Game/BP_BO/Puzzles/BPI_PuzzleHandler.Puzzle Failed` false)
        ;[1 0 0] Qui si potrebbe aggiungere la logica che fa partire l'allarme per l'IA
        (`KismetSystemLibrary.Delay` 0.2) ; Per non coprire l'altro SFX
      ))))

(event `Reset QTE`
  ;[1 1 1] Should the Puzzle start?
  (`KismetSystemLibrary.Delay` (`self.LockoutTimer`))
  (`PrimitiveComponent.SetMaterial` (`self.Monitor`) 1 "/Game/BP_BO/Puzzles/QTE_Puzzle/QTE/MATERIALS/M_QTE_Concept_A.M_QTE_Concept_A")
  (goto _label :!via `Reset`))

(event `/Game/BP_BO/Puzzles/BPI_PuzzleHandler.Puzzle Failed`
  (params (`Caller Is QTE?` :type Boolean))
  ;[1 1 1] QTE Gameplay and result management + CAMERA RESET
  (`PrimitiveComponent.SetMaterial` (`self.Monitor`) 1 "/Game/BP_BO/Puzzles/QTE_Puzzle/QTE/MATERIALS/M_QTE_Locked.M_QTE_Locked" :!label _label_2)
  (`Widget.SetVisibility` (`self.QTEWidget`) "Hidden")
  (`WidgetBlueprintLibrary.SetInputMode_GameOnly` (`GameplayStatics.GetPlayerController` 0))
  (`GameplayStatics.PlaySound2D` "/Game/SoundDesign/SoundWaves/SFX_CardReaderNegative_2_Individuals.SFX_CardReaderNegative_2_Individuals" 1.0 1.0 0.0 null null)
  (message `/Game/BP_BO/Puzzles/BPI_PuzzleHandler.Puzzle Failed` (`GameplayStatics.GetPlayerCharacter` 0) true)
  (`self.Reset QTE`)
  (set `self.PuzzleNotOngoing` true))

(event `QTE_Press`
  ;[1 1 1] QTE Gameplay and result management + CAMERA RESET
  (if (`Widget.IsVisible` (`self.QTEWidget`))
    (bind _result (`/Game/BP_BO/Puzzles/QTE_Puzzle/W_PUZ_QTE_Multi.Result QTE` (`self.QTEWidget`)))
    (switch `/Game/BP_BO/Enum/E_QTEResults` _result
      (:`NewEnumerator0`
        (goto _label_2))
      (:`NewEnumerator1`
        (`GameplayStatics.PlaySound2D` "/Game/BO_Custom/SOUNDS/GENERIC/Accepted.Accepted" 1.0 1.0 0.0 null null))
      (:`NewEnumerator2`
        (`PrimitiveComponent.SetMaterial` (`self.Monitor`) 1 "/Game/BP_BO/Puzzles/QTE_Puzzle/QTE/MATERIALS/M_QTE_WinScreen.M_QTE_WinScreen")
        (`Widget.SetVisibility` (`self.QTEWidget`) "Hidden")
        (`WidgetBlueprintLibrary.SetInputMode_GameOnly` (`GameplayStatics.GetPlayerController` 0))
        (`GameplayStatics.PlaySound2D` "/Game/BO_Custom/SOUNDS/TUT_LEV/Cues/SC_Verified.SC_Verified" 1.0 1.0 0.0 null null)
        (message `/Game/BP_BO/Puzzles/BPI_PuzzleHandler.Puzzle Solved` (`GameplayStatics.GetPlayerCharacter` 0) true)
        (message `/Game/BP_BO/Puzzles/BPI_Unlockable.OpenTargetDoor` (`self.Door To Open`) self)
        (set `self.PuzzleNotOngoing` true)
        ;[1 1 1] Disabilito permanentemente l'Outline
        (`PrimitiveComponent.SetRenderCustomDepth` (`self.Monitor`) false)
        (`ActorComponent.K2_DestroyComponent` (`self.TriggerBox`))))))

(fn `Check IF Interactable`
  (returns (`Is NOT Interactable` :type Boolean))
  (return false))

(fn `Set Puzzle`
  (bind _qtewidget (`self.QTEWidget`))
  (bind _outrownames (`DataTableFunctionLibrary.GetDataTableRowNames` "/Game/BP_BO/Puzzles/DT_QTE.DT_QTE"))
  (bind _returnvalue (`|GetDataTableRow` "/Game/BP_BO/Puzzles/DT_QTE.DT_QTE" (`|GetArrayItem` _outrownames (- (`self.Puzzle Level`) 1)))
    (:`then`
      (`/Game/BP_BO/Puzzles/QTE_Puzzle/W_PUZ_QTE_Multi.Clear QTE List` (`self.QTEWidget`))
      (for _ (range 1 (+ (break `/Game/BP_BO/Puzzles/S_QTEFormat` _returnvalue) 1))
        (bind _returnvalue_2 (`|CreateWidget` "/Game/BP_BO/Puzzles/QTE_Puzzle/W_PUZ_QTE_Widget.W_PUZ_QTE_Widget_C"))
        (`/Game/BP_BO/Puzzles/QTE_Puzzle/W_PUZ_QTE_Multi.AddQTE` (`self.QTEWidget`) _returnvalue_2))
      (`/Game/BP_BO/Puzzles/QTE_Puzzle/W_PUZ_QTE_Multi.Set QTE Angle Array` _qtewidget (`.Angle_9_FE6B1FF943EF8FE5F333DA920CB2AA1A` (break `/Game/BP_BO/Puzzles/S_QTEFormat` _returnvalue)))
      (`/Game/BP_BO/Puzzles/QTE_Puzzle/W_PUZ_QTE_Multi.Set QTE Speed Array` _qtewidget (`.Speed_10_A3098F6D432818CB43B67B91FFACA9EB` (break `/Game/BP_BO/Puzzles/S_QTEFormat` _returnvalue)))
      (`/Game/BP_BO/Puzzles/QTE_Puzzle/W_PUZ_QTE_Multi.Reset QTE` _qtewidget)
      (set `/Game/BP_BO/Puzzles/QTE_Puzzle/W_PUZ_QTE_Multi.ObjToOpen` self _qtewidget)
      (`/Game/BP_BO/Puzzles/QTE_Puzzle/W_PUZ_QTE_Multi.Set QTE Visibility` _qtewidget "Visible")
      (`Widget.SetVisibility` _qtewidget "Visible"))))

(fn `UserConstructionScript`)