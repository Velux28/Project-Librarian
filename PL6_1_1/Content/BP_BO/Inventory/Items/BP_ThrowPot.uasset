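; BP_ThrowPot is a pot item that shatters into five shards when it hits anything other than the player character.
; On BeginPlay, four physics constraints chain the shards together, and the shards are hidden behind the BrokenPot component.
; A qualifying hit on BrokenPot breaks the constraints, calls the sound component with an empty name, reveals the shards and destroys BrokenPot.
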(event `self.ReceiveBeginPlay`
  (`PhysicsConstraintComponent.SetConstrainedComponents` (`self.Constrain1`) (`self.PotShard0`) "None" (`self.PotShard1`) "None")
  (`PhysicsConstraintComponent.SetConstrainedComponents` (`self.Constrain2`) (`self.PotShard1`) "None" (`self.PotShard2`) "None")
  (`PhysicsConstraintComponent.SetConstrainedComponents` (`self.Constrain3`) (`self.PotShard2`) "None" (`self.PotShard3`) "None")
  (`PhysicsConstraintComponent.SetConstrainedComponents` (`self.Constrain4`) (`self.PotShard3`) "None" (`self.PotShard4`) "None")
  (`SceneComponent.SetVisibility` (`self.PotShard0`) false false)
  (`SceneComponent.SetVisibility` (`self.PotShard2`) false false)
  (`SceneComponent.SetVisibility` (`self.PotShard3`) false false)
  (`SceneComponent.SetVisibility` (`self.PotShard4`) false false)
  (`SceneComponent.SetVisibility` (`self.PotShard1`) false false))

(event `self.BrokenPot.OnComponentHit`
  (params (HitComponent :type "PrimitiveComponent Object Reference") (OtherActor :type "Actor Object Reference") (OtherComp :type "PrimitiveComponent Object Reference") (NormalImpulse :type "Vector Structure") (Hit :type "HitResult Structure (by ref)"))
  (if (!= OtherActor (`GameplayStatics.GetPlayerCharacter` 0))
    (`PhysicsConstraintComponent.BreakConstraint` (`self.Constrain4`))
    (`PhysicsConstraintComponent.BreakConstraint` (`self.Constrain3`))
    (`PhysicsConstraintComponent.BreakConstraint` (`self.Constrain1`))
    (`PhysicsConstraintComponent.BreakConstraint` (`self.Constrain2`))
    (`SoundComponent.PlaySoundByName` (`self.SoundComp`) "")
    (`SceneComponent.SetVisibility` (`self.PotShard0`) true false)
    (`SceneComponent.SetVisibility` (`self.PotShard2`) true false)
    (`SceneComponent.SetVisibility` (`self.PotShard3`) true false)
    (`SceneComponent.SetVisibility` (`self.PotShard4`) true false)
    (`SceneComponent.SetVisibility` (`self.PotShard1`) true false)
    ;[0.974 1 0] Maybe to much
    (`ActorComponent.K2_DestroyComponent` (`self.BrokenPot`))))

(fn `UserConstructionScript`)