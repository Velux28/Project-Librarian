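; Benchmark test actor that travels along the level's BP_BENCH_Spline when StartTestPath is called.
; The event finds and caches the spline actor, waits briefly, then plays a timeline whose track maps to distance along the spline, setting world location and rotation each update.
; The timeline play rate is the inverse of TimeToComplete, so run duration changes without editing the timeline.
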(event `StartTestPath`
  (bind _spline (`/Game/BP_BO/Benchmark/BP_BENCH_Spline.Spline` (`self.REF_BenchSpline`)))
  (bind _returnvalue (`GameplayStatics.GetActorOfClass` "/Game/BP_BO/Benchmark/BP_BENCH_Spline.BP_BENCH_Spline_C"))
  (set `self.REF_BenchSpline` _returnvalue)
  (`KismetSystemLibrary.Delay` 0.2)
  ;[1 1 1] Allows to dynamically change Timeline lenght without editing it
  (`TimelineComponent.SetPlayRate` (`self.T_MoveZiopera`) (/ 1.0 (`self.TimeToComplete`)))
  (bind (_direction _movetrack) (`Timeline|T_MoveZiopera`)
    (:`Update`
      (bind _returnvalue_2 (`KismetMathLibrary.Lerp` 0.0 (`SplineComponent.GetSplineLength` _spline) _movetrack))
      (`self.K2_SetActorLocationAndRotation` (`SplineComponent.GetLocationAtDistanceAlongSpline` _spline _returnvalue_2 "World") (`SplineComponent.GetRotationAtDistanceAlongSpline` _spline _returnvalue_2 "World")))))

(fn `UserConstructionScript`)