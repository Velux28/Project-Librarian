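; Benchmark camera that flies along the level's BP_BENCH_Spline to measure performance.
; A one-time SpaceBar press clears widgets and starts a timeline whose play rate derives from FTimeToComplete, so duration changes without editing the track.
; Each update lerps distance along the spline, applying its rotation and location, raised to simulate player height.
; FPS and unit stat commands run at start and again at finish, alongside a restart-level message.
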(event `self.ReceiveBeginPlay`
  ;[1 1 1] Set Spline Ref
  (bind _returnvalue (`GameplayStatics.GetActorOfClass` "/Game/BP_BO/Benchmark/BP_BENCH_Spline.BP_BENCH_Spline_C"))
  (set `self.REF_BenchSpline` _returnvalue)
  (`self.EnableInput` null) ; Needed for manula start
)

(event `Key|SpaceBar`
  (params (Key :type "Key Structure"))
  (:`Pressed`
    ;[1 1 1] Manual Benchmark Start
    (`/Engine/EditorBlueprintResources/StandardMacros.DoOnce` false
      (:`Completed`
        (`self.StartTestPath`)
        (`WidgetLayoutLibrary.RemoveAllWidgets`)))))

(event `StartTestPath`
  (bind _spline (`/Game/BP_BO/Benchmark/BP_BENCH_Spline.Spline` (`self.REF_BenchSpline`)))
  (`|ExecutionSequence`
    (:`then_0`
      ;[1 1 1] Allows to dynamically change Timeline lenght without editing it
      (`TimelineComponent.SetPlayRate` (`self.T_Move Camera`) (/ 1.0 (`self.F_TimeToComplete`)))
      (bind (_direction _movetrack) (`Timeline|T_Move Camera`)
        (:`Update`
          (bind _returnvalue (`KismetMathLibrary.Lerp` 0.0 (`SplineComponent.GetSplineLength` _spline) _movetrack))
          (bind (_returnvalue_x _returnvalue_y _returnvalue_z) (`KismetMathLibrary.BreakVector` (`SplineComponent.GetLocationAtDistanceAlongSpline` _spline _returnvalue "World")))
          ;[1 1 1] Moves camera along spline
          (`self.K2_SetActorLocationAndRotation` (`KismetMathLibrary.MakeVector` _returnvalue_x _returnvalue_y (+ _returnvalue_z 100.0)) (`SplineComponent.GetRotationAtDistanceAlongSpline` _spline _returnvalue "World")))
        (:`Finished`
          ;[1 1 1] Benchmark shutdown
          (`KismetSystemLibrary.PrintText` "BENCHMARK DONE, PLESE RESTART LEVEL")
          (`self.ShowStats`))))
    (:`then_1`
      (`self.ShowStats`))))

(event `ShowStats`
  ;[1 1 1] Show useful stats
  (`KismetSystemLibrary.ExecuteConsoleCommand` "stat fps" null)
  (`KismetSystemLibrary.ExecuteConsoleCommand` "stat unit" null))

(fn `UserConstructionScript`)