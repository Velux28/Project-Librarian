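; NPC character that attacks the player on touch and carries a scanner for AI detection.
; Capsule overlap with the player applies heavy damage meant to kill, plays the attack montage and halts movement.
; StartScanning lifts AIScanComponent's scanner above the actor and enables it; EndScanning drops it far below the world and disables it.
; The event graph's StartScanning call is unwired, noted as deprecated yet the version that positions correctly.
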(event `self.Capsule.OnComponentBeginOverlap`
  (params (OverlappedComponent :type "PrimitiveComponent Object Reference") (OtherActor :type "Actor Object Reference") (OtherComp :type "PrimitiveComponent Object Reference") (OtherBodyIndex :type Integer) (bFromSweep :type Boolean) (SweepResult :type "HitResult Structure (by ref)"))
  (bind _returnvalue (`GameplayStatics.GetPlayerCharacter` 0))
  ;[1 1 1] Kill Player
  (if (== OtherActor _returnvalue)
    (`GameplayStatics.ApplyDamage` _returnvalue 150.0 null self)
    (`|PlayMontage` (`self.Mesh`) "/Game/3DAssetLevel/LevelDesign/Animations/NPC_IA/Robot_New/Montages/MONT_AI_Attack.MONT_AI_Attack"
      (:`then`
        (`MovementComponent.StopMovementImmediately` (`self.CharacterMovement`))))))

(fn `End Scanning`
  (bind _ai_scan_component (`self.AI_Scan_Component`))
  (`/Game/BP_BO/ArtificialIntelligence/Components/AI_Scan_Component.Set Scanner Transform` _ai_scan_component (`KismetMathLibrary.MakeTransform` (0.0 0.0 -100000000.0)))
  (`/Game/BP_BO/ArtificialIntelligence/Components/AI_Scan_Component.SetScannerStatus` _ai_scan_component false))

(fn `Start Scanning`
  (bind _ai_scan_component (`self.AI_Scan_Component`))
  (bind _returnvalue (`self.GetTransform` self))
  (`/Game/BP_BO/ArtificialIntelligence/Components/AI_Scan_Component.Set Scanner Transform` _ai_scan_component (`KismetMathLibrary.MakeTransform` (`KismetMathLibrary.MakeVector` (.x (.location _returnvalue)) (.y (.location _returnvalue)) (+ (.z (.location _returnvalue)) 85.0)) (.rotation _returnvalue) (.scale _returnvalue)))
  (`/Game/BP_BO/ArtificialIntelligence/Components/AI_Scan_Component.SetScannerStatus` _ai_scan_component true))

(fn `UserConstructionScript`)