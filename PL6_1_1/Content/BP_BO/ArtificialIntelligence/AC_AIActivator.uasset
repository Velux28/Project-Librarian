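; Activator component that wakes and shuts down NPC AI on request.
; ActivateAI and DeactivateAI validate the character, cast its controller to AI_NPC and call CallForActivation or CallForDeActivation, leaving senses and behavior logic to the controller.
; The behavior tree input to ActivateAI is only checked for validity, never passed on.
; Older nodes that toggled senses, behavior tree and patrol directly remain disconnected.
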(fn `Activate AI`
  (params (AICharacter :type "/Game/BP_BO/ArtificialIntelligence/BP_NPC Object Reference") (AIBT :type "BehaviorTree Object Reference"))
  ;[1 1 1] Essendo reponsabilità dell'IA accendere i propri sensi ed entrare in Patrol, l'Activator deve solo far partire la funzione a questo relativa
  (`/Engine/EditorBlueprintResources/StandardMacros.IsValid` AICharacter
    (:`Is Valid`
      (`/Engine/EditorBlueprintResources/StandardMacros.IsValid` AIBT
        (:`Is Valid`
          (bind _asai_npc (cast `/Game/BP_BO/ArtificialIntelligence/AI_NPC` (`Pawn.GetController` AICharacter)))
          (`/Game/BP_BO/ArtificialIntelligence/AI_NPC.Call For Activation` _asai_npc))))))

(fn `De-activate AI`
  (params (`NPC Ref` :type "/Game/BP_BO/ArtificialIntelligence/BP_NPC Object Reference"))
  ;[1 1 1] Essendo reponsabilità dell'IA spegnere i propri sensi, l'Activator deve solo far partire la funzione a questo relativa
  (`/Engine/EditorBlueprintResources/StandardMacros.IsValid` `NPC Ref`
    (:`Is Valid`
      (bind _asai_npc (cast `/Game/BP_BO/ArtificialIntelligence/AI_NPC` (`Pawn.GetController` `NPC Ref`)))
      (`/Game/BP_BO/ArtificialIntelligence/AI_NPC.Call For De-Activation` _asai_npc))))