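; AC_Chase switches an enemy's AI into and out of a scripted chase.
; Both functions cast the controller of EnemyRef to AI_NPC and do nothing if the cast fails.
; ActivateChase calls GoToScriptedChase on that controller.
; DeactivateChase re-enables sight sensing and sets the AI state to Chase, so ending the scripted chase leaves the enemy in the Chase state.
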(fn `ActivateChase`
  (bind _asai_npc (cast `/Game/BP_BO/ArtificialIntelligence/AI_NPC` (`Pawn.GetController` (`self.EnemyRef`))))
  (`/Game/BP_BO/ArtificialIntelligence/AI_NPC.Go To Scripted Chase` _asai_npc))

(fn `DeactivateChase`
  (bind _asai_npc (cast `/Game/BP_BO/ArtificialIntelligence/AI_NPC` (`Pawn.GetController` (`self.EnemyRef`))))
  (`AIPerceptionComponent.SetSenseEnabled` (`NPCAIController.AISense` _asai_npc) "/Script/AIModule.AISense_Sight" true)
  (set `NPCAIController.CurrAIState` "Chase" _asai_npc))